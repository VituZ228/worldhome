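; ChoosePlanet is an actor that acts as an inventory of planets for the colony menu UI.
; On BeginPlay it sizes the slot array and creates the main UI widget, passing itself as the inventory and caching the colony menu.
; AddPlanet stores a planet class in the first empty slot and refreshes that slot's widget.
; Slots hold only classes, so planet info is read from class defaults.
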(event Custom|UpdateSlotAtIndex
  (params (Index :type Integer))
  (Default|UpdateSlot (Utilities|Array|Get(acopy) (Variables|/Game/UI_and_Widgets/ColonyMenu.ColonyMenu_C|GetSlotsWidgets (Variables|Default|GetColony%20Menu%20Widget)) Index)))

(event EventBeginPlay
  (Utilities|Array|Resize (Variables|Default|GetSlots) (Variables|Default|GetAmountOfSlots))
  (bind _returnvalue (UserInterface|CreateWidget "/Game/UI_and_Widgets/Main_UI_Widget.Main_UI_Widget_C" 0 self (Variables|Default|GetSlots%20Per%20Row)))
  (bind _output_get (Variables|Default|SetMainWidget _returnvalue))
  (Variables|Default|SetColony%20Menu%20Widget (Variables|/Game/UI_and_Widgets/Main_UI_Widget.Main_UI_Widget_C|GetColonyMenuWidget _output_get))
  (UserInterface|Viewport|AddtoViewport (Variables|Default|GetMainWidget) 0))

(event Collision|EventActorBeginOverlap
  (params (OtherActor :type Actor%20Object%20Reference)))

(event EventTick
  (params (DeltaSeconds :type Float%20%28single-precision%29)))

(fn ConstructionScript)

(fn IsSlotEmpty
  (params (Index :type Integer))
  (return (not (Utilities|IsValidClass (Utilities|Struct|BreakS_Planet_Slot (Utilities|Array|Get(acopy) (Variables|Default|GetSlots) Index))))))

(fn GetPlanetInfoatIndex
  (params (Index :type Integer))
  (bind _slots (Variables|Default|GetSlots))
  (bind _output (Utilities|Array|Get(acopy) _slots Index))
  (bind _planetclass (Utilities|Struct|BreakS_Planet_Slot _output))
  (if (Utilities|IsValidClass _planetclass)
    (return false (.PlanetInfo (Utilities|GetClassDefaults _planetclass)))
    (else
      (return true ""))))

(fn SearchEmptySlot
  (bind (_array_element _array_index) (Utilities|Array|ForEachLoopwithBreak (Variables|Default|GetSlots) :!label _label)
    (:LoopBody
      (if (not (Utilities|IsValidClass (Utilities|Struct|BreakS_Planet_Slot _array_element)))
        (LocalVariables|SetLocalBool true)
        (LocalVariables|SetLocal_Index _array_index)
        (goto _label Break)))
    (:Completed
      (return (LocalVariables|GetLocalBool) (LocalVariables|GetLocal_Index)))))

(fn AddPlanet
  (params (PlanetClass :type Master%20Planet%20Asset%20Class%20Reference))
  (LocalVariables|SetLocalPlanetClass PlanetClass)
  (bind (_sucsses_ _index) (CallFunction|SearchEmptySlot))
  (if _sucsses_
    (bind _output_get (LocalVariables|SetLocalFoundIndex _index))
    (Utilities|Array|SetArrayElem (Variables|Default|GetSlots) _output_get (Utilities|Struct|MakeS_Planet_Slot (LocalVariables|GetLocalPlanetClass)))
    (CallFunction|UpdateSlotatIndex (LocalVariables|GetLocalFoundIndex))
    (Development|PrintString "Planet Was Added To Colony Meny")
    (return true)
    (else
      (return false))))