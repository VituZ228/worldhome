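; Commander A4 spaceship actor with a selectable hull color scheme and two adjustable thruster flames.
; The construction script applies the chosen hull material, sets a matching thruster color for some schemes, and creates dynamic instances for the hull and four rocket flare layers.
; A Thrust value drives hull glow, flame length and flare opacity.
; An optional demo animates Thrust by timeline after a color-based delay on BeginPlay.
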(event EventBeginPlay
  (if (Variables|Default|GetAnimateThrusters_Demo)
    (Utilities|FlowControl|Delay (* (Variables|Default|GetColor) 0.4))
    (bind _thrust (Timeline|Timeline_0 Play)
      (:Update
        (Variables|Default|SetThrust _thrust)
        (CallFunction|AdjustThrusters)))))

(fn ConstructionScript
  (|CreateThrusterDynamicMaterials)
  (Math|Color|SelectColor)
  (|CreateShipDynamicMaterial)
  (CallFunction|AdjustThrusters)
  (|SetThrusterColor))

(fn AdjustThrusters
  (bind _thrust (Variables|Default|GetThrust))
  ;[1 1 1] Adjust Thruster Intensity
  (Rendering|Material|SetScalarParameterValue (Variables|Default|GetShipMaterial) "Thrust" (Math|Float|Lerp 0.0 5.0 _thrust) :!class /Script/Engine.MaterialInstanceDynamic)
  (Transformation|SetRelativeScale3D (Variables|Default|GetSM_Frigate_MB3_Thruster_TL) (Math|Vector|MakeVector (Math|Float|Lerp 0.0 3.5e+02 _thrust) 28.5 28.5))
  (Rendering|Material|SetScalarParameterValue (Variables|Default|GetDynMat_RocketFlare0) "Opacity" (Variables|Default|GetThrust) :!class /Script/Engine.MaterialInstanceDynamic))