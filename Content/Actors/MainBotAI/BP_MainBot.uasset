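; Computer opponent for a ship-based strategy game that runs the BT_MainBot behavior tree through its AI controller on BeginPlay.
; Every tick it scans all BasedShip actors to rebuild its team's army list and a class-weighted army size, clearing PushOpponentMode when that size is zero.
; A timer accumulated on Tick periodically grants free resources as an economy cheat and prints the totals for debugging.
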(event EventBeginPlay
  (AI|RunBehaviorTree (AI|GetAIController self) "/Game/Actors/MainBotAI/BT_MainBot.BT_MainBot"))

(event EventTick
  (params (DeltaSeconds :type Float%20%28single-precision%29))
  (Variables|Default|SetLocalCounter 0)
  (CallFunction|CountMyUnits)
  (Variables|Default|SetCurrentArmyAmount (Variables|Default|GetLocalCounter))
  (CallFunction|CheatResoursesFarming))

(fn ConstructionScript)

(fn CountMyUnits
  (Utilities|Array|Clear (Variables|Default|GetAllArmy))
  (bind _outactors (Actor|GetAllActorsOfClass "/Game/Actors/Units/SpaceShips/BasedShip.BasedShip_C"))
  (for _array_element _outactors
    (if (== (Variables|/Game/Actors/Units/SpaceShips/BasedShip.BasedShip_C|GetTeam _array_element) (Variables|Default|GetTeam))
      (Utilities|Array|AddUnique (Variables|Default|GetAllArmy) _array_element))
    (if (and (== (Variables|/Game/Actors/Units/SpaceShips/BasedShip.BasedShip_C|GetTeam _array_element) (Variables|Default|GetTeam)) (or (Utilities|Enum|Equal(Enum) (Variables|/Game/Actors/Units/SpaceShips/BasedShip.BasedShip_C|GetUnitClass _array_element) "NewEnumerator5") (Utilities|Enum|Equal(Enum) (Variables|/Game/Actors/Units/SpaceShips/BasedShip.BasedShip_C|GetUnitClass _array_element) "NewEnumerator6")))
      (Variables|Default|SetLocalCounter (+ (Variables|Default|GetLocalCounter) 1))
      (elif (and (or (Utilities|Enum|Equal(Enum) (Variables|/Game/Actors/Units/SpaceShips/BasedShip.BasedShip_C|GetUnitClass _array_element) "NewEnumerator7") (Utilities|Enum|Equal(Enum) (Variables|/Game/Actors/Units/SpaceShips/BasedShip.BasedShip_C|GetUnitClass _array_element) "NewEnumerator8")) (== (Variables|/Game/Actors/Units/SpaceShips/BasedShip.BasedShip_C|GetTeam _array_element) (Variables|Default|GetTeam)))
        (Variables|Default|SetLocalCounter (+ (Variables|Default|GetLocalCounter) 2))
        (elif (and (or (Utilities|Enum|Equal(Enum) (Variables|/Game/Actors/Units/SpaceShips/BasedShip.BasedShip_C|GetUnitClass _array_element) "NewEnumerator9") (Utilities|Enum|Equal(Enum) (Variables|/Game/Actors/Units/SpaceShips/BasedShip.BasedShip_C|GetUnitClass _array_element) "NewEnumerator10")) (== (Variables|/Game/Actors/Units/SpaceShips/BasedShip.BasedShip_C|GetTeam _array_element) (Variables|Default|GetTeam)))
          (Variables|Default|SetLocalCounter (+ (Variables|Default|GetLocalCounter) 3))))))
  (bind _output_get (Variables|Default|SetCurrentArmyAmount (Variables|Default|GetLocalCounter)))
  (if (== _output_get 0)
    (Variables|Default|SetPushOpponentMode false)))

(fn CheatResoursesFarming
  (bind _playerressourses (Variables|Default|GetPlayerRessourses))
  (bind _output (Utilities|Array|Get(acopy) _playerressourses 3))
  (bind _output_2 (Utilities|Array|Get(acopy) _playerressourses))
  (bind _output_3 (Utilities|Array|Get(acopy) _playerressourses 1))
  (bind _output_4 (Utilities|Array|Get(acopy) _playerressourses 2))
  (Variables|Default|SetResoursesTickCounter (+ (Variables|Default|GetResoursesTickCounter) (Utilities|Time|GetWorldDeltaSeconds)))
  (if (>= (Variables|Default|GetResoursesTickCounter) 5.0)
    (Variables|Default|SetResoursesTickCounter 0.0)
    (Utilities|Array|SetArrayElem _playerressourses 0 (+ _output_2 500))
    (Utilities|Array|SetArrayElem _playerressourses 1 (+ _output_3 500))
    (Utilities|Array|SetArrayElem _playerressourses 2 (+ _output_4 250))
    (Utilities|Array|SetArrayElem _playerressourses 3 (+ _output 250))
    (Development|PrintString (Utilities|String|ToString(Integer) _output_2))
    (Development|PrintString (Utilities|String|ToString(Integer) _output_3))
    (Development|PrintString (Utilities|String|ToString(Integer) _output_4))
    (Development|PrintString (Utilities|String|ToString(Integer) _output))))