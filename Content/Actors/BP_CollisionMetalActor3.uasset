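; BP_CollisionMetalActor3 is a collision hazard actor, apparently metal debris, that damages ships on impact.
; When its static mesh hits a BasedShip, it spawns an explosion emitter at the hit location and subtracts a fixed amount of CurrentHp unless the ship is invincible.
; Unconnected leftover nodes for swapping to a rubbish mesh and randomizing scale and mass never run.
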(event OnComponentHit(MainStaticMesh)
  (params (HitComponent :type Primitive%20Component%20Object%20Reference) (OtherActor :type Actor%20Object%20Reference) (OtherComp :type Primitive%20Component%20Object%20Reference) (NormalImpulse :type Vector :default "0, 0, 0") (Hit :type Hit%20Result%20Structure%20%28by%20ref%29))
  (bind _asbased_ship (Utilities|Casting|CastToBasedShip OtherActor))
  (Effects|SpawnEmitteratLocation "/Game/VFX_Toolkit_V1/ParticleSystems/356Days/Par_MatraBoom_01.Par_MatraBoom_01" (.Location (Collision|BreakHitResult Hit)))
  (if (not (Variables|/Game/Actors/Units/SpaceShips/BasedShip.BasedShip_C|GetUnitInvincible _asbased_ship))
    (Variables|/Game/Actors/Units/SpaceShips/BasedShip.BasedShip_C|SetCurrentHp _asbased_ship (- (Variables|/Game/Actors/Units/SpaceShips/BasedShip.BasedShip_C|GetCurrentHp _asbased_ship) 25.0))))

(event EventBeginPlay)

(fn ConstructionScript)