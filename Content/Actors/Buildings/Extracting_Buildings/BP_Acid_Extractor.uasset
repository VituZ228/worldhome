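; Acid extractor building that costs player resources when built, refunds a share when sold, and updates the shared building count in its widgets.
; Clicking it during energy-link mode attaches or detaches it from the chosen energy station, reserving or returning station energy.
; While powered, a self-retriggering Delay loop moves acid from the current planet to the player, with planet category boosting yield.
; Tick draws the station link using a debug line trace.
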(event OnClicked(BuildMesh)
  (params (TouchedComponent :type Primitive%20Component%20Object%20Reference) (ButtonPressed :type Key%20Structure :default "None"))
  (bind _gameinstance_ref (Variables|Default|GetGameInstance_Ref))
  (bind _buildinginteractionwidget_ref (Variables|Default|GetBuildingInteractionWidget_Ref))
  (bind _buildinginteractionwidget_ref_2 (Variables|Default|GetBuildingInteractionWidget_Ref))
  (bind _idofenergy (Variables|/Game/SaveGame/GlobalGameInstance.GlobalGameInstance_C|Getidofenergy _gameinstance_ref))
  (if (Variables|/Game/SaveGame/GlobalGameInstance.GlobalGameInstance_C|GetActive_Energy _gameinstance_ref)
    (if (Variables|Default|GetAlready_Work)
      (if (== (Variables|Default|GetId_Added_Station) _idofenergy)
        (Variables|Default|SetAlready_Work false)
        (Variables|/Game/SaveGame/GlobalGameInstance.GlobalGameInstance_C|SetActive_Energy _gameinstance_ref true)
        (bind _outactors (Actor|GetAllActorsOfClass "/Game/Actors/Buildings/Civilian_Buildings/BP_Energy_Station.BP_Energy_Station_C"))
        (Variables|/Game/Actors/Buildings/Civilian_Buildings/BP_Energy_Station.BP_Energy_Station_C|Setenergy%20cost (Utilities|Array|Get(acopy) _outactors _idofenergy) (+ (Variables|/Game/Actors/Buildings/Civilian_Buildings/BP_Energy_Station.BP_Energy_Station_C|Getenergy%20cost (Utilities|Array|Get(acopy) _outactors _idofenergy)) 1e+03))
        (Default|GetBuildingInfo _buildinginteractionwidget_ref "Добыча Кислот" "Активен" (Variables|/Game/UI_and_Widgets/Colony_system/BuildingsWidgets/Building_Interaction_Widget.Building_Interaction_Widget_C|GetBuildingAmount _buildinginteractionwidget_ref) (Utilities|Text|ToText(Float) (* (Variables|Default|GetSellCost) 1e+02) "HalfToEven") false))
      (else
        (bind _outactors_2 (Actor|GetAllActorsOfClass "/Game/Actors/Buildings/Civilian_Buildings/BP_Energy_Station.BP_Energy_Station_C"))
        (if (not (< (Variables|/Game/Actors/Buildings/Civilian_Buildings/BP_Energy_Station.BP_Energy_Station_C|Getenergy%20cost (Utilities|Array|Get(acopy) _outactors_2 _idofenergy)) 1e+03))
          (Variables|/Game/Actors/Buildings/Civilian_Buildings/BP_Energy_Station.BP_Energy_Station_C|Setenergy%20cost (Utilities|Array|Get(acopy) _outactors_2 _idofenergy) (- (Variables|/Game/Actors/Buildings/Civilian_Buildings/BP_Energy_Station.BP_Energy_Station_C|Getenergy%20cost (Utilities|Array|Get(acopy) _outactors_2 _idofenergy)) 1e+03))
          (Variables|Default|SetAlready_Work true)
          (Variables|Default|SetVector (Transformation|GetActorLocation (Utilities|Array|Get(acopy) _outactors_2 _idofenergy)))
          (Variables|/Game/SaveGame/GlobalGameInstance.GlobalGameInstance_C|SetActive_Energy _gameinstance_ref false)
          (Variables|Default|Setid_added_station _idofenergy)
          (CallFunction|TickAcidExtractor)
          (Default|GetBuildingInfo _buildinginteractionwidget_ref_2 "Добыча Кислот" "Требуется энергия" (Variables|/Game/UI_and_Widgets/Colony_system/BuildingsWidgets/Building_Interaction_Widget.Building_Interaction_Widget_C|GetBuildingAmount _buildinginteractionwidget_ref_2) (Utilities|Text|ToText(Float) (* (Variables|Default|GetSellCost) 1e+02) "HalfToEven") false))))))

(event Custom|SellBtn_Pressed_Event
  ;[0 0.1566 1] СЛЕДИТ ЗА НАЖАТИЕМ НА КНОПКУ ПРОДАЖИ, ПРИ НАЖАТИИ ВОЗВРАЩАЕТ ЦЕНУ ЗДАНИЯ УМНОЖЕНУЮ НА ПРОЦЕНТ SellCost
  (if (Variables|/Script/Engine.PrimitiveComponent|GetbRenderCustomDepth (Variables|Default|GetBuildMesh))
    (Actor|DestroyActor)))

(event Custom|Tick_AcidExtractor
  (bind _valueofproduction (Variables|Default|GetValueOfProduction))
  (bind _currentplanet (Variables|Default|GetCurrentPlanet))
  (bind _controllercam_ref (Variables|Default|GetControllerCam_Ref))
  (bind _planetressourses (Variables|/Game/Actors/Planets/Master_Planet_Asset.Master_Planet_Asset_C|GetPlanetRessourses _currentplanet))
  (bind _playerressourses (Variables|/Game/CameraAndControllerStuff/controllerCam.controllerCam_C|GetPlayerRessourses _controllercam_ref))
  (bind _output (Utilities|Array|Get(acopy) _planetressourses 2))
  (bind _output_2 (Utilities|Array|Get(acopy) _playerressourses 2))
  ;[0 0.1673 1] КАЖДЫЕ 3 СЕКУНДЫ КАЧАЕТ РЕСУРСЫ ИЗ ПЛАНЕТЫ ПО ЗНАЧЕНИЮ ValueOfProduction, ЕСЛИ ЗДАНИЕ ПОДКЛЮЧЕНО К ЭЛЕКТРОСТАНЦИИ
  (if (< _output _valueofproduction)
    (Utilities|Array|SetArrayElem _playerressourses 2 (+ _output_2 _output))
    (Utilities|Array|SetArrayElem _planetressourses 2 (- _output _output))
    (else
      (Utilities|Array|SetArrayElem _playerressourses 2 (+ _output_2 (Variables|Default|GetValueOfProduction)))
      (Utilities|Array|SetArrayElem _planetressourses 2 (- _output _valueofproduction))))
  (Utilities|FlowControl|Delay 3.0)
  (if (Variables|Default|GetAlready_Work)
    (CallFunction|TickAcidExtractor)))

(event Collision|EventActorBeginOverlap
  (params (OtherActor :type Actor%20Object%20Reference)))

(event EventDestroyed
  (Widget|SetVisibility (Variables|/Game/SaveGame/GlobalGameInstance.GlobalGameInstance_C|GetBuildingInteractionOnViewport (Variables|Default|GetAsGlobalGameInstance)) "Hidden")
  ;[0 0.1566 1] СЛЕДИТ ЗА НАЖАТИЕМ НА КНОПКУ ПРОДАЖИ, ПРИ НАЖАТИИ ВОЗВРАЩАЕТ ЦЕНУ ЗДАНИЯ УМНОЖЕНУЮ НА ПРОЦЕНТ SellCost
  (bind _outactors (Actor|GetAllActorsOfClass "/Game/CameraAndControllerStuff/controllerCam.controllerCam_C"))
  (for (_array_element _array_index) (Variables|Default|GetCost)
    (Utilities|Array|SetArrayElem (Variables|/Game/CameraAndControllerStuff/controllerCam.controllerCam_C|GetPlayerRessourses (Utilities|Array|Get(acopy) _outactors)) _array_index (+ (Utilities|Array|Get(acopy) (Variables|/Game/CameraAndControllerStuff/controllerCam.controllerCam_C|GetPlayerRessourses (Utilities|Array|Get(acopy) _outactors)) _array_index) (* _array_element (Variables|Default|GetSellCost))))
    (bind _outactors_2 (Actor|GetAllActorsOfClass "BP_Acid_Extractor_C"))
    (for _array_element_2 _outactors_2
      (bind _asbuilding_interaction_widget (Utilities|Casting|CastToBuilding_Interaction_Widget (UserInterface|GetWidget (Variables|BP_Acid_Extractor_C|GetBuildingWidget _array_element_2))))
      (Default|GetBuildingInfo _asbuilding_interaction_widget "Добыча Кислот" (Variables|/Game/UI_and_Widgets/Colony_system/BuildingsWidgets/Building_Interaction_Widget.Building_Interaction_Widget_C|GetBuildingStatus _asbuilding_interaction_widget) (Utilities|Text|ToText(Integer) (- (Utilities|Array|Length _outactors_2) 1)) (Utilities|Text|ToText(Float) (* (Variables|Default|GetSellCost) 1e+02) "HalfToEven") true))))

(event EventTick
  (params (DeltaSeconds :type Float%20%28single-precision%29))
  (bind _returnvalue (Transformation|GetActorLocation))
  (bind _vector (Variables|Default|GetVector))
  (if (Variables|Default|GetAlready_Work)
    (Collision|LineTraceByChannel (Math|Vector|MakeVector (.x _returnvalue) (.y _returnvalue) (+ (.z _returnvalue) 1e+02)) (Math|Vector|MakeVector (.x _vector) (.y _vector) (+ (.z _vector) 1e+02)) "TraceTypeQuery1" false 0 "ForDuration" false "(R=0.000000,G=0.000000,B=0.000000,A=1.000000)" "(R=0.000000,G=0.000000,B=0.000000,A=1.000000)" 0.2)))

(event EventBeginPlay
  (CallFunction|SetRandomStaticMesh)
  (bind _asglobal_game_instance (Utilities|Casting|CastToGlobalGameInstance (Game|GetGameInstance)))
  (Variables|Default|SetAsGlobalGameInstance _asglobal_game_instance)
  (bind _asbuilding_interaction_widget (Utilities|Casting|CastToBuilding_Interaction_Widget (UserInterface|GetWidget (Variables|Default|GetBuildingWidget))))
  (Variables|Default|SetBuildingInteractionWidget_Ref _asbuilding_interaction_widget)
  ;[0.2434 0 1] ОТНИМАЕТ У ИГРОКА КОЛ-ВО РЕССУРСОВ НА ПОСТРОЙКУ ЗНАНИЯ СООТВЕТСТВУЮЩЕЕ ПЕРЕМЕННОЙ Cost
  (bind _ascontroller_cam (Utilities|Casting|CastTocontrollerCam (Game|GetPlayerController 0)))
  (Variables|Default|SetControllerCam_Ref _ascontroller_cam)
  (for (_array_element _array_index) (Variables|Default|GetCost)
    (Utilities|Array|SetArrayElem (Variables|/Game/CameraAndControllerStuff/controllerCam.controllerCam_C|GetPlayerRessourses (Variables|Default|GetControllerCam_Ref)) _array_index (- (Utilities|Array|Get(acopy) (Variables|/Game/CameraAndControllerStuff/controllerCam.controllerCam_C|GetPlayerRessourses (Variables|Default|GetControllerCam_Ref)) _array_index) _array_element))
    ;[0 0.1566 1] СЛЕДИТ ЗА НАЖАТИЕМ НА КНОПКУ ПРОДАЖИ, ПРИ НАЖАТИИ ВОЗВРАЩАЕТ ЦЕНУ ЗДАНИЯ УМНОЖЕНУЮ НА ПРОЦЕНТ SellCost
    (EventDispatchers|AssignSellBtnPressed (Variables|/Game/SaveGame/GlobalGameInstance.GlobalGameInstance_C|GetBuildingInteractionOnViewport (Variables|Default|GetAsGlobalGameInstance)) (delegate Custom|SellBtn_Pressed_Event))
    ;[0.6703 0 1] ПРОВЕРКА КАТЕГОРИИ ПЛАНЕТЫ ДЛЯ ПРИСВОЕНИЯ БАФФА К ПРОИЗВОТСТВУ ТОГО ИЛИ ИНОГО РЕСУРСА (ЕСЛИ НЕОБХОДИМАЯ КАТЕГОРИЯ ЕСТЬ valueOfProduction УВЕЛИЧИВАЕТСЯ, ЕСЛИ НЕТ ОСТАЕТСЯ СТАНДАРТНОЕ ЗНАЧЕНИЕ)
    (bind _asglobal_game_instance_2 (Utilities|Casting|CastToGlobalGameInstance (Game|GetGameInstance)))
    (bind _output_get (Variables|Default|SetGameInstance_Ref _asglobal_game_instance_2))
    (bind _outactors (Actor|GetAllActorsOfClass "/Game/Actors/Planets/Master_Planet_Asset.Master_Planet_Asset_C"))
    (Variables|Default|SetCurrentPlanet (Utilities|Array|Get(acopy) _outactors (Variables|/Game/SaveGame/GlobalGameInstance.GlobalGameInstance_C|GetIndexOfPlanet _output_get)))
    (bind _array_element_2 (Utilities|Array|ForEachLoopwithBreak (.categories (Variables|/Game/Actors/Planets/Master_Planet_Asset.Master_Planet_Asset_C|GetPlanetInfo (Utilities|Array|Get(acopy) _outactors (Variables|/Game/SaveGame/GlobalGameInstance.GlobalGameInstance_C|GetIndexOfPlanet _output_get)))) :!label _label)
      (:LoopBody
        (if (Utilities|Enum|Equal(Enum) _array_element_2 "NewEnumerator0")
          (Variables|Default|SetValueOfProduction 20)
          (goto _label Break)))
      (:Completed
        (bind _outactors_2 (Actor|GetAllActorsOfClass "BP_Acid_Extractor_C"))
        (for _array_element_3 _outactors_2
          (bind _asbuilding_interaction_widget_2 (Utilities|Casting|CastToBuilding_Interaction_Widget (UserInterface|GetWidget (Variables|BP_Acid_Extractor_C|GetBuildingWidget _array_element_3))))
          (Default|GetBuildingInfo _asbuilding_interaction_widget_2 "Добыча Кислот" "Требуется энергия" (Utilities|Text|ToText(Integer) (Utilities|Array|Length _outactors_2)) (Utilities|Text|ToText(Float) (* (Variables|Default|GetSellCost) 1e+02) "HalfToEven") false))))))

(fn ConstructionScript)

(fn SetRandomStaticMesh
  (bind _returnvalue (Math|Random|RandomInteger 1))
  (bind _buildmesh (Variables|Default|GetBuildMesh))
  (if (== _returnvalue 0)
    (Components|StaticMesh|SetStaticMesh _buildmesh "/Game/All_Resourses/BuildingsAndUnitsResourses/Озеро_1_/Озеро1.Озеро1")
    (elif (== _returnvalue 1)
      (Components|StaticMesh|SetStaticMesh _buildmesh "/Game/All_Resourses/BuildingsAndUnitsResourses/Озеро2_1_/Озеро3.Озеро3"))))