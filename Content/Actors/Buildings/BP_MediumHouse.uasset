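; BP_MediumHouse is a building actor that spawns two Colonist characters when play begins.
; BeginPlay calls NewSpawn twice, two seconds apart, placing each colonist at a fixed X offset and slightly above the house, then spawning its default controller.
; An unconnected chain that would print and increase the current planet's colonist population in GlobalGameInstance never runs, so the house leaves that count unchanged.
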(event Custom|new%20spawn
  (bind _returnvalue (Transformation|GetActorLocation))
  (bind _returnvalue_2 (Game|SpawnActorfromClass "/Game/Actors/Units/chuvachochki/colonist.colonist_C" (Math|Transform|MakeTransform (Math|Vector|MakeVector (+ (.x _returnvalue) 1e+03) (.y _returnvalue) (+ (.z _returnvalue) 1e+02)) "0, 0, 0" "1.000000,1.000000,1.000000") "Undefined" "MultiplyWithRoot" 0 0))
  (Pawn|SpawnDefaultController _returnvalue_2))

(event EventBeginPlay
  (CallFunction|NewSpawn)
  (Utilities|FlowControl|Delay 2.0)
  (CallFunction|NewSpawn))

(fn ConstructionScript)