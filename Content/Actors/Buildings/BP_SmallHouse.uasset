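; Small house building actor that adds colonists to the current planet when it begins play.
; BeginPlay spawns a Colonist offset along world X and slightly raised, then gives it a default controller.
; It reads the planet index from GlobalGameInstance and raises that planet's entry in the player controller's (controllerCam) ColonistsPopulation array by a fixed amount.
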(event EventBeginPlay
  (bind _returnvalue (Transformation|GetActorLocation))
  (bind _returnvalue_2 (Game|SpawnActorfromClass "/Game/Actors/Units/chuvachochki/colonist.colonist_C" (Math|Transform|MakeTransform (Math|Vector|MakeVector (+ (.x _returnvalue) 1e+03) (.y _returnvalue) (+ (.z _returnvalue) 1e+02)) "0, 0, 0" "1.000000,1.000000,1.000000") "AdjustIfPossibleButAlwaysSpawn" "MultiplyWithRoot" 0 0))
  (Pawn|SpawnDefaultController _returnvalue_2)
  (bind _asglobal_game_instance (Utilities|Casting|CastToGlobalGameInstance (Game|GetGameInstance)))
  (bind _ascontroller_cam (Utilities|Casting|CastTocontrollerCam (Game|GetPlayerController 0)))
  (bind _output_get (Variables|Default|SetCurrentPlanet (Variables|/Game/SaveGame/GlobalGameInstance.GlobalGameInstance_C|GetIndexOfPlanet _asglobal_game_instance)))
  (Utilities|Array|SetArrayElem (Variables|/Game/CameraAndControllerStuff/controllerCam.controllerCam_C|GetColonistsPopulation _ascontroller_cam) _output_get (+ (Utilities|Array|Get(acopy) (Variables|/Game/CameraAndControllerStuff/controllerCam.controllerCam_C|GetColonistsPopulation _ascontroller_cam) _output_get) 300)))

(fn ConstructionScript)