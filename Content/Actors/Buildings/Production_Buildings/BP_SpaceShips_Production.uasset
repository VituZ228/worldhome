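; Starship production building that charges the player its resource cost on BeginPlay and refunds a SellCost share when destroyed.
; Production widget events spawn a BasedShip beside the native planet for resources, or sell the building if its mesh is highlighted.
; While energy linking is active, clicks attach or detach an energy station's power, drawn each Tick as a debug trace line.
; All instances share status and count updates through their interaction widgets.
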(event OnClicked(BuildMesh)
  (params (TouchedComponent :type Primitive%20Component%20Object%20Reference) (ButtonPressed :type Key%20Structure :default "None"))
  (bind _buildinginteractionwidget_ref (Variables|Default|GetBuildingInteractionWidget_Ref))
  (bind _buildinginteractionwidget_ref_2 (Variables|Default|GetBuildingInteractionWidget_Ref))
  (bind _asglobal_game_instance (Utilities|Casting|CastToGlobalGameInstance (Game|GetGameInstance)))
  (if (Variables|/Game/SaveGame/GlobalGameInstance.GlobalGameInstance_C|GetActive_Energy _asglobal_game_instance)
    (if (Variables|Default|GetAlready_Work)
      (if (== (Variables|Default|GetId_Added_Station) (Variables|/Game/SaveGame/GlobalGameInstance.GlobalGameInstance_C|Getidofenergy _asglobal_game_instance))
        (Variables|Default|SetAlready_Work false)
        (Variables|/Game/SaveGame/GlobalGameInstance.GlobalGameInstance_C|SetActive_Energy _asglobal_game_instance true)
        (bind _outactors (Actor|GetAllActorsOfClass "/Game/Actors/Buildings/Civilian_Buildings/BP_Energy_Station.BP_Energy_Station_C"))
        (Variables|/Game/Actors/Buildings/Civilian_Buildings/BP_Energy_Station.BP_Energy_Station_C|Setenergy%20cost (Utilities|Array|Get(acopy) _outactors (Variables|/Game/SaveGame/GlobalGameInstance.GlobalGameInstance_C|Getidofenergy _asglobal_game_instance)) (+ (Variables|/Game/Actors/Buildings/Civilian_Buildings/BP_Energy_Station.BP_Energy_Station_C|Getenergy%20cost (Utilities|Array|Get(acopy) _outactors (Variables|/Game/SaveGame/GlobalGameInstance.GlobalGameInstance_C|Getidofenergy _asglobal_game_instance))) 1e+03))
        (Development|PrintString (Utilities|String|ToString(Integer) (Variables|Default|GetId_Added_Station)))
        (Development|PrintString (Utilities|String|ToString(Integer) (Variables|/Game/SaveGame/GlobalGameInstance.GlobalGameInstance_C|Getidofenergy _asglobal_game_instance)))
        (Default|GetBuildingInfo _buildinginteractionwidget_ref "Цех звездолетов" "Требуется энергия" (Variables|/Game/UI_and_Widgets/Colony_system/BuildingsWidgets/Building_Interaction_Widget.Building_Interaction_Widget_C|GetBuildingAmount _buildinginteractionwidget_ref) (Utilities|Text|ToText(Float) (* (Variables|Default|GetSellCost) 1e+02) "HalfToEven") false))
      (else
        (bind _outactors_2 (Actor|GetAllActorsOfClass "/Game/Actors/Buildings/Civilian_Buildings/BP_Energy_Station.BP_Energy_Station_C"))
        (if (not (< (Variables|/Game/Actors/Buildings/Civilian_Buildings/BP_Energy_Station.BP_Energy_Station_C|Getenergy%20cost (Utilities|Array|Get(acopy) _outactors_2 (Variables|/Game/SaveGame/GlobalGameInstance.GlobalGameInstance_C|Getidofenergy _asglobal_game_instance))) 1e+03))
          (Variables|/Game/Actors/Buildings/Civilian_Buildings/BP_Energy_Station.BP_Energy_Station_C|Setenergy%20cost (Utilities|Array|Get(acopy) _outactors_2 (Variables|/Game/SaveGame/GlobalGameInstance.GlobalGameInstance_C|Getidofenergy _asglobal_game_instance)) (- (Variables|/Game/Actors/Buildings/Civilian_Buildings/BP_Energy_Station.BP_Energy_Station_C|Getenergy%20cost (Utilities|Array|Get(acopy) _outactors_2 (Variables|/Game/SaveGame/GlobalGameInstance.GlobalGameInstance_C|Getidofenergy _asglobal_game_instance))) 1e+03))
          (Variables|Default|SetAlready_Work true)
          (Variables|Default|SetVector (Transformation|GetActorLocation (Utilities|Array|Get(acopy) _outactors_2 (Variables|/Game/SaveGame/GlobalGameInstance.GlobalGameInstance_C|Getidofenergy _asglobal_game_instance))))
          (Variables|/Game/SaveGame/GlobalGameInstance.GlobalGameInstance_C|SetActive_Energy _asglobal_game_instance false)
          (Variables|Default|SetId_Added_Station (Variables|/Game/SaveGame/GlobalGameInstance.GlobalGameInstance_C|Getidofenergy _asglobal_game_instance))
          (Default|GetBuildingInfo _buildinginteractionwidget_ref_2 "Цех звездолетов" "Активен" (Variables|/Game/UI_and_Widgets/Colony_system/BuildingsWidgets/Building_Interaction_Widget.Building_Interaction_Widget_C|GetBuildingAmount _buildinginteractionwidget_ref_2) (Utilities|Text|ToText(Float) (* (Variables|Default|GetSellCost) 1e+02) "HalfToEven") false))))))

(event Custom|SellBtn_Pressed_Event
  ;[0 0.1566 1] СЛЕДИТ ЗА НАЖАТИЕМ НА КНОПКУ ПРОДАЖИ, ПРИ НАЖАТИИ ВОЗВРАЩАЕТ ЦЕНУ ЗДАНИЯ УМНОЖЕНУЮ НА ПРОЦЕНТ SellCost
  (if (Variables|/Script/Engine.PrimitiveComponent|GetbRenderCustomDepth (Variables|Default|GetBuildMesh))
    (Actor|DestroyActor)))

(event Custom|Event_CarrierSpawn_Event
  (bind _nativeplanet (Variables|Default|GetNativePlanet))
  (bind _controllercam_ref (Variables|Default|GetControllerCam_Ref))
  (bind _controllercam_ref_2 (Variables|Default|GetControllerCam_Ref))
  (bind _returnvalue (Transformation|GetActorLocation _nativeplanet))
  (bind _playerressourses (Variables|/Game/CameraAndControllerStuff/controllerCam.controllerCam_C|GetPlayerRessourses _controllercam_ref))
  (bind _playerressourses_2 (Variables|/Game/CameraAndControllerStuff/controllerCam.controllerCam_C|GetPlayerRessourses _controllercam_ref_2))
  (bind _output (Utilities|Array|Get(acopy) _playerressourses_2))
  (bind _output_2 (Utilities|Array|Get(acopy) _playerressourses_2 1))
  ;[1 0 0.3224] СПАВНИТ БОЕВОЙ КРЕЙСЕР
  (if (or (< _output 1500) (< _output_2 3500))
    (Development|PrintString "ВАМ НЕ ХВАТАЕТ РЕССУРСОВ ЧТОБЫ СОЗДАТЬ ЭТОГО ЮНИТА")
    (else
      (Utilities|Array|SetArrayElem _playerressourses 0 (- _output 1500))
      (Utilities|Array|SetArrayElem _playerressourses 1 (- _output_2 3500))
      (Game|SpawnActorfromClass "/Game/Actors/Units/SpaceShips/BasedShip.BasedShip_C" (Math|Transform|MakeTransform (+ (Math|Vector|MakeVector (.x _returnvalue) (.y _returnvalue) -267.0) (Math|Vector|MakeVector (+ (* (Variables|/Game/Actors/Planets/Master_Planet_Asset.Master_Planet_Asset_C|GetRangeInKm _nativeplanet) 1e+03) 2e+03) 0.0 0.0)) "0, 0, 0" "1.000000,1.000000,1.000000") "AdjustIfPossibleButAlwaysSpawn" "MultiplyWithRoot" 0 "NewEnumerator5" 0 true 0))))

(event Custom|StationPlugBtn_Pressed_Event
  ;[0 0.1566 1] СЛЕДИТ ЗА НАЖАТИЕМ НА КНОПКУ ПРОДАЖИ, ПРИ НАЖАТИИ ВОЗВРАЩАЕТ ЦЕНУ ЗДАНИЯ УМНОЖЕНУЮ НА ПРОЦЕНТ SellCost
)

(event EventBeginPlay
  (bind _asglobal_game_instance (Utilities|Casting|CastToGlobalGameInstance (Game|GetGameInstance)))
  (Variables|Default|SetAs%20Global%20Game%20Instance _asglobal_game_instance)
  (bind _outactors (Actor|GetAllActorsOfClass "/Game/Actors/Planets/Master_Planet_Asset.Master_Planet_Asset_C"))
  (Variables|Default|SetNativePlanet (Utilities|Array|Get(acopy) _outactors (Variables|/Game/SaveGame/GlobalGameInstance.GlobalGameInstance_C|GetIndexOfPlanet _asglobal_game_instance)))
  (bind _asspace_ships_production_widget (Utilities|Casting|CastToSpaceShips_Production_Widget (UserInterface|GetWidget (Variables|Default|GetBuildingWidget))))
  (Variables|Default|SetAs%20Space%20Ships%20Production%20Widget _asspace_ships_production_widget)
  (Variables|Default|SetBuildingInteractionWidget_Ref (Variables|/Game/UI_and_Widgets/Colony_system/BuildingsWidgets/SpaceShips_Production_Widget.SpaceShips_Production_Widget_C|GetBuilding_Interaction_Widget _asspace_ships_production_widget))
  ;[0.2434 0 1] ОТНИМАЕТ У ИГРОКА КОЛ-ВО РЕССУРСОВ НА ПОСТРОЙКУ ЗНАНИЯ СООТВЕТСТВУЮЩЕЕ ПЕРЕМЕННОЙ Cost
  (bind _ascontroller_cam (Utilities|Casting|CastTocontrollerCam (Game|GetPlayerController 0)))
  (Variables|Default|SetControllerCam_Ref _ascontroller_cam)
  (for (_array_element _array_index) (Variables|Default|GetCost)
    (Utilities|Array|SetArrayElem (Variables|/Game/CameraAndControllerStuff/controllerCam.controllerCam_C|GetPlayerRessourses (Variables|Default|GetControllerCam_Ref)) _array_index (- (Utilities|Array|Get(acopy) (Variables|/Game/CameraAndControllerStuff/controllerCam.controllerCam_C|GetPlayerRessourses (Variables|Default|GetControllerCam_Ref)) _array_index) _array_element))
    ;[1 0 0.3224] СПАВНИТ БОЕВОЙ КРЕЙСЕР
    (EventDispatchers|AssignEventCarrierSpawn (Variables|/Game/SaveGame/GlobalGameInstance.GlobalGameInstance_C|GetShipsProductionWidgetOnViewport (Variables|Default|GetAs%20Global%20Game%20Instance)) (delegate Custom|Event_CarrierSpawn_Event))
    ;[0 0.1566 1] СЛЕДИТ ЗА НАЖАТИЕМ НА КНОПКУ ПРОДАЖИ, ПРИ НАЖАТИИ ВОЗВРАЩАЕТ ЦЕНУ ЗДАНИЯ УМНОЖЕНУЮ НА ПРОЦЕНТ SellCost
    (EventDispatchers|AssignSellBtnPressed (Variables|/Game/UI_and_Widgets/Colony_system/BuildingsWidgets/SpaceShips_Production_Widget.SpaceShips_Production_Widget_C|GetBuilding_Interaction_Widget (Variables|/Game/SaveGame/GlobalGameInstance.GlobalGameInstance_C|GetShipsProductionWidgetOnViewport (Variables|Default|GetAs%20Global%20Game%20Instance))) (delegate Custom|SellBtn_Pressed_Event))
    (EventDispatchers|AssignStationPlugBtnPressed (Variables|/Game/UI_and_Widgets/Colony_system/BuildingsWidgets/SpaceShips_Production_Widget.SpaceShips_Production_Widget_C|GetBuilding_Interaction_Widget (Variables|/Game/SaveGame/GlobalGameInstance.GlobalGameInstance_C|GetShipsProductionWidgetOnViewport (Variables|Default|GetAs%20Global%20Game%20Instance))) (delegate Custom|StationPlugBtn_Pressed_Event))
    (bind _outactors_2 (Actor|GetAllActorsOfClass "BP_SpaceShips_Production_C"))
    (for _array_element_2 _outactors_2
      (Default|GetBuildingInfo (Variables|BP_SpaceShips_Production_C|GetBuildingInteractionWidget_Ref _array_element_2) "Цех звездолетов" "Требуется энергия" (Utilities|Text|ToText(Integer) (Utilities|Array|Length _outactors_2)) (Utilities|Text|ToText(Float) (* (Variables|Default|GetSellCost) 1e+02) "HalfToEven") false))))

(event Collision|EventActorBeginOverlap
  (params (OtherActor :type Actor%20Object%20Reference)))

(event EventTick
  (params (DeltaSeconds :type Float%20%28single-precision%29))
  (bind _returnvalue (Transformation|GetActorLocation))
  (bind _vector (Variables|Default|GetVector))
  (if (Variables|Default|GetAlready_Work)
    (Collision|LineTraceByChannel (Math|Vector|MakeVector (.x _returnvalue) (.y _returnvalue) (+ (.z _returnvalue) 1e+02)) (Math|Vector|MakeVector (.x _vector) (.y _vector) (+ (.z _vector) 1e+02)) "TraceTypeQuery1" false 0 "ForDuration" false "(R=0.000000,G=0.000000,B=0.000000,A=1.000000)" "(R=0.000000,G=0.000000,B=0.000000,A=1.000000)" 0.2)))

(event EventDestroyed
  (Widget|SetVisibility (Variables|/Game/UI_and_Widgets/Colony_system/BuildingsWidgets/SpaceShips_Production_Widget.SpaceShips_Production_Widget_C|GetBuilding_Interaction_Widget (Variables|/Game/SaveGame/GlobalGameInstance.GlobalGameInstance_C|GetShipsProductionWidgetOnViewport (Variables|Default|GetAs%20Global%20Game%20Instance))) "Hidden")
  ;[0 0.1566 1] СЛЕДИТ ЗА НАЖАТИЕМ НА КНОПКУ ПРОДАЖИ, ПРИ НАЖАТИИ ВОЗВРАЩАЕТ ЦЕНУ ЗДАНИЯ УМНОЖЕНУЮ НА ПРОЦЕНТ SellCost
  (bind _outactors (Actor|GetAllActorsOfClass "/Game/CameraAndControllerStuff/controllerCam.controllerCam_C"))
  (for (_array_element _array_index) (Variables|Default|GetCost)
    (Utilities|Array|SetArrayElem (Variables|/Game/CameraAndControllerStuff/controllerCam.controllerCam_C|GetPlayerRessourses (Utilities|Array|Get(acopy) _outactors)) _array_index (+ (Utilities|Array|Get(acopy) (Variables|/Game/CameraAndControllerStuff/controllerCam.controllerCam_C|GetPlayerRessourses (Utilities|Array|Get(acopy) _outactors)) _array_index) (* _array_element (Variables|Default|GetSellCost))))
    (bind _outactors_2 (Actor|GetAllActorsOfClass "BP_SpaceShips_Production_C"))
    (for _array_element_2 _outactors_2
      (Default|GetBuildingInfo (Variables|BP_SpaceShips_Production_C|GetBuildingInteractionWidget_Ref _array_element_2) "Цех звездолетов" (Variables|/Game/UI_and_Widgets/Colony_system/BuildingsWidgets/Building_Interaction_Widget.Building_Interaction_Widget_C|GetBuildingStatus (Variables|BP_SpaceShips_Production_C|GetBuildingInteractionWidget_Ref _array_element_2)) (Utilities|Text|ToText(Integer) (- (Utilities|Array|Length _outactors_2) 1)) (Utilities|Text|ToText(Float) (* (Variables|Default|GetSellCost) 1e+02) "HalfToEven") false))))

(fn ConstructionScript)