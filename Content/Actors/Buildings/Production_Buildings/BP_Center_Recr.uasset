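; Recruitment center building that converts a planet's colonists into SvoPopulation at a food cost while powered.
; On placement it deducts build cost and AutoPrisos seeks the nearest in-range energy station or working tower, reserving energy and workers.
; Widget events drive recruitment, power toggling via NullAllStation/AutoPrisos, and selling with a partial refund.
; Status is mirrored to the viewport widget, and a per-tick debug line trace draws the power link.
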(event OnClicked(BuildMesh)
  (params (TouchedComponent :type Primitive%20Component%20Object%20Reference) (ButtonPressed :type Key%20Structure :default "None")))

(event Custom|porn
  (bind _as_global_game_instance (Variables|Default|GetAs%20Global%20Game%20Instance))
  (bind _as_global_game_instance_2 (Variables|Default|GetAs%20Global%20Game%20Instance))
  (bind _controllercam_ref (Variables|Default|GetControllerCam_Ref))
  (bind _controllercam_ref_2 (Variables|Default|GetControllerCam_Ref))
  (bind _colonistspopulation (Variables|/Game/CameraAndControllerStuff/controllerCam.controllerCam_C|GetColonistsPopulation _controllercam_ref_2))
  (bind _indexofplanet (Variables|/Game/SaveGame/GlobalGameInstance.GlobalGameInstance_C|GetIndexOfPlanet _as_global_game_instance))
  (bind _svopopulation (Variables|/Game/CameraAndControllerStuff/controllerCam.controllerCam_C|GetSvoPopulation _controllercam_ref_2))
  (bind _coloniesfood (Variables|/Game/CameraAndControllerStuff/controllerCam.controllerCam_C|GetColoniesFood _controllercam_ref))
  (bind _centerrecrutonviewport (Variables|/Game/SaveGame/GlobalGameInstance.GlobalGameInstance_C|GetCenterRecrutOnViewport _as_global_game_instance_2))
  (bind _output (Utilities|Array|Get(acopy) _colonistspopulation _indexofplanet))
  (bind _output_2 (Utilities|Array|Get(acopy) _coloniesfood _indexofplanet))
  (bind _raremetcost_textblock (Variables|/Game/UI_and_Widgets/Colony_and_units_system/BuildingsWidgets/Center_Widget.Center_Widget_C|GetRareMetCost_TextBlock _centerrecrutonviewport))
  (bind _returnvalue (Class|TextBlock|GetText _raremetcost_textblock))
  (bind _returnvalue_2 (Utilities|String|ToString(Text) _returnvalue))
  (bind _returnvalue_3 (Math|Conversions|ToInteger(Byte) _returnvalue_2))
  (if (Variables|Default|GetBuildingIsDoneForWork)
    (if (> (Class|Slider|GetValue (Variables|/Game/UI_and_Widgets/Colony_and_units_system/BuildingsWidgets/Center_Widget.Center_Widget_C|GetAmountSlider _centerrecrutonviewport)) _output)
      (Development|PrintString "недостаточно колонистов")
      (elif (> _returnvalue_3 _output_2)
        (Development|PrintString "недостаточно еды")
        (else
          (bind _output_get (Variables|Default|SetcolonistToSvo (Math|Conversions|ToInteger(Byte) (Utilities|String|ToString(Text) (Default|GetAmountTextBlockText _centerrecrutonviewport)))))
          (Utilities|Array|SetArrayElem _colonistspopulation _indexofplanet (- _output _output_get))
          (Utilities|Array|SetArrayElem _svopopulation _indexofplanet (+ (Utilities|Array|Get(acopy) _svopopulation _indexofplanet) _output_get))
          (Utilities|Array|SetArrayElem _coloniesfood _indexofplanet (- _output_2 _returnvalue_3)))))
    (else
      (Development|PrintString "Центр не включен"))))

(event Custom|StationPlugBtn_Pressed_Event
  ;[0 0.1566 1] СЛЕДИТ ЗА НАЖАТИЕМ НА КНОПКУ ПРОДАЖИ, ПРИ НАЖАТИИ ВОЗВРАЩАЕТ ЦЕНУ ЗДАНИЯ УМНОЖЕНУЮ НА ПРОЦЕНТ SellCost
)

(event Custom|porn2
  ;[0 0.1566 1] СЛЕДИТ ЗА НАЖАТИЕМ НА КНОПКУ ПРОДАЖИ, ПРИ НАЖАТИИ ВОЗВРАЩАЕТ ЦЕНУ ЗДАНИЯ УМНОЖЕНУЮ НА ПРОЦЕНТ SellCost
  (if (Variables|/Script/Engine.PrimitiveComponent|GetbRenderCustomDepth (Variables|Default|GetBuildMesh))
    (Actor|DestroyActor)))

(event Custom|CustomEvent
  (if (Variables|/Script/Engine.PrimitiveComponent|GetbRenderCustomDepth (Variables|Default|GetBuildMesh))
    (if (Variables|Default|GetBuildingIsDoneForWork)
      (CallFunction|NullAllStation)
      (else
        (CallFunction|AutoPrisos)))))

(event EventBeginPlay
  (bind _asglobal_game_instance (Utilities|Casting|CastToGlobalGameInstance (Game|GetGameInstance)))
  (Variables|Default|SetAs%20Global%20Game%20Instance _asglobal_game_instance)
  (bind _outactors (Actor|GetAllActorsOfClass "/Game/Actors/Planets/Master_Planet_BigVer_Asset.Master_Planet_BigVer_Asset_C"))
  (Variables|Default|SetWorldOrigin (Transformation|GetActorLocation (Utilities|Array|Get(acopy) _outactors (Variables|/Game/SaveGame/GlobalGameInstance.GlobalGameInstance_C|GetIndexOfPlanet (Variables|Default|GetAs%20Global%20Game%20Instance)))))
  (bind _outactors_2 (Actor|GetAllActorsOfClass "/Game/Actors/Planets/Master_Planet_Asset.Master_Planet_Asset_C"))
  (Variables|Default|SetNativePlanet (Utilities|Array|Get(acopy) _outactors_2 (Variables|/Game/SaveGame/GlobalGameInstance.GlobalGameInstance_C|GetIndexOfPlanet _asglobal_game_instance)))
  (if (not (Utilities|Enum|Equal(Enum) (Utilities|String|LeftChop (Utilities|GetObjectName (Components|GetOwner)) 4) "BP_MainBot"))
    (bind _ascenter_widget (Utilities|Casting|CastToCenter_Widget (UserInterface|GetWidget (Variables|Default|GetBuildingWidget))))
    (Variables|Default|Setcenter%20widget%20ref _ascenter_widget)
    (Variables|Default|SetBuildingInteractionWidget_Ref (Variables|/Game/UI_and_Widgets/Colony_and_units_system/BuildingsWidgets/Center_Widget.Center_Widget_C|GetBuilding_Interaction_Widget _ascenter_widget))
    ;[0.2434 0 1] ОТНИМАЕТ У ИГРОКА КОЛ-ВО РЕССУРСОВ НА ПОСТРОЙКУ ЗНАНИЯ СООТВЕТСТВУЮЩЕЕ ПЕРЕМЕННОЙ Cost
    (CallFunction|AutoPrisos)
    (bind _ascontroller_cam (Utilities|Casting|CastTocontrollerCam (Game|GetPlayerController 0)))
    (Variables|Default|SetControllerCam_Ref _ascontroller_cam)
    (for (_array_element _array_index) (Variables|Default|GetCost)
      (Utilities|Array|SetArrayElem (Variables|/Game/CameraAndControllerStuff/controllerCam.controllerCam_C|GetPlayerRessourses (Variables|Default|GetControllerCam_Ref)) _array_index (- (Utilities|Array|Get(acopy) (Variables|/Game/CameraAndControllerStuff/controllerCam.controllerCam_C|GetPlayerRessourses (Variables|Default|GetControllerCam_Ref)) _array_index) _array_element))
      (EventDispatchers|BindEventtoStationPlugBtnPressed (Variables|/Game/UI_and_Widgets/Colony_and_units_system/BuildingsWidgets/SpaceShips_Production_Widget.SpaceShips_Production_Widget_C|GetBuilding_Interaction_Widget (Variables|/Game/SaveGame/GlobalGameInstance.GlobalGameInstance_C|GetShipsProductionWidgetOnViewport (Variables|Default|GetAs%20Global%20Game%20Instance))) (delegate Custom|CustomEvent))
      ;[0 0.1566 1] СЛЕДИТ ЗА НАЖАТИЕМ НА КНОПКУ ПРОДАЖИ, ПРИ НАЖАТИИ ВОЗВРАЩАЕТ ЦЕНУ ЗДАНИЯ УМНОЖЕНУЮ НА ПРОЦЕНТ SellCost
      (EventDispatchers|BindEventtoSellBtnPressed (Variables|/Game/UI_and_Widgets/Colony_and_units_system/BuildingsWidgets/Center_Widget.Center_Widget_C|GetBuilding_Interaction_Widget (Variables|/Game/SaveGame/GlobalGameInstance.GlobalGameInstance_C|GetCenterRecrutOnViewport (Variables|Default|GetAs%20Global%20Game%20Instance))) (delegate Custom|porn2))
      (EventDispatchers|BindEventtoStartTravelPressed (Variables|/Game/SaveGame/GlobalGameInstance.GlobalGameInstance_C|GetCenterRecrutOnViewport (Variables|Default|GetAs%20Global%20Game%20Instance)) (delegate Custom|porn))
      (bind _outactors_3 (Actor|GetAllActorsOfClass "BP_Center_Recr_C"))
      (for _array_element_2 _outactors_3
        (Default|GetBuildingInfo (Variables|BP_Center_Recr_C|GetBuildingInteractionWidget_Ref _array_element_2) (Variables|/Game/UI_and_Widgets/Colony_and_units_system/BuildingsWidgets/Building_Interaction_Widget.Building_Interaction_Widget_C|GetBuildingName (Variables|BP_Center_Recr_C|GetBuildingInteractionWidget_Ref _array_element_2)) (Variables|/Game/UI_and_Widgets/Colony_and_units_system/BuildingsWidgets/Building_Interaction_Widget.Building_Interaction_Widget_C|GetBuildingStatus (Variables|BP_Center_Recr_C|GetBuildingInteractionWidget_Ref _array_element_2)) (Utilities|Text|ToText(Integer) (Utilities|Array|Length _outactors_3)) (Variables|/Game/UI_and_Widgets/Colony_and_units_system/BuildingsWidgets/Building_Interaction_Widget.Building_Interaction_Widget_C|GetBuildingSellCost (Variables|BP_Center_Recr_C|GetBuildingInteractionWidget_Ref _array_element_2)) false)))))

(event Collision|EventActorBeginOverlap
  (params (OtherActor :type Actor%20Object%20Reference)))

(event EventTick
  (params (DeltaSeconds :type Float%20%28single-precision%29))
  (CallFunction|LineTrace))

(event EventDestroyed
  ;[0 0.1566 1] СЛЕДИТ ЗА НАЖАТИЕМ НА КНОПКУ ПРОДАЖИ, ПРИ НАЖАТИИ ВОЗВРАЩАЕТ ЦЕНУ ЗДАНИЯ УМНОЖЕНУЮ НА ПРОЦЕНТ SellCost
  (Effects|SpawnEmitteratLocation "/Game/VFX_Toolkit_V1/ParticleSystems/356Days/Par_LuCoins.Par_LuCoins" (Transformation|GetActorLocation) (Transformation|GetActorRotation) "50.000000,50.000000,50.000000")
  (Widget|SetVisibility (Variables|/Game/SaveGame/GlobalGameInstance.GlobalGameInstance_C|GetShipsProductionWidgetOnViewport (Variables|Default|GetAs%20Global%20Game%20Instance)) "Hidden")
  (bind _outactors (Actor|GetAllActorsOfClass "/Game/CameraAndControllerStuff/controllerCam.controllerCam_C"))
  (for (_array_element _array_index) (Variables|Default|GetCost)
    (Utilities|Array|SetArrayElem (Variables|/Game/CameraAndControllerStuff/controllerCam.controllerCam_C|GetPlayerRessourses (Utilities|Array|Get(acopy) _outactors)) _array_index (+ (Utilities|Array|Get(acopy) (Variables|/Game/CameraAndControllerStuff/controllerCam.controllerCam_C|GetPlayerRessourses (Utilities|Array|Get(acopy) _outactors)) _array_index) (* _array_element (Variables|Default|GetSellCost))))
    (bind _outactors_2 (Actor|GetAllActorsOfClass "BP_Center_Recr_C"))
    (for _array_element_2 _outactors_2
      (Default|GetBuildingInfo (Variables|BP_Center_Recr_C|GetBuildingInteractionWidget_Ref _array_element_2) (Variables|/Game/UI_and_Widgets/Colony_and_units_system/BuildingsWidgets/Building_Interaction_Widget.Building_Interaction_Widget_C|GetBuildingName (Variables|BP_Center_Recr_C|GetBuildingInteractionWidget_Ref _array_element_2)) (Variables|/Game/UI_and_Widgets/Colony_and_units_system/BuildingsWidgets/Building_Interaction_Widget.Building_Interaction_Widget_C|GetBuildingStatus (Variables|BP_Center_Recr_C|GetBuildingInteractionWidget_Ref _array_element_2)) (Utilities|Text|ToText(Integer) (- (Utilities|Array|Length _outactors_2) 1)) (Variables|/Game/UI_and_Widgets/Colony_and_units_system/BuildingsWidgets/Building_Interaction_Widget.Building_Interaction_Widget_C|GetBuildingSellCost (Variables|BP_Center_Recr_C|GetBuildingInteractionWidget_Ref _array_element_2)) false))))

(fn ConstructionScript)

(fn AutoPrisos
  (bind _as_global_game_instance (Variables|Default|GetAs%20Global%20Game%20Instance))
  (bind _indexofplanet (Variables|/Game/SaveGame/GlobalGameInstance.GlobalGameInstance_C|GetIndexOfPlanet _as_global_game_instance))
  (bind _outactors (Actor|GetAllActorsOfClass "/Game/Actors/Buildings/Civilian_Buildings/BP_Energy_Station.BP_Energy_Station_C"))
  (for _array_element _outactors
    (if (<= (Math|Vector|Distance(Vector) (Transformation|GetActorLocation) (Transformation|GetActorLocation _array_element)) (Variables|/Game/SaveGame/GlobalGameInstance.GlobalGameInstance_C|Getrange%20of%20electric (Variables|Default|GetAs%20Global%20Game%20Instance)))
      (if (<= (Math|Vector|Distance(Vector) (Transformation|GetActorLocation) (Transformation|GetActorLocation _array_element)) (Variables|Default|Getmin%20distance))
        (Variables|Default|Setmin%20distance (Math|Vector|Distance(Vector) (Transformation|GetActorLocation) (Transformation|GetActorLocation _array_element)))
        (Variables|Default|Setbp_energy%20station _array_element)
        (Variables|Default|SetGoNextOrNo true))
      (else
        (Development|PrintString "электростанция слишком далеко"))))
  (bind _outactors_2 (Actor|GetAllActorsOfClass "/Game/Actors/Buildings/Civilian_Buildings/BP_EnergyTower.BP_EnergyTower_C"))
  (for _array_element_2 _outactors_2
    (if (Variables|/Game/Actors/Buildings/Civilian_Buildings/BP_EnergyTower.BP_EnergyTower_C|Getalready_work _array_element_2)
      (if (<= (Math|Vector|Distance(Vector) (Transformation|GetActorLocation) (Transformation|GetActorLocation _array_element_2)) (Variables|/Game/SaveGame/GlobalGameInstance.GlobalGameInstance_C|Getrange%20of%20electric (Variables|Default|GetAs%20Global%20Game%20Instance)))
        (if (<= (Math|Vector|Distance(Vector) (Transformation|GetActorLocation) (Transformation|GetActorLocation _array_element_2)) (Variables|Default|Getmin%20distance))
          (Variables|Default|Setmin%20distance (Math|Vector|Distance(Vector) (Transformation|GetActorLocation) (Transformation|GetActorLocation _array_element_2)))
          (Variables|Default|Setbp_energy%20tower _array_element_2)
          (Variables|Default|Setprisoska%20na%20tavek%20ili%20net true)
          (Variables|Default|SetGoNextOrNo true)))))
  (if (Variables|Default|GetGoNextOrNo)
    (bind _ascontroller_cam (Utilities|Casting|CastTocontrollerCam (Game|GetPlayerController 0)))
    (if (<= (Variables|Default|GetHowMuchColonistNeedToWork) (Utilities|Array|Get(acopy) (Variables|/Game/CameraAndControllerStuff/controllerCam.controllerCam_C|GetColonistsPopulation _ascontroller_cam) (Variables|/Game/SaveGame/GlobalGameInstance.GlobalGameInstance_C|GetIndexOfPlanet (Variables|Default|GetAs%20Global%20Game%20Instance))))
      (if (Variables|Default|Getprisoska%20na%20tavek%20ili%20net)
        (Variables|Default|Setint%20for%20delite (- (Variables|/Game/Actors/Buildings/Civilian_Buildings/BP_EnergyTower.BP_EnergyTower_C|Getkakoq%20to%20int (Variables|Default|Getbp_energy%20tower)) 100000))
        (bind _outactors_3 (Actor|GetAllActorsOfClass "/Game/Actors/Buildings/Civilian_Buildings/BP_Energy_Station.BP_Energy_Station_C"))
        (if (not (< (Variables|/Game/Actors/Buildings/Civilian_Buildings/BP_Energy_Station.BP_Energy_Station_C|Getenergy%20cost (Utilities|Array|Get(acopy) _outactors_3 (Variables|/Game/Actors/Buildings/Civilian_Buildings/BP_EnergyTower.BP_EnergyTower_C|Getid%20of%20added%20station (Variables|Default|Getbp_energy%20tower)))) (Variables|Default|Getbuilding%20cost)))
          (Variables|/Game/Actors/Buildings/Civilian_Buildings/BP_Energy_Station.BP_Energy_Station_C|Setenergy%20cost (Utilities|Array|Get(acopy) _outactors_3 (Variables|/Game/Actors/Buildings/Civilian_Buildings/BP_EnergyTower.BP_EnergyTower_C|Getid%20of%20added%20station (Variables|Default|Getbp_energy%20tower))) (- (Variables|/Game/Actors/Buildings/Civilian_Buildings/BP_Energy_Station.BP_Energy_Station_C|Getenergy%20cost (Utilities|Array|Get(acopy) _outactors_3 (Variables|/Game/Actors/Buildings/Civilian_Buildings/BP_EnergyTower.BP_EnergyTower_C|Getid%20of%20added%20station (Variables|Default|Getbp_energy%20tower)))) (Variables|Default|Getbuilding%20cost)))
          (Variables|Default|Setvector (Transformation|GetActorLocation (Variables|Default|Getbp_energy%20tower)))
          (Variables|Default|Setid_added_station (+ (Math|Conversions|ToInteger(Byte) (Utilities|String|GetSubstring (Utilities|GetObjectName (Variables|Default|Getbp_energy%20tower)) 17 3)) 100000))
          (bind _ascontroller_cam_2 (Utilities|Casting|CastTocontrollerCam (Game|GetPlayerController 0) :!label _label))
          (bind _outactors_4 (Actor|GetAllActorsOfClass "/Game/Actors/Planets/Master_Planet_Asset.Master_Planet_Asset_C"))
          (Variables|/Game/Actors/Planets/Master_Planet_Asset.Master_Planet_Asset_C|SetLimitOfPopulation (Utilities|Array|Get(acopy) _outactors_4 _indexofplanet) (- (Variables|/Game/Actors/Planets/Master_Planet_Asset.Master_Planet_Asset_C|GetLimitOfPopulation (Utilities|Array|Get(acopy) _outactors_4 _indexofplanet)) (Variables|Default|GetHowMuchColonistNeedToWork)))
          (Utilities|Array|SetArrayElem (Variables|/Game/CameraAndControllerStuff/controllerCam.controllerCam_C|GetColonistsPopulation _ascontroller_cam_2) _indexofplanet (- (Utilities|Array|Get(acopy) (Variables|/Game/CameraAndControllerStuff/controllerCam.controllerCam_C|GetColonistsPopulation _ascontroller_cam_2) _indexofplanet) (Variables|Default|GetHowMuchColonistNeedToWork)))
          (Variables|Default|SetBuildingIsDoneForWork true)
          (bind _outactors_5 (Actor|GetAllActorsOfClass "BP_Center_Recr_C"))
          (Rendering|Components|TextRender|SetText (Variables|/Game/UI_and_Widgets/Colony_and_units_system/BuildingsWidgets/Building_Interaction_Widget.Building_Interaction_Widget_C|GetTextBlock_270 (Variables|/Game/UI_and_Widgets/Colony_and_units_system/BuildingsWidgets/Center_Widget.Center_Widget_C|GetBuilding_Interaction_Widget (Variables|Default|Getcenter%20widget%20ref))) "Отключить")
          (Default|GetBuildingInfo (Variables|/Game/UI_and_Widgets/Colony_and_units_system/BuildingsWidgets/Center_Widget.Center_Widget_C|GetBuilding_Interaction_Widget (Variables|Default|Getcenter%20widget%20ref)) "Центр Рекрутировки" "Здание работает" (Utilities|Text|ToText(Integer) (Utilities|Array|Length _outactors_5)) (Utilities|Text|ToText(Float) (* (Variables|Default|GetSellCost) 1e+02) "HalfToEven") false)
          (CallFunction|LocalWidgettoGlobal))
        (elif (not (< (Variables|/Game/Actors/Buildings/Civilian_Buildings/BP_Energy_Station.BP_Energy_Station_C|Getenergy%20cost (Variables|Default|Getbp_energy%20station)) (Variables|Default|Getbuilding%20cost)))
          (Variables|/Game/Actors/Buildings/Civilian_Buildings/BP_Energy_Station.BP_Energy_Station_C|Setenergy%20cost (Variables|Default|Getbp_energy%20station) (- (Variables|/Game/Actors/Buildings/Civilian_Buildings/BP_Energy_Station.BP_Energy_Station_C|Getenergy%20cost (Variables|Default|Getbp_energy%20station)) (Variables|Default|Getbuilding%20cost)))
          (Variables|Default|Setvector (Transformation|GetActorLocation (Variables|Default|Getbp_energy%20station)))
          (Variables|Default|Setid_added_station (Math|Conversions|ToInteger(Byte) (Utilities|String|GetSubstring (Utilities|GetObjectName (Variables|Default|Getbp_energy%20station)) 20 3)))
          (goto _label)))
      (else
        (Development|PrintString "недостаточно рабочих")))
    (else
      (Development|PrintString "поблизости нет электростанций"))))

(fn LineTrace
  (if (Variables|Default|GetBuildingIsDoneForWork)
    (Collision|LineTraceByChannel (+ (* (Math|Vector|GetUnitDirection(Vector) (Variables|Default|GetWorldOrigin) (Variables|Default|Getvector)) "1000.000000,1000.000000,1000.000000") (Variables|Default|Getvector)) (+ (* (Math|Vector|GetUnitDirection(Vector) (Variables|Default|GetWorldOrigin) (Transformation|GetActorLocation)) "1000.000000,1000.000000,1000.000000") (Transformation|GetActorLocation)) "TraceTypeQuery1" false 0 "ForDuration" false "(R=0.000000,G=0.000000,B=0.000000,A=1.000000)" "(R=0.000000,G=0.000000,B=0.000000,A=1.000000)" 0.2)))

(fn NullAllStation
  (bind _as_global_game_instance (Variables|Default|GetAs%20Global%20Game%20Instance))
  (bind _as_global_game_instance_2 (Variables|Default|GetAs%20Global%20Game%20Instance))
  (bind _idofenergy (Variables|/Game/SaveGame/GlobalGameInstance.GlobalGameInstance_C|Getidofenergy _as_global_game_instance_2))
  (bind _indexofplanet (Variables|/Game/SaveGame/GlobalGameInstance.GlobalGameInstance_C|GetIndexOfPlanet _as_global_game_instance))
  (if (> (Variables|/Game/SaveGame/GlobalGameInstance.GlobalGameInstance_C|Getidofenergy (Variables|Default|GetAs%20Global%20Game%20Instance)) 99999)
    (bind _outactors (Actor|GetAllActorsOfClass "/Game/Actors/Buildings/Civilian_Buildings/BP_EnergyTower.BP_EnergyTower_C"))
    (bind _outactors_2 (Actor|GetAllActorsOfClass "/Game/Actors/Buildings/Civilian_Buildings/BP_Energy_Station.BP_Energy_Station_C"))
    (Variables|/Game/Actors/Buildings/Civilian_Buildings/BP_Energy_Station.BP_Energy_Station_C|Setenergy%20cost (Utilities|Array|Get(acopy) _outactors_2 (Variables|/Game/Actors/Buildings/Civilian_Buildings/BP_EnergyTower.BP_EnergyTower_C|Getid%20of%20added%20station (Utilities|Array|Get(acopy) _outactors (- _idofenergy 100000)))) (+ (Variables|Default|Getbuilding%20cost) (Variables|/Game/Actors/Buildings/Civilian_Buildings/BP_Energy_Station.BP_Energy_Station_C|Getenergy%20cost (Utilities|Array|Get(acopy) _outactors_2 (Variables|/Game/Actors/Buildings/Civilian_Buildings/BP_EnergyTower.BP_EnergyTower_C|Getid%20of%20added%20station (Utilities|Array|Get(acopy) _outactors (- _idofenergy 100000)))))))
    (else
      (bind _outactors_3 (Actor|GetAllActorsOfClass "/Game/Actors/Buildings/Civilian_Buildings/BP_Energy_Station.BP_Energy_Station_C"))
      (Variables|/Game/Actors/Buildings/Civilian_Buildings/BP_Energy_Station.BP_Energy_Station_C|Setenergy%20cost (Utilities|Array|Get(acopy) _outactors_3 _idofenergy) (+ (Variables|/Game/Actors/Buildings/Civilian_Buildings/BP_Energy_Station.BP_Energy_Station_C|Getenergy%20cost (Utilities|Array|Get(acopy) _outactors_3 _idofenergy)) (Variables|Default|Getbuilding%20cost)))))
  (Variables|Default|SetBuildingIsDoneForWork false)
  (bind _ascontroller_cam (Utilities|Casting|CastTocontrollerCam (Game|GetPlayerController 0)))
  (bind _outactors_4 (Actor|GetAllActorsOfClass "/Game/Actors/Planets/Master_Planet_Asset.Master_Planet_Asset_C"))
  (Variables|/Game/Actors/Planets/Master_Planet_Asset.Master_Planet_Asset_C|SetLimitOfPopulation (Utilities|Array|Get(acopy) _outactors_4) (+ (Variables|/Game/Actors/Planets/Master_Planet_Asset.Master_Planet_Asset_C|GetLimitOfPopulation (Utilities|Array|Get(acopy) _outactors_4)) (Variables|Default|GetHowMuchColonistNeedToWork)))
  (Utilities|Array|SetArrayElem (Variables|/Game/CameraAndControllerStuff/controllerCam.controllerCam_C|GetColonistsPopulation _ascontroller_cam) _indexofplanet (+ (Utilities|Array|Get(acopy) (Variables|/Game/CameraAndControllerStuff/controllerCam.controllerCam_C|GetColonistsPopulation _ascontroller_cam) _indexofplanet) (Variables|Default|GetHowMuchColonistNeedToWork)))
  (Rendering|Components|TextRender|SetText (Variables|/Game/UI_and_Widgets/Colony_and_units_system/BuildingsWidgets/Building_Interaction_Widget.Building_Interaction_Widget_C|GetTextBlock_270 (Variables|/Game/UI_and_Widgets/Colony_and_units_system/BuildingsWidgets/Center_Widget.Center_Widget_C|GetBuilding_Interaction_Widget (Variables|Default|Getcenter%20widget%20ref))) "Подключить")
  (bind _outactors_5 (Actor|GetAllActorsOfClass "BP_Center_Recr_C"))
  (Default|GetBuildingInfo (Variables|/Game/UI_and_Widgets/Colony_and_units_system/BuildingsWidgets/Center_Widget.Center_Widget_C|GetBuilding_Interaction_Widget (Variables|Default|Getcenter%20widget%20ref)) "Центр Рекрутировки" "Неактивен" (Utilities|Text|ToText(Integer) (Utilities|Array|Length _outactors_5)) (Utilities|Text|ToText(Float) (* (Variables|Default|GetSellCost) 1e+02) "HalfToEven") false)
  (CallFunction|LocalWidgettoGlobal))

(fn LocalWidgettoGlobal
  (bind _center_widget_ref (Variables|Default|Getcenter%20widget%20ref))
  (bind _building_interaction_widget (Variables|/Game/UI_and_Widgets/Colony_and_units_system/BuildingsWidgets/Center_Widget.Center_Widget_C|GetBuilding_Interaction_Widget _center_widget_ref))
  (Rendering|Components|TextRender|SetText (Variables|/Game/UI_and_Widgets/Colony_and_units_system/BuildingsWidgets/Building_Interaction_Widget.Building_Interaction_Widget_C|GetTextBlock_270 (Variables|/Game/UI_and_Widgets/Colony_and_units_system/BuildingsWidgets/Center_Widget.Center_Widget_C|GetBuilding_Interaction_Widget (Variables|/Game/SaveGame/GlobalGameInstance.GlobalGameInstance_C|GetCenterRecrutOnViewport (Variables|Default|GetAs%20Global%20Game%20Instance)))) (Variables|/Script/UMG.TextBlock|GetText (Variables|/Game/UI_and_Widgets/Colony_and_units_system/BuildingsWidgets/Building_Interaction_Widget.Building_Interaction_Widget_C|GetTextBlock_270 (Variables|/Game/UI_and_Widgets/Colony_and_units_system/BuildingsWidgets/Center_Widget.Center_Widget_C|GetBuilding_Interaction_Widget (Variables|Default|Getcenter%20widget%20ref)))))
  (Default|GetBuildingInfo (Variables|/Game/UI_and_Widgets/Colony_and_units_system/BuildingsWidgets/Center_Widget.Center_Widget_C|GetBuilding_Interaction_Widget (Variables|/Game/SaveGame/GlobalGameInstance.GlobalGameInstance_C|GetCenterRecrutOnViewport (Variables|Default|GetAs%20Global%20Game%20Instance))) (Variables|/Game/UI_and_Widgets/Colony_and_units_system/BuildingsWidgets/Building_Interaction_Widget.Building_Interaction_Widget_C|GetBuildingName _building_interaction_widget) (Variables|/Game/UI_and_Widgets/Colony_and_units_system/BuildingsWidgets/Building_Interaction_Widget.Building_Interaction_Widget_C|GetBuildingStatus _building_interaction_widget) (Variables|/Game/UI_and_Widgets/Colony_and_units_system/BuildingsWidgets/Building_Interaction_Widget.Building_Interaction_Widget_C|GetBuildingAmount _building_interaction_widget) (Variables|/Game/UI_and_Widgets/Colony_and_units_system/BuildingsWidgets/Building_Interaction_Widget.Building_Interaction_Widget_C|GetBuildingSellCost _building_interaction_widget) false))