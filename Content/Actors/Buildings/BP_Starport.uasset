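; Starport building that, when clicked in energy mode, draws 1000 energy from the selected energy station and calls in the nearest colonist as a worker.
; The colonist walks over and is destroyed on arrival to count as inside.
; Clicking again with the same station selected refunds the energy and spawns an AI beside the building if occupied.
; While working, Tick uses a debug-drawn line trace to show the station link.
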(event OnClicked(Cube)
  (params (TouchedComponent :type Primitive%20Component%20Object%20Reference) (ButtonPressed :type Key%20Structure :default "None"))
  (bind _returnvalue (Transformation|GetActorLocation))
  (bind _returnvalue_2 (Transformation|GetActorLocation))
  (bind _returnvalue_3 (Transformation|GetActorLocation))
  (bind _asglobal_game_instance (Utilities|Casting|CastToGlobalGameInstance (Game|GetGameInstance)))
  (if (Variables|/Game/SaveGame/GlobalGameInstance.GlobalGameInstance_C|GetActive_Energy _asglobal_game_instance)
    (if (Variables|Default|Getalready_work)
      (if (== (Variables|Default|Getid_added_station) (Variables|/Game/SaveGame/GlobalGameInstance.GlobalGameInstance_C|Getidofenergy _asglobal_game_instance))
        (Variables|Default|Setalready_work false)
        (Variables|/Game/SaveGame/GlobalGameInstance.GlobalGameInstance_C|SetActive_Energy _asglobal_game_instance true)
        (bind _outactors (Actor|GetAllActorsOfClass "/Game/Actors/Buildings/BP_Energy_Station.BP_Energy_Station_C"))
        (Variables|/Game/Actors/Buildings/BP_Energy_Station.BP_Energy_Station_C|Setenergy%20cost (Utilities|Array|Get(acopy) _outactors (Variables|/Game/SaveGame/GlobalGameInstance.GlobalGameInstance_C|Getidofenergy _asglobal_game_instance)) (+ (Variables|/Game/Actors/Buildings/BP_Energy_Station.BP_Energy_Station_C|Getenergy%20cost (Utilities|Array|Get(acopy) _outactors (Variables|/Game/SaveGame/GlobalGameInstance.GlobalGameInstance_C|Getidofenergy _asglobal_game_instance))) 1e+03))
        (if (Variables|Default|Getalready_in_building)
          (AI|SpawnAIFromClass 0 0 (Math|Vector|MakeVector (+ (.x _returnvalue_3) 1e+03) (.y _returnvalue_3) (+ (.z _returnvalue_3) 1e+02)) "0, 0, 0" false 0)
          (Variables|Default|Setalready_in_building false)
          (else
            (bind _returnvalue_4 (Actor|GetActorOfClass "/Script/Engine.TargetPoint"))
            (bind _randomlocation (Class|NavigationSystemV1|GetRandomLocationinNavigableRadius (Transformation|GetActorLocation _returnvalue_4) 1e+04 0 0))
            (AI|AIMoveTo 0 _randomlocation 0 5.0 false))))
      (else
        (bind _outactors_2 (Actor|GetAllActorsOfClass "/Game/Actors/Buildings/BP_Energy_Station.BP_Energy_Station_C"))
        (if (not (< (Variables|/Game/Actors/Buildings/BP_Energy_Station.BP_Energy_Station_C|Getenergy%20cost (Utilities|Array|Get(acopy) _outactors_2 (Variables|/Game/SaveGame/GlobalGameInstance.GlobalGameInstance_C|Getidofenergy _asglobal_game_instance))) 1e+03))
          (Variables|/Game/Actors/Buildings/BP_Energy_Station.BP_Energy_Station_C|Setenergy%20cost (Utilities|Array|Get(acopy) _outactors_2 (Variables|/Game/SaveGame/GlobalGameInstance.GlobalGameInstance_C|Getidofenergy _asglobal_game_instance)) (- (Variables|/Game/Actors/Buildings/BP_Energy_Station.BP_Energy_Station_C|Getenergy%20cost (Utilities|Array|Get(acopy) _outactors_2 (Variables|/Game/SaveGame/GlobalGameInstance.GlobalGameInstance_C|Getidofenergy _asglobal_game_instance))) 1e+03))
          (Variables|Default|Setalready_work true)
          (Variables|Default|Setvector (Transformation|GetActorLocation (Utilities|Array|Get(acopy) _outactors_2 (Variables|/Game/SaveGame/GlobalGameInstance.GlobalGameInstance_C|Getidofenergy _asglobal_game_instance))))
          (Variables|/Game/SaveGame/GlobalGameInstance.GlobalGameInstance_C|SetActive_Energy _asglobal_game_instance false)
          (Variables|Default|Setid_added_station (Variables|/Game/SaveGame/GlobalGameInstance.GlobalGameInstance_C|Getidofenergy _asglobal_game_instance))
          (bind _outactors_3 (Actor|GetAllActorsOfClass "/Game/Actors/Units/chuvachochki/colonist.colonist_C"))
          (for (_ _array_index) _outactors_3
            (if (not (< (Variables|Default|Getmin_vector_colonist) (Math|Float|Sqrt (+ (* (- (.x _returnvalue) (.x (Transformation|GetActorLocation (Utilities|Array|Get(acopy) _outactors_3 _array_index)))) (- (.x _returnvalue) (.x (Transformation|GetActorLocation (Utilities|Array|Get(acopy) _outactors_3 _array_index))))) (* (- (.y _returnvalue) (.y (Transformation|GetActorLocation (Utilities|Array|Get(acopy) _outactors_3 _array_index)))) (- (.y _returnvalue) (.y (Transformation|GetActorLocation (Utilities|Array|Get(acopy) _outactors_3 _array_index)))))))))
              (Variables|Default|Setmin_vector_colonist (Math|Float|Sqrt (+ (* (- (.x _returnvalue) (.x (Transformation|GetActorLocation (Utilities|Array|Get(acopy) _outactors_3 _array_index)))) (- (.x _returnvalue) (.x (Transformation|GetActorLocation (Utilities|Array|Get(acopy) _outactors_3 _array_index))))) (* (- (.y _returnvalue) (.y (Transformation|GetActorLocation (Utilities|Array|Get(acopy) _outactors_3 _array_index)))) (- (.y _returnvalue) (.y (Transformation|GetActorLocation (Utilities|Array|Get(acopy) _outactors_3 _array_index))))))))
              (Variables|Default|Setindex_walker _array_index)))
          (Variables|Default|Setmin_vector_colonist 1e+05)
          (bind _outactors_4 (Actor|GetAllActorsOfClass "/Game/Actors/Units/chuvachochki/colonist.colonist_C"))
          (AI|AIMoveTo (Utilities|Array|Get(acopy) _outactors_4 (Variables|Default|Getindex_walker)) (Math|Vector|MakeVector (.x _returnvalue_2) (.y _returnvalue_2) 0.0) 0 8e+02 false
            (:OnSuccess
              (Actor|DestroyActor (Utilities|Array|Get(acopy) _outactors_4 (Variables|Default|Getindex_walker)))
              (Variables|Default|Setalready_in_building true))))))))

(event EventTick
  (params (DeltaSeconds :type Float%20%28single-precision%29))
  (bind _returnvalue (Transformation|GetActorLocation))
  (bind _vector (Variables|Default|Getvector))
  (if (Variables|Default|Getalready_work)
    (Collision|LineTraceByChannel (Math|Vector|MakeVector (.x _returnvalue) (.y _returnvalue) (+ (.z _returnvalue) 1e+02)) (Math|Vector|MakeVector (.x _vector) (.y _vector) (+ (.z _vector) 1e+02)) "TraceTypeQuery1" false 0 "ForDuration" false "(R=0.000000,G=0.000000,B=0.000000,A=1.000000)" "(R=0.000000,G=0.000000,B=0.000000,A=1.000000)" 0.2)))

(fn ConstructionScript)