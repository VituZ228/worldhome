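; Energy tower building that relays power links from energy stations or other towers on a planet.
; On BeginPlay it can auto-attach to the nearest station or working tower in range; clicks link, unlink or select sources through GlobalGameInstance.
; Tower IDs come from object names plus a 100000 offset, and unlinking cascades to dependent towers and starports.
; Tick draws links and the mouse drag line as debug line traces, raising links away from the planet center.
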(event OnClicked(Building)
  (params (TouchedComponent :type Primitive%20Component%20Object%20Reference) (ButtonPressed :type Key%20Structure :default "None"))
  (bind _global_game_instance_ref (Variables|Default|Getglobal%20game%20instance%20ref))
  (bind _global_game_instance_ref_2 (Variables|Default|Getglobal%20game%20instance%20ref))
  (if (Variables|/Game/SaveGame/GlobalGameInstance.GlobalGameInstance_C|GetActive_Energy _global_game_instance_ref_2)
    ;[1 1 1] фолс включает станцию
    (if (Variables|Default|Getalready_work)
      (if (== (Variables|Default|Getid_added_station) (Variables|/Game/SaveGame/GlobalGameInstance.GlobalGameInstance_C|Getidofenergy _global_game_instance_ref))
        (CallFunction|Delite)
        (Variables|Default|Setalready_work false)
        (Variables|/Game/SaveGame/GlobalGameInstance.GlobalGameInstance_C|SetActive_Energy _global_game_instance_ref true)
        (else
          (Variables|/Game/SaveGame/GlobalGameInstance.GlobalGameInstance_C|SetActive_Energy _global_game_instance_ref false)))
      (else
        (if (> (Variables|/Game/SaveGame/GlobalGameInstance.GlobalGameInstance_C|Getidofenergy (Variables|Default|Getglobal%20game%20instance%20ref)) 99999)
          (bind _outactors (Actor|GetAllActorsOfClass "BP_EnergyTower_C"))
          (Variables|Default|Setint%20for%20delite (- (Variables|/Game/SaveGame/GlobalGameInstance.GlobalGameInstance_C|Getidofenergy _global_game_instance_ref) 100000))
          (Variables|Default|Setid%20of%20added%20station (Variables|BP_EnergyTower_C|Getid%20of%20added%20station (Utilities|Array|Get(acopy) _outactors (- (Variables|/Game/SaveGame/GlobalGameInstance.GlobalGameInstance_C|Getidofenergy _global_game_instance_ref) 100000))))
          (Variables|Default|Setvector (Transformation|GetActorLocation (Utilities|Array|Get(acopy) _outactors (- (Variables|/Game/SaveGame/GlobalGameInstance.GlobalGameInstance_C|Getidofenergy _global_game_instance_ref) 100000))))
          (else
            (bind _outactors_2 (Actor|GetAllActorsOfClass "/Game/Actors/Buildings/Civilian_Buildings/BP_Energy_Station.BP_Energy_Station_C"))
            (Variables|Default|Setvector (Transformation|GetActorLocation (Utilities|Array|Get(acopy) _outactors_2 (Variables|/Game/SaveGame/GlobalGameInstance.GlobalGameInstance_C|Getidofenergy _global_game_instance_ref))))
            (Variables|Default|Setid%20of%20added%20station (Variables|/Game/SaveGame/GlobalGameInstance.GlobalGameInstance_C|Getidofenergy _global_game_instance_ref))))
        (Variables|Default|Setalready_work true)
        (Variables|/Game/SaveGame/GlobalGameInstance.GlobalGameInstance_C|SetActive_Energy _global_game_instance_ref false)
        (Variables|Default|Setid_added_station (Variables|/Game/SaveGame/GlobalGameInstance.GlobalGameInstance_C|Getidofenergy _global_game_instance_ref))))
    (elif (Variables|Default|Getalready_work)
      (Variables|/Game/SaveGame/GlobalGameInstance.GlobalGameInstance_C|SetActive_Energy _global_game_instance_ref_2 true)
      (Variables|/Game/SaveGame/GlobalGameInstance.GlobalGameInstance_C|Setidofenergy _global_game_instance_ref_2 (+ (Math|Conversions|ToInteger(Byte) (Utilities|String|GetSubstring (Utilities|GetObjectName self) 17 3)) 100000)))))

(event Custom|null%20all%20towers
  (CallFunction|Delite)
  (Variables|Default|Setalready_work false)
  (Variables|/Game/SaveGame/GlobalGameInstance.GlobalGameInstance_C|SetActive_Energy (Variables|Default|Getglobal%20game%20instance%20ref) true))

(event EventBeginPlay
  (bind _asglobal_game_instance (Utilities|Casting|CastToGlobalGameInstance (Game|GetGameInstance)))
  (bind _output_get (Variables|Default|Setglobal%20game%20instance%20ref _asglobal_game_instance))
  (Variables|Default|Setkakoq%20to%20int (+ (Math|Conversions|ToInteger(Byte) (Utilities|String|GetSubstring (Utilities|GetObjectName self) 17 3)) 100000))
  (bind _outactors (Actor|GetAllActorsOfClass "/Game/Actors/Planets/Master_Planet_BigVer_Asset.Master_Planet_BigVer_Asset_C"))
  (Variables|Default|Setworld%20origin (Transformation|GetActorLocation (Utilities|Array|Get(acopy) _outactors (Variables|/Game/SaveGame/GlobalGameInstance.GlobalGameInstance_C|GetIndexOfPlanet (Variables|Default|Getglobal%20game%20instance%20ref)))))
  (if (Variables|/Game/SaveGame/GlobalGameInstance.GlobalGameInstance_C|Getauto%20prisoska _output_get)
    (CallFunction|Prisosik)))

(event EventTick
  (params (DeltaSeconds :type Float%20%28single-precision%29))
  (bind _global_game_instance_ref (Variables|Default|Getglobal%20game%20instance%20ref))
  (if (Variables|Default|Getalready_work)
    (Collision|LineTraceByChannel (+ (* (Math|Vector|GetUnitDirection(Vector) (Variables|Default|Getworld%20origin) (Transformation|GetActorLocation)) "1000.000000,1000.000000,1000.000000") (Transformation|GetActorLocation)) (+ (* (Math|Vector|GetUnitDirection(Vector) (Variables|Default|Getworld%20origin) (Variables|Default|Getvector)) "1000.000000,1000.000000,1000.000000") (Variables|Default|Getvector)) "TraceTypeQuery1" false 0 "ForDuration" false "(R=0.000000,G=0.000000,B=0.000000,A=1.000000)" "(R=0.000000,G=0.000000,B=0.000000,A=1.000000)" 0.2))
  (if (== (Variables|/Game/SaveGame/GlobalGameInstance.GlobalGameInstance_C|Getidofenergy _global_game_instance_ref) (Variables|Default|Getkakoq%20to%20int))
    (if (Variables|/Game/SaveGame/GlobalGameInstance.GlobalGameInstance_C|GetActive_Energy _global_game_instance_ref)
      (Collision|LineTraceByChannel (.WorldLocation (Game|Player|ConvertMouseLocationToWorldSpace (Game|GetPlayerController 0))) (Transformation|GetActorLocation) "TraceTypeQuery1" false 0 "ForDuration" false "(R=0.000000,G=0.000000,B=0.000000,A=1.000000)" "(R=0.000000,G=0.000000,B=0.000000,A=1.000000)" 0.02))))

(fn ConstructionScript)

(fn Delite
  (bind _outactors (Actor|GetAllActorsOfClass "/Game/Actors/Buildings/Civilian_Buildings/BP_Starport.BP_Starport_C"))
  (for _array_element _outactors
    (if (== (- (Variables|Default|Getkakoq%20to%20int) 100000) (Variables|/Game/Actors/Buildings/Civilian_Buildings/BP_Starport.BP_Starport_C|Getint%20for%20delite _array_element))
      (Default|NullEveryStartport _array_element)))
  (bind _outactors_2 (Actor|GetAllActorsOfClass "BP_EnergyTower_C"))
  (for _array_element_2 _outactors_2
    (if (== (Variables|BP_EnergyTower_C|Getint%20for%20delite _array_element_2) (- (Variables|Default|Getkakoq%20to%20int) 100000))
      (CallFunction|NullAllTowers _array_element_2))))

(fn Prisosik
  (bind _outactors (Actor|GetAllActorsOfClass "/Game/Actors/Buildings/Civilian_Buildings/BP_Energy_Station.BP_Energy_Station_C"))
  (for _array_element _outactors
    (if (<= (Math|Vector|Distance(Vector) (Transformation|GetActorLocation) (Transformation|GetActorLocation _array_element)) (Variables|/Game/SaveGame/GlobalGameInstance.GlobalGameInstance_C|Getrange%20of%20electric (Variables|Default|Getglobal%20game%20instance%20ref)))
      (if (<= (Math|Vector|Distance(Vector) (Transformation|GetActorLocation) (Transformation|GetActorLocation _array_element)) (Variables|Default|Getmin%20distance))
        (Variables|Default|Setmin%20distance (Math|Vector|Distance(Vector) (Transformation|GetActorLocation) (Transformation|GetActorLocation _array_element)))
        (Variables|Default|Setbp%20energy%20station _array_element))))
  (bind _outactors_2 (Actor|GetAllActorsOfClass "BP_EnergyTower_C"))
  (for _array_element_2 _outactors_2
    (if (Variables|BP_EnergyTower_C|Getalready_work _array_element_2)
      (if (<= (Math|Vector|Distance(Vector) (Transformation|GetActorLocation) (Transformation|GetActorLocation _array_element_2)) (Variables|/Game/SaveGame/GlobalGameInstance.GlobalGameInstance_C|GetRange%20Of%20Electric (Variables|Default|Getglobal%20game%20instance%20ref)))
        (if (<= (Math|Vector|Distance(Vector) (Transformation|GetActorLocation) (Transformation|GetActorLocation _array_element_2)) (Variables|Default|Getmin%20distance))
          (Variables|Default|Setmin%20distance (Math|Vector|Distance(Vector) (Transformation|GetActorLocation) (Transformation|GetActorLocation _array_element_2)))
          (Variables|Default|Setbp%20energy%20tower _array_element_2)
          (Variables|Default|Setprisoska%20na%20tavek%20ili%20net true)))))
  (if (not (== (Variables|Default|Getmin%20distance) 1e+09))
    (if (Variables|Default|Getprisoska%20na%20tavek%20ili%20net)
      (Variables|Default|Setvector (Transformation|GetActorLocation (Variables|Default|Getbp%20energy%20tower)))
      (Variables|Default|Setid%20of%20added%20station (Variables|BP_EnergyTower_C|Getid%20of%20added%20station (Variables|Default|Getbp%20energy%20tower)))
      (Variables|Default|Setid_added_station (Variables|BP_EnergyTower_C|Getkakoq%20to%20int (Variables|Default|Getbp%20energy%20tower)))
      (Variables|Default|Setint%20for%20delite (- (Variables|BP_EnergyTower_C|Getkakoq%20to%20int (Variables|Default|Getbp%20energy%20tower)) 100000))
      (else
        (Variables|Default|Setvector (Transformation|GetActorLocation (Variables|Default|Getbp%20energy%20station)))
        (Variables|Default|Setid%20of%20added%20station (Math|Conversions|ToInteger(Byte) (Utilities|String|GetSubstring (Utilities|GetObjectName (Variables|Default|Getbp%20energy%20station)) 20 3)))))
    (Variables|Default|Setalready_work true)))