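; Starport building that dispatches cargo or civilian ships carrying colonists or food to planets with another starport.
; On spawn it charges resources and auto-connects to a nearby energy station or tower, taking energy and workers; destruction refunds part of the cost.
; Shared viewport widget events affect only the custom-depth highlighted port: plug toggle, sell, and validated launches handed to ControllerCam after an animation.
; Tick draws the power link with debug line traces.
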(event Custom|StartTravel_Pressed_Event
  (bind _as_global_game_instance (Variables|Default|GetAs%20Global%20Game%20Instance))
  (bind _as_global_game_instance_2 (Variables|Default|GetAs%20Global%20Game%20Instance))
  (bind _controllercam_ref (Variables|Default|GetControllerCam_Ref))
  (bind _starportwidgetonviewport (Variables|/Game/SaveGame/GlobalGameInstance.GlobalGameInstance_C|GetStarportWidgetOnViewport _as_global_game_instance))
  (bind _starportwidgetonviewport_2 (Variables|/Game/SaveGame/GlobalGameInstance.GlobalGameInstance_C|GetStarportWidgetOnViewport _as_global_game_instance_2))
  (bind _playerressourses (Variables|/Game/CameraAndControllerStuff/controllerCam.controllerCam_C|GetPlayerRessourses _controllercam_ref))
  ;[1 0 0.3182] ЛОГИКА ВЫЛЕТА НАЗНАЧЕНЫХ КОРАБЛЕЙ ДО ВЫБРАННОГО ПУНКТА НАЗНАЧЕНИЯ ВЫЗЫВАЕМАЯ КНОПКОЙ РЕГЕСТРАЦИИ РЕЙСА (НАСТОЯЩЕЕ ЕЕ ВЫПОЛНЕНИЕ НАХОДИТСЯ В ControllerCam И BasedShip)
  (if (Variables|Default|GetBuildingIsDoneForWork)
    (if (Variables|/Script/Engine.PrimitiveComponent|GetbRenderCustomDepth (Variables|Default|GetBuildMesh))
      (if (Utilities|Enum|Equal(Enum) (Class|ComboBoxString|GetSelectedOption (Variables|/Game/UI_and_Widgets/Colony_and_units_system/BuildingsWidgets/Starport_Widget.Starport_Widget_C|GetComboBoxString_Planets _starportwidgetonviewport)) "Выберите пункт назначения...")
        (Development|PrintString "НЕОБХОДИМО ВЫБРАТЬ ПУНКТ НАЗНАЧЕНИЯ")
        (elif (Utilities|Enum|Equal(Enum) (Class|ComboBoxString|GetSelectedOption (Variables|/Game/UI_and_Widgets/Colony_and_units_system/BuildingsWidgets/Starport_Widget.Starport_Widget_C|GetComboBoxString_Planets _starportwidgetonviewport)) (Utilities|String|ToString(Text) (.name (Variables|/Game/Actors/Planets/Master_Planet_Asset.Master_Planet_Asset_C|GetPlanetInfo (Variables|Default|GetNativePlanet)))))
          (Development|PrintString "НЕЛЬЗЯ ЗАРЕГЕСТРИРОВАТЬ ПЕРЕЛЕТ С ПЛАНЕТЫ НА ЭТУ ЖЕ ПЛАНЕТУ")
          (elif (Math|Boolean|ORBoolean (< (Utilities|Array|Get(acopy) _playerressourses) (Math|Conversions|ToInteger(Byte) (Utilities|String|ToString(Text) (Variables|/Script/UMG.TextBlock|GetText (Variables|/Game/UI_and_Widgets/Colony_and_units_system/BuildingsWidgets/Starport_Widget.Starport_Widget_C|GetRareMetCost_TextBlock _starportwidgetonviewport_2))))) (< (Utilities|Array|Get(acopy) _playerressourses 1) (Math|Conversions|ToInteger(Byte) (Utilities|String|ToString(Text) (Variables|/Script/UMG.TextBlock|GetText (Variables|/Game/UI_and_Widgets/Colony_and_units_system/BuildingsWidgets/Starport_Widget.Starport_Widget_C|GetPromMetCost_TextBlock _starportwidgetonviewport_2))))) (< (Utilities|Array|Get(acopy) _playerressourses 2) (Math|Conversions|ToInteger(Byte) (Utilities|String|ToString(Text) (Variables|/Script/UMG.TextBlock|GetText (Variables|/Game/UI_and_Widgets/Colony_and_units_system/BuildingsWidgets/Starport_Widget.Starport_Widget_C|GetAcidCost_TextBlock _starportwidgetonviewport_2))))) (< (Utilities|Array|Get(acopy) _playerressourses 3) (Math|Conversions|ToInteger(Byte) (Utilities|String|ToString(Text) (Variables|/Script/UMG.TextBlock|GetText (Variables|/Game/UI_and_Widgets/Colony_and_units_system/BuildingsWidgets/Starport_Widget.Starport_Widget_C|GetGazCost_TextBlock _starportwidgetonviewport_2))))))
            (Development|PrintString "ВАМ НЕ ХВАТАЕТ РЕССУРСОВ ЧТОБЫ ОСУЩЕСТВИТЬ ЭТОТ РЕЙС")
            (else
              (CallFunction|CheckStarport)
              (if (Variables|Default|GetIsSomeStarportOnPlanet)
                (bind _output_get (Variables|Default|SetColichestvoChelovNaPerelet (Math|Conversions|ToInteger(Byte) (Utilities|String|ToString(Text) (Default|GetAmountTextBlockText (Variables|/Game/SaveGame/GlobalGameInstance.GlobalGameInstance_C|GetStarportWidgetOnViewport (Variables|Default|Getgame%20global%20ref)))))))
                (if (Utilities|Enum|Equal(Enum) (Class|ComboBoxString|GetSelectedOption (Variables|/Game/UI_and_Widgets/Colony_and_units_system/BuildingsWidgets/Starport_Widget.Starport_Widget_C|GetComboBoxString_TypeOfTravel (Variables|/Game/SaveGame/GlobalGameInstance.GlobalGameInstance_C|GetStarportWidgetOnViewport (Variables|Default|GetAs%20Global%20Game%20Instance)))) "Провизия")
                  (Variables|Default|Setcolonist%20or%20not false)
                  (if (>= (Utilities|Array|Get(acopy) (Variables|/Game/CameraAndControllerStuff/controllerCam.controllerCam_C|GetColoniesFood (Variables|Default|GetControllerCam_Ref)) (Variables|/Game/SaveGame/GlobalGameInstance.GlobalGameInstance_C|GetIndexOfPlanet (Variables|Default|GetAs%20Global%20Game%20Instance))) _output_get)
                    (CallFunction|ContinPerelet :!label _label)
                    (else
                      (Development|PrintString "недостаточно еды")))
                  (else
                    (Variables|Default|Setcolonist%20or%20not true)
                    (if (>= (Utilities|Array|Get(acopy) (Variables|/Game/CameraAndControllerStuff/controllerCam.controllerCam_C|GetColonistsPopulation (Variables|Default|GetControllerCam_Ref)) (Variables|/Game/SaveGame/GlobalGameInstance.GlobalGameInstance_C|GetIndexOfPlanet (Variables|Default|GetAs%20Global%20Game%20Instance))) _output_get)
                      (goto _label)
                      (else
                        (Development|PrintString "недостаточно колонистов")))))
                (else
                  (Development|PrintString "на этой планете нет старпортов"))))))))
    (else
      (Development|PrintString "Центр не включен"))))

(event Custom|SellBtn_Pressed_Event
  ;[0 0.1566 1] СЛЕДИТ ЗА НАЖАТИЕМ НА КНОПКУ ПРОДАЖИ, ПРИ НАЖАТИИ ВОЗВРАЩАЕТ ЦЕНУ ЗДАНИЯ УМНОЖЕНУЮ НА ПРОЦЕНТ SellCost
  (if (Variables|/Script/Engine.PrimitiveComponent|GetbRenderCustomDepth (Variables|Default|GetBuildMesh))
    (Actor|DestroyActor)))

(event Custom|continPerelet
  (bind _as_global_game_instance (Variables|Default|GetAs%20Global%20Game%20Instance))
  (bind _controllercam_ref (Variables|Default|GetControllerCam_Ref))
  (bind _as_air_base_main_anim (Variables|Default|GetAs%20Air%20Base%20Main%20Anim))
  (bind _as_global_game_instance_2 (Variables|Default|GetAs%20Global%20Game%20Instance))
  (bind _as_global_game_instance_3 (Variables|Default|GetAs%20Global%20Game%20Instance))
  (bind _controllercam_ref_2 (Variables|Default|GetControllerCam_Ref))
  (bind _as_global_game_instance_4 (Variables|Default|GetAs%20Global%20Game%20Instance))
  (bind _nativeplanet (Variables|Default|GetNativePlanet))
  (bind _game_global_ref (Variables|Default|Getgame%20global%20ref))
  (bind _returnvalue (Transformation|GetActorLocation _nativeplanet))
  (bind _indexofplanet (Variables|/Game/SaveGame/GlobalGameInstance.GlobalGameInstance_C|GetIndexOfPlanet _as_global_game_instance))
  (bind _rangeinkm (Variables|/Game/Actors/Planets/Master_Planet_Asset.Master_Planet_Asset_C|GetRangeInKm _nativeplanet))
  (bind _starportwidgetonviewport (Variables|/Game/SaveGame/GlobalGameInstance.GlobalGameInstance_C|GetStarportWidgetOnViewport _as_global_game_instance_2))
  (bind _starportwidgetonviewport_2 (Variables|/Game/SaveGame/GlobalGameInstance.GlobalGameInstance_C|GetStarportWidgetOnViewport _as_global_game_instance_3))
  (bind _playerressourses (Variables|/Game/CameraAndControllerStuff/controllerCam.controllerCam_C|GetPlayerRessourses _controllercam_ref_2))
  (bind _playerressourses_2 (Variables|/Game/CameraAndControllerStuff/controllerCam.controllerCam_C|GetPlayerRessourses _controllercam_ref))
  (bind _starportwidgetonviewport_3 (Variables|/Game/SaveGame/GlobalGameInstance.GlobalGameInstance_C|GetStarportWidgetOnViewport _game_global_ref))
  (bind _returnvalue_2 (* _rangeinkm 1e+03))
  (bind _destinationplanet (Variables|/Game/UI_and_Widgets/Colony_and_units_system/BuildingsWidgets/Starport_Widget.Starport_Widget_C|GetDestinationPlanet _starportwidgetonviewport_3))
  (bind _shiptype_comboboxstring (Variables|/Game/UI_and_Widgets/Colony_and_units_system/BuildingsWidgets/Starport_Widget.Starport_Widget_C|GetShipType_ComboBoxString _starportwidgetonviewport))
  (bind _returnvalue_3 (Utilities|GetObjectName _destinationplanet))
  (bind _returnvalue_4 (Class|ComboBoxString|GetSelectedOption _shiptype_comboboxstring))
  (bind _returnvalue_5 (+ _returnvalue_2 2e+03))
  (bind _returnvalue_6 (Utilities|String|Len _returnvalue_3))
  (bind _returnvalue_7 (+ (Math|Vector|MakeVector (.x _returnvalue) (.y _returnvalue) -267.0) (Math|Vector|MakeVector _returnvalue_5 0.0 0.0)))
  (bind _returnvalue_8 (- _returnvalue_6 1))
  (bind _returnvalue_9 (Utilities|String|RightChop _returnvalue_3 _returnvalue_8))
  (bind _returnvalue_10 (Math|Conversions|ToInteger(Byte) _returnvalue_9))
  ;[1 0 0.3182] ЛОГИКА ВЫЛЕТА НАЗНАЧЕНЫХ КОРАБЛЕЙ ДО ВЫБРАННОГО ПУНКТА НАЗНАЧЕНИЯ ВЫЗЫВАЕМАЯ КНОПКОЙ РЕГЕСТРАЦИИ РЕЙСА (НАСТОЯЩЕЕ ЕЕ ВЫПОЛНЕНИЕ НАХОДИТСЯ В ControllerCam И BasedShip)
  (bind _ascontroller_cam (Utilities|Casting|CastTocontrollerCam (Game|GetPlayerController 0)))
  (if (Variables|Default|Getcolonist%20or%20not)
    (Utilities|Array|SetArrayElem (Variables|/Game/CameraAndControllerStuff/controllerCam.controllerCam_C|GetColonistsPopulation _ascontroller_cam) _indexofplanet (- (Utilities|Array|Get(acopy) (Variables|/Game/CameraAndControllerStuff/controllerCam.controllerCam_C|GetColonistsPopulation _ascontroller_cam) _indexofplanet) (Variables|Default|GetColichestvoChelovNaPerelet)))
    (else
      (Utilities|Array|SetArrayElem (Variables|/Game/CameraAndControllerStuff/controllerCam.controllerCam_C|GetColoniesFood _ascontroller_cam) _indexofplanet (- (Utilities|Array|Get(acopy) (Variables|/Game/CameraAndControllerStuff/controllerCam.controllerCam_C|GetColoniesFood _ascontroller_cam) _indexofplanet) (Variables|Default|GetColichestvoChelovNaPerelet)))))
  (Utilities|Array|SetArrayElem _playerressourses_2 0 (- (Utilities|Array|Get(acopy) _playerressourses) (Math|Conversions|ToInteger(Byte) (Utilities|String|ToString(Text) (Variables|/Script/UMG.TextBlock|GetText (Variables|/Game/UI_and_Widgets/Colony_and_units_system/BuildingsWidgets/Starport_Widget.Starport_Widget_C|GetRareMetCost_TextBlock _starportwidgetonviewport_2))))))
  (Utilities|Array|SetArrayElem _playerressourses_2 1 (- (Utilities|Array|Get(acopy) _playerressourses 1) (Math|Conversions|ToInteger(Byte) (Utilities|String|ToString(Text) (Variables|/Script/UMG.TextBlock|GetText (Variables|/Game/UI_and_Widgets/Colony_and_units_system/BuildingsWidgets/Starport_Widget.Starport_Widget_C|GetPromMetCost_TextBlock _starportwidgetonviewport_2))))))
  (Utilities|Array|SetArrayElem _playerressourses_2 2 (- (Utilities|Array|Get(acopy) _playerressourses 2) (Math|Conversions|ToInteger(Byte) (Utilities|String|ToString(Text) (Variables|/Script/UMG.TextBlock|GetText (Variables|/Game/UI_and_Widgets/Colony_and_units_system/BuildingsWidgets/Starport_Widget.Starport_Widget_C|GetAcidCost_TextBlock _starportwidgetonviewport_2))))))
  (Utilities|Array|SetArrayElem _playerressourses_2 3 (- (Utilities|Array|Get(acopy) _playerressourses 3) (Math|Conversions|ToInteger(Byte) (Utilities|String|ToString(Text) (Variables|/Script/UMG.TextBlock|GetText (Variables|/Game/UI_and_Widgets/Colony_and_units_system/BuildingsWidgets/Starport_Widget.Starport_Widget_C|GetGazCost_TextBlock _starportwidgetonviewport_2))))))
  (Variables|/Game/SSF_Buildings/Buildings/AirBase/Animations/AirBase_MainAnim.AirBase_MainAnim_C|SetShipsSpawning _as_air_base_main_anim true)
  (Variables|/Game/SaveGame/GlobalGameInstance.GlobalGameInstance_C|SetStarport_Animating _as_global_game_instance_4 true)
  (Utilities|FlowControl|Delay 6.67)
  (Variables|/Game/SaveGame/GlobalGameInstance.GlobalGameInstance_C|SetStarport_Animating _as_global_game_instance_4 false)
  (Variables|/Game/SSF_Buildings/Buildings/AirBase/Animations/AirBase_MainAnim.AirBase_MainAnim_C|SetShipsSpawning _as_air_base_main_anim false)
  (if (Utilities|Enum|Equal(Enum) _returnvalue_4 "Грузовой корабль \"Старкос\"")
    (bind _returnvalue_11 (Game|SpawnActorfromClass "/Game/Actors/Units/SpaceShips/BasedShip.BasedShip_C" (Math|Transform|MakeTransform _returnvalue_7 "0, 0, 0" "1.000000,1.000000,1.000000") "AdjustIfPossibleButAlwaysSpawn" "MultiplyWithRoot" 0 "NewEnumerator1" 0 false 1 false false 0))
    (Default|StartNewTravel (Variables|Default|GetControllerCam_Ref) _returnvalue_11 (Variables|Default|GetColichestvoChelovNaPerelet) _returnvalue_10 (Variables|Default|Getcolonist%20or%20not))
    (elif (Utilities|Enum|Equal(Enum) _returnvalue_4 "Гражданский транспортник \"Авелон\"")
      (bind _returnvalue_12 (Game|SpawnActorfromClass "/Game/Actors/Units/SpaceShips/BasedShip.BasedShip_C" (Math|Transform|MakeTransform _returnvalue_7 "0, 0, 0" "1.000000,1.000000,1.000000") "AdjustIfPossibleButAlwaysSpawn" "MultiplyWithRoot" 0 "NewEnumerator0" 0 false 1 false false 0))
      (Default|StartNewTravel (Variables|Default|GetControllerCam_Ref) _returnvalue_12 (Variables|Default|GetColichestvoChelovNaPerelet) _returnvalue_10 (Variables|Default|Getcolonist%20or%20not)))))

(event Custom|StationPlugBtn_Pressed_Event
  (if (Variables|/Script/Engine.PrimitiveComponent|GetbRenderCustomDepth (Variables|Default|GetBuildMesh))
    (if (Variables|Default|GetBuildingIsDoneForWork)
      (CallFunction|NullAllStation)
      (else
        (CallFunction|AutoPrisos)))))

(event EventDestroyed
  ;[0 0.1566 1] СЛЕДИТ ЗА НАЖАТИЕМ НА КНОПКУ ПРОДАЖИ, ПРИ НАЖАТИИ ВОЗВРАЩАЕТ ЦЕНУ ЗДАНИЯ УМНОЖЕНУЮ НА ПРОЦЕНТ SellCost
  (Widget|SetVisibility (Variables|/Game/SaveGame/GlobalGameInstance.GlobalGameInstance_C|GetStarportWidgetOnViewport (Variables|Default|GetAs%20Global%20Game%20Instance)) "Hidden")
  (bind _outactors (Actor|GetAllActorsOfClass "/Game/CameraAndControllerStuff/controllerCam.controllerCam_C"))
  (for (_array_element _array_index) (Variables|Default|GetCost)
    (Utilities|Array|SetArrayElem (Variables|/Game/CameraAndControllerStuff/controllerCam.controllerCam_C|GetPlayerRessourses (Utilities|Array|Get(acopy) _outactors)) _array_index (+ (Utilities|Array|Get(acopy) (Variables|/Game/CameraAndControllerStuff/controllerCam.controllerCam_C|GetPlayerRessourses (Utilities|Array|Get(acopy) _outactors)) _array_index) (* _array_element (Variables|Default|GetSellCost))))
    (bind _outactors_2 (Actor|GetAllActorsOfClass "BP_Starport_C"))
    (for _array_element_2 _outactors_2
      (Default|GetBuildingInfo (Variables|BP_Starport_C|GetBuildingInteractionWidget_Ref _array_element_2) (Variables|/Game/UI_and_Widgets/Colony_and_units_system/BuildingsWidgets/Building_Interaction_Widget.Building_Interaction_Widget_C|GetBuildingName (Variables|BP_Starport_C|GetBuildingInteractionWidget_Ref _array_element_2)) (Variables|/Game/UI_and_Widgets/Colony_and_units_system/BuildingsWidgets/Building_Interaction_Widget.Building_Interaction_Widget_C|GetBuildingStatus (Variables|BP_Starport_C|GetBuildingInteractionWidget_Ref _array_element_2)) (Utilities|Text|ToText(Integer) (- (Utilities|Array|Length _outactors_2) 1)) (Variables|/Game/UI_and_Widgets/Colony_and_units_system/BuildingsWidgets/Building_Interaction_Widget.Building_Interaction_Widget_C|GetBuildingSellCost (Variables|BP_Starport_C|GetBuildingInteractionWidget_Ref _array_element_2)) false))))

(event EventBeginPlay
  (bind _asair_base_main_anim (Utilities|Casting|CastToAirBase_MainAnim (Components|SkeletalMesh|GetAnimInstance (Variables|Default|GetBuildMesh))))
  (Variables|Default|SetAs%20Air%20Base%20Main%20Anim _asair_base_main_anim)
  (bind _asglobal_game_instance (Utilities|Casting|CastToGlobalGameInstance (Game|GetGameInstance)))
  (Variables|Default|SetAs%20Global%20Game%20Instance _asglobal_game_instance)
  (Variables|Default|Setgame%20global%20ref _asglobal_game_instance)
  (Default|UpdatePlanets (Variables|/Game/SaveGame/GlobalGameInstance.GlobalGameInstance_C|GetStarportWidgetOnViewport _asglobal_game_instance))
  (bind _outactors (Actor|GetAllActorsOfClass "/Game/Actors/Planets/Master_Planet_BigVer_Asset.Master_Planet_BigVer_Asset_C"))
  (Variables|Default|Setindex%20of%20planet (Variables|/Game/SaveGame/GlobalGameInstance.GlobalGameInstance_C|GetIndexOfPlanet (Variables|Default|Getgame%20global%20ref)))
  (Variables|Default|SetWorldOrigin (Transformation|GetActorLocation (Utilities|Array|Get(acopy) _outactors (Variables|/Game/SaveGame/GlobalGameInstance.GlobalGameInstance_C|GetIndexOfPlanet (Variables|Default|Getgame%20global%20ref)))))
  (bind _outactors_2 (Actor|GetAllActorsOfClass "/Game/Actors/Planets/Master_Planet_Asset.Master_Planet_Asset_C"))
  (Variables|Default|SetNativePlanet (Utilities|Array|Get(acopy) _outactors_2 (Variables|/Game/SaveGame/GlobalGameInstance.GlobalGameInstance_C|GetIndexOfPlanet _asglobal_game_instance)))
  (bind _asstarport_widget (Utilities|Casting|CastToStarport_Widget (UserInterface|GetWidget (Variables|Default|GetStarportWidget))))
  (Variables|Default|SetStarportWidget_Ref _asstarport_widget)
  (Variables|Default|SetBuildingInteractionWidget_Ref (Variables|/Game/UI_and_Widgets/Colony_and_units_system/BuildingsWidgets/Starport_Widget.Starport_Widget_C|GetBuilding_Interaction_Widget _asstarport_widget))
  ;[0.2434 0 1] ОТНИМАЕТ У ИГРОКА КОЛ-ВО РЕССУРСОВ НА ПОСТРОЙКУ ЗНАНИЯ СООТВЕТСТВУЮЩЕЕ ПЕРЕМЕННОЙ Cost
  (CallFunction|AutoPrisos)
  (bind _ascontroller_cam (Utilities|Casting|CastTocontrollerCam (Game|GetPlayerController 0)))
  (Variables|Default|SetControllerCam_Ref _ascontroller_cam)
  (for (_array_element _array_index) (Variables|Default|GetCost)
    (Utilities|Array|SetArrayElem (Variables|/Game/CameraAndControllerStuff/controllerCam.controllerCam_C|GetPlayerRessourses (Variables|Default|GetControllerCam_Ref)) _array_index (- (Utilities|Array|Get(acopy) (Variables|/Game/CameraAndControllerStuff/controllerCam.controllerCam_C|GetPlayerRessourses (Variables|Default|GetControllerCam_Ref)) _array_index) _array_element)))
  ;[1 0 0.3182] ЛОГИКА ВЫЛЕТА НАЗНАЧЕНЫХ КОРАБЛЕЙ ДО ВЫБРАННОГО ПУНКТА НАЗНАЧЕНИЯ ВЫЗЫВАЕМАЯ КНОПКОЙ РЕГЕСТРАЦИИ РЕЙСА (НАСТОЯЩЕЕ ЕЕ ВЫПОЛНЕНИЕ НАХОДИТСЯ В ControllerCam И BasedShip)
  (EventDispatchers|AssignStartTravelPressed (Variables|/Game/SaveGame/GlobalGameInstance.GlobalGameInstance_C|GetStarportWidgetOnViewport (Variables|Default|GetAs%20Global%20Game%20Instance)) (delegate Custom|StartTravel_Pressed_Event))
  ;[0 0.1566 1] СЛЕДИТ ЗА НАЖАТИЕМ НА КНОПКУ ПРОДАЖИ, ПРИ НАЖАТИИ ВОЗВРАЩАЕТ ЦЕНУ ЗДАНИЯ УМНОЖЕНУЮ НА ПРОЦЕНТ SellCost
  (EventDispatchers|AssignStationPlugBtnPressed (Variables|/Game/UI_and_Widgets/Colony_and_units_system/BuildingsWidgets/Starport_Widget.Starport_Widget_C|GetBuilding_Interaction_Widget (Variables|/Game/SaveGame/GlobalGameInstance.GlobalGameInstance_C|GetStarportWidgetOnViewport (Variables|Default|GetAs%20Global%20Game%20Instance))) (delegate Custom|StationPlugBtn_Pressed_Event))
  (EventDispatchers|AssignSellBtnPressed (Variables|/Game/UI_and_Widgets/Colony_and_units_system/BuildingsWidgets/Starport_Widget.Starport_Widget_C|GetBuilding_Interaction_Widget (Variables|/Game/SaveGame/GlobalGameInstance.GlobalGameInstance_C|GetStarportWidgetOnViewport (Variables|Default|GetAs%20Global%20Game%20Instance))) (delegate Custom|SellBtn_Pressed_Event))
  (bind _outactors_3 (Actor|GetAllActorsOfClass "BP_Starport_C"))
  (for _array_element_2 _outactors_3
    (Default|GetBuildingInfo (Variables|BP_Starport_C|GetBuildingInteractionWidget_Ref _array_element_2) (Variables|/Game/UI_and_Widgets/Colony_and_units_system/BuildingsWidgets/Building_Interaction_Widget.Building_Interaction_Widget_C|GetBuildingName (Variables|BP_Starport_C|GetBuildingInteractionWidget_Ref _array_element_2)) (Variables|/Game/UI_and_Widgets/Colony_and_units_system/BuildingsWidgets/Building_Interaction_Widget.Building_Interaction_Widget_C|GetBuildingStatus (Variables|BP_Starport_C|GetBuildingInteractionWidget_Ref _array_element_2)) (Utilities|Text|ToText(Integer) (Utilities|Array|Length _outactors_3)) (Variables|/Game/UI_and_Widgets/Colony_and_units_system/BuildingsWidgets/Building_Interaction_Widget.Building_Interaction_Widget_C|GetBuildingSellCost (Variables|BP_Starport_C|GetBuildingInteractionWidget_Ref _array_element_2)) false)))

(event EventTick
  (params (DeltaSeconds :type Float%20%28single-precision%29))
  (CallFunction|LineTrace))

(fn ConstructionScript)

(fn AutoPrisos
  (bind _as_global_game_instance (Variables|Default|GetAs%20Global%20Game%20Instance))
  (bind _indexofplanet (Variables|/Game/SaveGame/GlobalGameInstance.GlobalGameInstance_C|GetIndexOfPlanet _as_global_game_instance))
  (bind _outactors (Actor|GetAllActorsOfClass "/Game/Actors/Buildings/Civilian_Buildings/BP_Energy_Station.BP_Energy_Station_C"))
  (for _array_element _outactors
    (if (<= (Math|Vector|Distance(Vector) (Transformation|GetActorLocation) (Transformation|GetActorLocation _array_element)) (Variables|/Game/SaveGame/GlobalGameInstance.GlobalGameInstance_C|Getrange%20of%20electric (Variables|Default|Getgame%20global%20ref)))
      (if (<= (Math|Vector|Distance(Vector) (Transformation|GetActorLocation) (Transformation|GetActorLocation _array_element)) (Variables|Default|Getmin%20distance))
        (Variables|Default|Setmin%20distance (Math|Vector|Distance(Vector) (Transformation|GetActorLocation) (Transformation|GetActorLocation _array_element)))
        (Variables|Default|Setbp_energy%20station _array_element)
        (Variables|Default|SetGoNextOrNo true))
      (else
        (Development|PrintString "электростанция слишком далеко"))))
  (bind _outactors_2 (Actor|GetAllActorsOfClass "/Game/Actors/Buildings/Civilian_Buildings/BP_EnergyTower.BP_EnergyTower_C"))
  (for _array_element_2 _outactors_2
    (if (Variables|/Game/Actors/Buildings/Civilian_Buildings/BP_EnergyTower.BP_EnergyTower_C|Getalready_work _array_element_2)
      (if (<= (Math|Vector|Distance(Vector) (Transformation|GetActorLocation) (Transformation|GetActorLocation _array_element_2)) (Variables|/Game/SaveGame/GlobalGameInstance.GlobalGameInstance_C|Getrange%20of%20electric (Variables|Default|Getgame%20global%20ref)))
        (if (<= (Math|Vector|Distance(Vector) (Transformation|GetActorLocation) (Transformation|GetActorLocation _array_element_2)) (Variables|Default|Getmin%20distance))
          (Variables|Default|Setmin%20distance (Math|Vector|Distance(Vector) (Transformation|GetActorLocation) (Transformation|GetActorLocation _array_element_2)))
          (Variables|Default|Setbp_energy%20tower _array_element_2)
          (Variables|Default|Setprisoska%20na%20tavek%20ili%20net true)
          (Variables|Default|SetGoNextOrNo true)))))
  (if (Variables|Default|GetGoNextOrNo)
    (bind _ascontroller_cam (Utilities|Casting|CastTocontrollerCam (Game|GetPlayerController 0)))
    (if (<= (Variables|Default|GetHowMuchColonistNeedToWork) (Utilities|Array|Get(acopy) (Variables|/Game/CameraAndControllerStuff/controllerCam.controllerCam_C|GetColonistsPopulation _ascontroller_cam) (Variables|/Game/SaveGame/GlobalGameInstance.GlobalGameInstance_C|GetIndexOfPlanet (Variables|Default|GetAs%20Global%20Game%20Instance))))
      (if (Variables|Default|Getprisoska%20na%20tavek%20ili%20net)
        (Variables|Default|Setint%20for%20delite (- (Variables|/Game/Actors/Buildings/Civilian_Buildings/BP_EnergyTower.BP_EnergyTower_C|Getkakoq%20to%20int (Variables|Default|Getbp_energy%20tower)) 100000))
        (bind _outactors_3 (Actor|GetAllActorsOfClass "/Game/Actors/Buildings/Civilian_Buildings/BP_Energy_Station.BP_Energy_Station_C"))
        (if (not (< (Variables|/Game/Actors/Buildings/Civilian_Buildings/BP_Energy_Station.BP_Energy_Station_C|Getenergy%20cost (Utilities|Array|Get(acopy) _outactors_3 (Variables|/Game/Actors/Buildings/Civilian_Buildings/BP_EnergyTower.BP_EnergyTower_C|Getid%20of%20added%20station (Variables|Default|Getbp_energy%20tower)))) (Variables|Default|Getbuilding%20cost)))
          (Variables|/Game/Actors/Buildings/Civilian_Buildings/BP_Energy_Station.BP_Energy_Station_C|Setenergy%20cost (Utilities|Array|Get(acopy) _outactors_3 (Variables|/Game/Actors/Buildings/Civilian_Buildings/BP_EnergyTower.BP_EnergyTower_C|Getid%20of%20added%20station (Variables|Default|Getbp_energy%20tower))) (- (Variables|/Game/Actors/Buildings/Civilian_Buildings/BP_Energy_Station.BP_Energy_Station_C|Getenergy%20cost (Utilities|Array|Get(acopy) _outactors_3 (Variables|/Game/Actors/Buildings/Civilian_Buildings/BP_EnergyTower.BP_EnergyTower_C|Getid%20of%20added%20station (Variables|Default|Getbp_energy%20tower)))) (Variables|Default|Getbuilding%20cost)))
          (Variables|Default|Setvector (Transformation|GetActorLocation (Variables|Default|Getbp_energy%20tower)))
          (Variables|Default|Setid_added_station (+ (Math|Conversions|ToInteger(Byte) (Utilities|String|GetSubstring (Utilities|GetObjectName (Variables|Default|Getbp_energy%20tower)) 17 3)) 100000))
          (bind _ascontroller_cam_2 (Utilities|Casting|CastTocontrollerCam (Game|GetPlayerController 0) :!label _label))
          (bind _outactors_4 (Actor|GetAllActorsOfClass "/Game/Actors/Planets/Master_Planet_Asset.Master_Planet_Asset_C"))
          (Variables|/Game/Actors/Planets/Master_Planet_Asset.Master_Planet_Asset_C|SetLimitOfPopulation (Utilities|Array|Get(acopy) _outactors_4 _indexofplanet) (- (Variables|/Game/Actors/Planets/Master_Planet_Asset.Master_Planet_Asset_C|GetLimitOfPopulation (Utilities|Array|Get(acopy) _outactors_4 _indexofplanet)) (Variables|Default|GetHowMuchColonistNeedToWork)))
          (Utilities|Array|SetArrayElem (Variables|/Game/CameraAndControllerStuff/controllerCam.controllerCam_C|GetColonistsPopulation _ascontroller_cam_2) _indexofplanet (- (Utilities|Array|Get(acopy) (Variables|/Game/CameraAndControllerStuff/controllerCam.controllerCam_C|GetColonistsPopulation _ascontroller_cam_2) _indexofplanet) (Variables|Default|GetHowMuchColonistNeedToWork)))
          (Variables|Default|SetBuildingIsDoneForWork true)
          (bind _outactors_5 (Actor|GetAllActorsOfClass "BP_Starport_C"))
          (Rendering|Components|TextRender|SetText (Variables|/Game/UI_and_Widgets/Colony_and_units_system/BuildingsWidgets/Building_Interaction_Widget.Building_Interaction_Widget_C|GetTextBlock_270 (Variables|/Game/UI_and_Widgets/Colony_and_units_system/BuildingsWidgets/Starport_Widget.Starport_Widget_C|GetBuilding_Interaction_Widget (Variables|Default|GetStarportWidget_Ref))) "Отключить")
          (Default|GetBuildingInfo (Variables|/Game/UI_and_Widgets/Colony_and_units_system/BuildingsWidgets/Starport_Widget.Starport_Widget_C|GetBuilding_Interaction_Widget (Variables|Default|GetStarportWidget_Ref)) "Звездный Порт" "Здание работает" (Utilities|Text|ToText(Integer) (Utilities|Array|Length _outactors_5)) (Utilities|Text|ToText(Float) (* (Variables|Default|GetSellCost) 1e+02) "HalfToEven") false)
          (CallFunction|LocalWidgettoGlobal))
        (elif (not (< (Variables|/Game/Actors/Buildings/Civilian_Buildings/BP_Energy_Station.BP_Energy_Station_C|Getenergy%20cost (Variables|Default|Getbp_energy%20station)) (Variables|Default|Getbuilding%20cost)))
          (Variables|/Game/Actors/Buildings/Civilian_Buildings/BP_Energy_Station.BP_Energy_Station_C|Setenergy%20cost (Variables|Default|Getbp_energy%20station) (- (Variables|/Game/Actors/Buildings/Civilian_Buildings/BP_Energy_Station.BP_Energy_Station_C|Getenergy%20cost (Variables|Default|Getbp_energy%20station)) (Variables|Default|Getbuilding%20cost)))
          (Variables|Default|Setvector (Transformation|GetActorLocation (Variables|Default|Getbp_energy%20station)))
          (Variables|Default|Setid_added_station (Math|Conversions|ToInteger(Byte) (Utilities|String|GetSubstring (Utilities|GetObjectName (Variables|Default|Getbp_energy%20station)) 20 3)))
          (goto _label)))
      (else
        (Development|PrintString "недостаточно рабочих")))
    (else
      (Development|PrintString "поблизости нет электростанций"))))

(fn CheckStarport
  (bind _outactors (Actor|GetAllActorsOfClass "BP_Starport_C"))
  (bind _array_element (Utilities|Array|ForEachLoopwithBreak _outactors :!label _label)
    (:LoopBody
      (if (== (Variables|/Game/UI_and_Widgets/Colony_and_units_system/BuildingsWidgets/Starport_Widget.Starport_Widget_C|GetDestinationPlanet (Variables|/Game/SaveGame/GlobalGameInstance.GlobalGameInstance_C|GetStarportWidgetOnViewport (Variables|Default|Getgame%20global%20ref))) (Variables|BP_Starport_C|GetNativePlanet _array_element))
        (Variables|Default|SetIsSomeStarportOnPlanet true)
        (Variables|Default|SetStarportForSpawn%20ref _array_element)
        (goto _label Break)))))

(fn NullAllStation
  (bind _as_global_game_instance (Variables|Default|GetAs%20Global%20Game%20Instance))
  (bind _game_global_ref (Variables|Default|Getgame%20global%20ref))
  (bind _idofenergy (Variables|/Game/SaveGame/GlobalGameInstance.GlobalGameInstance_C|Getidofenergy _game_global_ref))
  (bind _indexofplanet (Variables|/Game/SaveGame/GlobalGameInstance.GlobalGameInstance_C|GetIndexOfPlanet _as_global_game_instance))
  (if (> (Variables|/Game/SaveGame/GlobalGameInstance.GlobalGameInstance_C|Getidofenergy (Variables|Default|Getgame%20global%20ref)) 99999)
    (bind _outactors (Actor|GetAllActorsOfClass "/Game/Actors/Buildings/Civilian_Buildings/BP_EnergyTower.BP_EnergyTower_C"))
    (bind _outactors_2 (Actor|GetAllActorsOfClass "/Game/Actors/Buildings/Civilian_Buildings/BP_Energy_Station.BP_Energy_Station_C"))
    (Variables|/Game/Actors/Buildings/Civilian_Buildings/BP_Energy_Station.BP_Energy_Station_C|Setenergy%20cost (Utilities|Array|Get(acopy) _outactors_2 (Variables|/Game/Actors/Buildings/Civilian_Buildings/BP_EnergyTower.BP_EnergyTower_C|Getid%20of%20added%20station (Utilities|Array|Get(acopy) _outactors (- _idofenergy 100000)))) (+ (Variables|Default|Getbuilding%20cost) (Variables|/Game/Actors/Buildings/Civilian_Buildings/BP_Energy_Station.BP_Energy_Station_C|Getenergy%20cost (Utilities|Array|Get(acopy) _outactors_2 (Variables|/Game/Actors/Buildings/Civilian_Buildings/BP_EnergyTower.BP_EnergyTower_C|Getid%20of%20added%20station (Utilities|Array|Get(acopy) _outactors (- _idofenergy 100000)))))))
    (else
      (bind _outactors_3 (Actor|GetAllActorsOfClass "/Game/Actors/Buildings/Civilian_Buildings/BP_Energy_Station.BP_Energy_Station_C"))
      (Variables|/Game/Actors/Buildings/Civilian_Buildings/BP_Energy_Station.BP_Energy_Station_C|Setenergy%20cost (Utilities|Array|Get(acopy) _outactors_3 _idofenergy) (+ (Variables|/Game/Actors/Buildings/Civilian_Buildings/BP_Energy_Station.BP_Energy_Station_C|Getenergy%20cost (Utilities|Array|Get(acopy) _outactors_3 _idofenergy)) (Variables|Default|Getbuilding%20cost)))))
  (Variables|Default|SetBuildingIsDoneForWork false)
  (bind _ascontroller_cam (Utilities|Casting|CastTocontrollerCam (Game|GetPlayerController 0)))
  (bind _outactors_4 (Actor|GetAllActorsOfClass "/Game/Actors/Planets/Master_Planet_Asset.Master_Planet_Asset_C"))
  (Variables|/Game/Actors/Planets/Master_Planet_Asset.Master_Planet_Asset_C|SetLimitOfPopulation (Utilities|Array|Get(acopy) _outactors_4) (+ (Variables|/Game/Actors/Planets/Master_Planet_Asset.Master_Planet_Asset_C|GetLimitOfPopulation (Utilities|Array|Get(acopy) _outactors_4)) (Variables|Default|GetHowMuchColonistNeedToWork)))
  (Utilities|Array|SetArrayElem (Variables|/Game/CameraAndControllerStuff/controllerCam.controllerCam_C|GetColonistsPopulation _ascontroller_cam) _indexofplanet (+ (Utilities|Array|Get(acopy) (Variables|/Game/CameraAndControllerStuff/controllerCam.controllerCam_C|GetColonistsPopulation _ascontroller_cam) _indexofplanet) (Variables|Default|GetHowMuchColonistNeedToWork)))
  (Rendering|Components|TextRender|SetText (Variables|/Game/UI_and_Widgets/Colony_and_units_system/BuildingsWidgets/Building_Interaction_Widget.Building_Interaction_Widget_C|GetTextBlock_270 (Variables|/Game/UI_and_Widgets/Colony_and_units_system/BuildingsWidgets/Starport_Widget.Starport_Widget_C|GetBuilding_Interaction_Widget (Variables|Default|GetStarportWidget_Ref))) "Подключить")
  (bind _outactors_5 (Actor|GetAllActorsOfClass "BP_Starport_C"))
  (Default|GetBuildingInfo (Variables|/Game/UI_and_Widgets/Colony_and_units_system/BuildingsWidgets/Starport_Widget.Starport_Widget_C|GetBuilding_Interaction_Widget (Variables|Default|GetStarportWidget_Ref)) "Звездный Порт" "Неактивен" (Utilities|Text|ToText(Integer) (Utilities|Array|Length _outactors_5)) (Utilities|Text|ToText(Float) (* (Variables|Default|GetSellCost) 1e+02) "HalfToEven") false)
  (CallFunction|LocalWidgettoGlobal))

(fn LineTrace
  (if (Variables|Default|GetBuildingIsDoneForWork)
    (Collision|LineTraceByChannel (+ (Math|Vector|GetUnitDirection(Vector) (Variables|Default|GetWorldOrigin) (Variables|Default|Getvector)) (Variables|Default|Getvector)) (+ (* (Math|Vector|GetUnitDirection(Vector) (Variables|Default|GetWorldOrigin) (Transformation|GetActorLocation)) "1000.000000,1000.000000,1000.000000") (Transformation|GetActorLocation)) "TraceTypeQuery1" false 0 "ForDuration" false "(R=0.000000,G=0.000000,B=0.000000,A=1.000000)" "(R=0.000000,G=0.000000,B=0.000000,A=1.000000)" 0.2)))

(fn LocalWidgettoGlobal
  (bind _starportwidget_ref (Variables|Default|GetStarportWidget_Ref))
  (bind _building_interaction_widget (Variables|/Game/UI_and_Widgets/Colony_and_units_system/BuildingsWidgets/Starport_Widget.Starport_Widget_C|GetBuilding_Interaction_Widget _starportwidget_ref))
  (Rendering|Components|TextRender|SetText (Variables|/Game/UI_and_Widgets/Colony_and_units_system/BuildingsWidgets/Building_Interaction_Widget.Building_Interaction_Widget_C|GetTextBlock_270 (Variables|/Game/UI_and_Widgets/Colony_and_units_system/BuildingsWidgets/Starport_Widget.Starport_Widget_C|GetBuilding_Interaction_Widget (Variables|/Game/SaveGame/GlobalGameInstance.GlobalGameInstance_C|GetStarportWidgetOnViewport (Variables|Default|GetAs%20Global%20Game%20Instance)))) (Variables|/Script/UMG.TextBlock|GetText (Variables|/Game/UI_and_Widgets/Colony_and_units_system/BuildingsWidgets/Building_Interaction_Widget.Building_Interaction_Widget_C|GetTextBlock_270 (Variables|/Game/UI_and_Widgets/Colony_and_units_system/BuildingsWidgets/Starport_Widget.Starport_Widget_C|GetBuilding_Interaction_Widget (Variables|Default|GetStarportWidget_Ref)))))
  (Default|GetBuildingInfo (Variables|/Game/UI_and_Widgets/Colony_and_units_system/BuildingsWidgets/Starport_Widget.Starport_Widget_C|GetBuilding_Interaction_Widget (Variables|/Game/SaveGame/GlobalGameInstance.GlobalGameInstance_C|GetStarportWidgetOnViewport (Variables|Default|GetAs%20Global%20Game%20Instance))) (Variables|/Game/UI_and_Widgets/Colony_and_units_system/BuildingsWidgets/Building_Interaction_Widget.Building_Interaction_Widget_C|GetBuildingName _building_interaction_widget) (Variables|/Game/UI_and_Widgets/Colony_and_units_system/BuildingsWidgets/Building_Interaction_Widget.Building_Interaction_Widget_C|GetBuildingStatus _building_interaction_widget) (Variables|/Game/UI_and_Widgets/Colony_and_units_system/BuildingsWidgets/Building_Interaction_Widget.Building_Interaction_Widget_C|GetBuildingAmount _building_interaction_widget) (Variables|/Game/UI_and_Widgets/Colony_and_units_system/BuildingsWidgets/Building_Interaction_Widget.Building_Interaction_Widget_C|GetBuildingSellCost _building_interaction_widget) false))