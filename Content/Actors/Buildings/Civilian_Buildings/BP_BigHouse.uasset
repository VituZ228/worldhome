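; Residential complex building that raises the current planet's population limit while it stands.
; On BeginPlay it deducts its Cost from player resources, updates every house's info widget and spawns three Colonist2 actors at staggered intervals, offset away from the planet.
; The shared sell button destroys only houses with custom depth enabled.
; Destruction plays a coin effect, refunds a SellCost fraction, lowers the limit and trims excess colonists.
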(event Custom|SellBtn_Pressed_Event
  ;[0 0.1566 1] СЛЕДИТ ЗА НАЖАТИЕМ НА КНОПКУ ПРОДАЖИ, ПРИ НАЖАТИИ ВОЗВРАЩАЕТ ЦЕНУ ЗДАНИЯ УМНОЖЕНУЮ НА ПРОЦЕНТ SellCost
  (if (Variables|/Script/Engine.PrimitiveComponent|GetbRenderCustomDepth (Variables|Default|GetBuildMesh))
    (Actor|DestroyActor)))

(event Custom|new%20spawn
  (bind _returnvalue (Transformation|GetActorLocation))
  (bind _returnvalue_2 (Game|SpawnActorfromClass "/Game/Actors/Units/chuvachochki/colonist2.colonist2_C" (Math|Transform|MakeTransform (+ (* (Math|Vector|GetUnitDirection(Vector) (Variables|Default|Getworld%20origin) _returnvalue) "10000.000000,10000.000000,10000.000000") _returnvalue) (Transformation|GetActorRotation) "1.000000,1.000000,1.000000") "AlwaysSpawn" "MultiplyWithRoot" 0 0))
  (Default|IndexOfHouse _returnvalue_2 self))

(event EventDestroyed
  (bind _returnvalue (Transformation|GetActorLocation))
  (Effects|SpawnEmitteratLocation "/Game/VFX_Toolkit_V1/ParticleSystems/356Days/Par_LuCoins.Par_LuCoins" (+ (* (Math|Vector|GetUnitDirection(Vector) "0.000000,10000.000000,1000.000000" _returnvalue) "10000.000000,10000.000000,10000.000000") _returnvalue) (Transformation|GetActorRotation) "50.000000,50.000000,50.000000")
  ;[0 0.1566 1] СЛЕДИТ ЗА НАЖАТИЕМ НА КНОПКУ ПРОДАЖИ, ПРИ НАЖАТИИ ВОЗВРАЩАЕТ ЦЕНУ ЗДАНИЯ УМНОЖЕНУЮ НА ПРОЦЕНТ SellCost
  (Widget|SetVisibility (Variables|/Game/SaveGame/GlobalGameInstance.GlobalGameInstance_C|GetBuildingInteractionOnViewport (Variables|Default|GetAsGlobalGameInstance)) "Hidden")
  (bind _outactors (Actor|GetAllActorsOfClass "/Game/CameraAndControllerStuff/controllerCam.controllerCam_C"))
  (for (_array_element _array_index) (Variables|Default|GetCost)
    (Utilities|Array|SetArrayElem (Variables|/Game/CameraAndControllerStuff/controllerCam.controllerCam_C|GetPlayerRessourses (Utilities|Array|Get(acopy) _outactors)) _array_index (+ (Utilities|Array|Get(acopy) (Variables|/Game/CameraAndControllerStuff/controllerCam.controllerCam_C|GetPlayerRessourses (Utilities|Array|Get(acopy) _outactors)) _array_index) (* _array_element (Variables|Default|GetSellCost)))))
  ;[0 0.1139 1] КОГДА ЗДАНИЕ СНОСИТСЯ ОТНИМАЕТ У ИГРОКА ЛИМИТ НАСЕЛЕНИЯ И КОЛОНИСТОВ УХОДЯЩИХ ЗА ЭТОТ ЛИМИТ
  (bind _ascontroller_cam (Utilities|Casting|CastTocontrollerCam (Game|GetPlayerController 0)))
  (bind _asglobal_game_instance (Utilities|Casting|CastToGlobalGameInstance (Game|GetGameInstance)))
  (bind _outactors_2 (Actor|GetAllActorsOfClass "/Game/Actors/Planets/Master_Planet_Asset.Master_Planet_Asset_C"))
  (bind _output_get (Variables|/Game/Actors/Planets/Master_Planet_Asset.Master_Planet_Asset_C|SetLimitOfPopulation (Utilities|Array|Get(acopy) _outactors_2 (Variables|/Game/SaveGame/GlobalGameInstance.GlobalGameInstance_C|GetIndexOfPlanet _asglobal_game_instance)) (- (Variables|/Game/Actors/Planets/Master_Planet_Asset.Master_Planet_Asset_C|GetLimitOfPopulation (Utilities|Array|Get(acopy) _outactors_2 (Variables|/Game/SaveGame/GlobalGameInstance.GlobalGameInstance_C|GetIndexOfPlanet _asglobal_game_instance))) 300)))
  (while (> (Utilities|Array|Get(acopy) (Variables|/Game/CameraAndControllerStuff/controllerCam.controllerCam_C|GetColonistsPopulation _ascontroller_cam) (Variables|/Game/SaveGame/GlobalGameInstance.GlobalGameInstance_C|GetIndexOfPlanet _asglobal_game_instance)) _output_get)
    (Utilities|Array|SetArrayElem (Variables|/Game/CameraAndControllerStuff/controllerCam.controllerCam_C|GetColonistsPopulation _ascontroller_cam) (Variables|/Game/SaveGame/GlobalGameInstance.GlobalGameInstance_C|GetIndexOfPlanet _asglobal_game_instance) (- (Utilities|Array|Get(acopy) (Variables|/Game/CameraAndControllerStuff/controllerCam.controllerCam_C|GetColonistsPopulation _ascontroller_cam) (Variables|/Game/SaveGame/GlobalGameInstance.GlobalGameInstance_C|GetIndexOfPlanet _asglobal_game_instance)) 1))
    (bind _outactors_3 (Actor|GetAllActorsOfClass "BP_BigHouse_C"))
    (for _array_element_2 _outactors_3
      (bind _asbuilding_interaction_widget (Utilities|Casting|CastToBuilding_Interaction_Widget (UserInterface|GetWidget (Variables|BP_BigHouse_C|GetBuildingWidget _array_element_2))))
      (Default|GetBuildingInfo _asbuilding_interaction_widget "Жилой комплекс" (Variables|/Game/UI_and_Widgets/Colony_and_units_system/BuildingsWidgets/Building_Interaction_Widget.Building_Interaction_Widget_C|GetBuildingStatus _asbuilding_interaction_widget) (Utilities|Text|ToText(Integer) (- (Utilities|Array|Length _outactors_3) 1)) (Utilities|Text|ToText(Float) (* (Variables|Default|GetSellCost) 1e+02) "HalfToEven") true))))

(event EventBeginPlay
  (bind _outactors (Actor|GetAllActorsOfClass "/Game/Actors/Planets/Master_Planet_BigVer_Asset.Master_Planet_BigVer_Asset_C"))
  (bind _asglobal_game_instance (Utilities|Casting|CastToGlobalGameInstance (Game|GetGameInstance)))
  (Variables|Default|Setworld%20origin (Transformation|GetActorLocation (Utilities|Array|Get(acopy) _outactors (Variables|/Game/SaveGame/GlobalGameInstance.GlobalGameInstance_C|GetIndexOfPlanet _asglobal_game_instance))))
  (bind _asglobal_game_instance_2 (Utilities|Casting|CastToGlobalGameInstance (Game|GetGameInstance)))
  (Variables|Default|SetAsGlobalGameInstance _asglobal_game_instance_2)
  (bind _asbuilding_interaction_widget (Utilities|Casting|CastToBuilding_Interaction_Widget (UserInterface|GetWidget (Variables|Default|GetBuildingWidget))))
  (Variables|Default|SetBuildingInteraction_Ref _asbuilding_interaction_widget)
  ;[0.2434 0 1] ОТНИМАЕТ У ИГРОКА КОЛ-ВО РЕССУРСОВ НА ПОСТРОЙКУ ЗНАНИЯ СООТВЕТСТВУЮЩЕЕ ПЕРЕМЕННОЙ Cost
  (bind _ascontroller_cam (Utilities|Casting|CastTocontrollerCam (Game|GetPlayerController 0)))
  (Variables|Default|SetControllerCam_Ref _ascontroller_cam)
  (for (_array_element _array_index) (Variables|Default|GetCost)
    (Utilities|Array|SetArrayElem (Variables|/Game/CameraAndControllerStuff/controllerCam.controllerCam_C|GetPlayerRessourses (Variables|Default|GetControllerCam_Ref)) _array_index (- (Utilities|Array|Get(acopy) (Variables|/Game/CameraAndControllerStuff/controllerCam.controllerCam_C|GetPlayerRessourses (Variables|Default|GetControllerCam_Ref)) _array_index) _array_element)))
  ;[0 0.1566 1] СЛЕДИТ ЗА НАЖАТИЕМ НА КНОПКУ ПРОДАЖИ, ПРИ НАЖАТИИ ВОЗВРАЩАЕТ ЦЕНУ ЗДАНИЯ УМНОЖЕНУЮ НА ПРОЦЕНТ SellCost
  (EventDispatchers|AssignSellBtnPressed (Variables|/Game/SaveGame/GlobalGameInstance.GlobalGameInstance_C|GetBuildingInteractionOnViewport (Variables|Default|GetAsGlobalGameInstance)) (delegate Custom|SellBtn_Pressed_Event))
  (bind _outactors_2 (Actor|GetAllActorsOfClass "BP_BigHouse_C"))
  (for _array_element_2 _outactors_2
    (bind _asbuilding_interaction_widget_2 (Utilities|Casting|CastToBuilding_Interaction_Widget (UserInterface|GetWidget (Variables|BP_BigHouse_C|GetBuildingWidget _array_element_2))))
    (Default|GetBuildingInfo _asbuilding_interaction_widget_2 "Жилой комплекс" "Активен" (Utilities|Text|ToText(Integer) (Utilities|Array|Length _outactors_2)) (Utilities|Text|ToText(Float) (* (Variables|Default|GetSellCost) 1e+02) "HalfToEven") true))
  (bind _asglobal_game_instance_3 (Utilities|Casting|CastToGlobalGameInstance (Game|GetGameInstance)))
  (bind _ascontroller_cam_2 (Utilities|Casting|CastTocontrollerCam (Game|GetPlayerController 0)))
  (bind _outactors_3 (Actor|GetAllActorsOfClass "/Game/Actors/Planets/Master_Planet_Asset.Master_Planet_Asset_C"))
  (Variables|/Game/Actors/Planets/Master_Planet_Asset.Master_Planet_Asset_C|SetLimitOfPopulation (Utilities|Array|Get(acopy) _outactors_3 (Variables|/Game/SaveGame/GlobalGameInstance.GlobalGameInstance_C|GetIndexOfPlanet _asglobal_game_instance_3)) (+ (Variables|/Game/Actors/Planets/Master_Planet_Asset.Master_Planet_Asset_C|GetLimitOfPopulation (Utilities|Array|Get(acopy) _outactors_3 (Variables|/Game/SaveGame/GlobalGameInstance.GlobalGameInstance_C|GetIndexOfPlanet _asglobal_game_instance_3))) 300))
  (CallFunction|NewSpawn)
  (Utilities|FlowControl|Delay 2.0)
  (CallFunction|NewSpawn)
  (Utilities|FlowControl|Delay 2.0)
  (CallFunction|NewSpawn))

(event EventTick
  (params (DeltaSeconds :type Float%20%28single-precision%29)))

(fn ConstructionScript)