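; BP_MainHouse is a civilian colony building that can be bought and sold.
; Unless owned by BP_MainBot, BeginPlay adds colony food, deducts Cost from player resources, and pins a house widget onto the matching Master_Planet_Asset using a line-trace face index.
; The shared sell button destroys the house when its custom-depth highlight is on, refunding a SellCost fraction.
; Spawning and destruction also refresh every energy station's info widget.
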(event Custom|SellBtn_Pressed_Event
  ;[0 0.1566 1] СЛЕДИТ ЗА НАЖАТИЕМ НА КНОПКУ ПРОДАЖИ, ПРИ НАЖАТИИ ВОЗВРАЩАЕТ ЦЕНУ ЗДАНИЯ УМНОЖЕНУЮ НА ПРОЦЕНТ SellCost
  (if (Variables|/Script/Engine.PrimitiveComponent|GetbRenderCustomDepth (Variables|Default|GetSkeletalMesh))
    (Actor|DestroyActor)))

(event EventBeginPlay
  (bind _outactors (Actor|GetAllActorsOfClass "/Game/CameraAndControllerStuff/cameraplayer.cameraplayer_C"))
  ;[1 1 1] НОмер игрока
  (Variables|Default|SetCameraplayer (Utilities|Array|Get(acopy) _outactors))
  (Variables|Default|Settransform (Transformation|GetActorTransform (Utilities|Array|Get(acopy) _outactors)))
  (bind _outactors_2 (Actor|GetAllActorsOfClass "/Game/Actors/Planets/Master_Planet_BigVer_Asset.Master_Planet_BigVer_Asset_C"))
  (Variables|Default|SetNewVar_0 (Utilities|Array|Get(acopy) _outactors_2))
  (bind _asglobal_game_instance (Utilities|Casting|CastToGlobalGameInstance (Game|GetGameInstance)))
  (bind _output_get (Variables|Default|SetGlobalGameInstance_Ref _asglobal_game_instance))
  (if (Utilities|Enum|Equal(Enum) (Utilities|String|LeftChop (Utilities|GetObjectName (Components|GetOwner)) 4) "BP_MainBot")
    _
    (else
      (bind _ascontroller_cam (Utilities|Casting|CastTocontrollerCam (Game|GetPlayerController 0)))
      (Variables|Default|SetControllerCam_Ref _ascontroller_cam)
      (Utilities|Array|SetArrayElem (Variables|/Game/CameraAndControllerStuff/controllerCam.controllerCam_C|GetColoniesFood (Variables|Default|GetControllerCam_Ref)) (Variables|Default|GetCurrentPlanet) (+ (Utilities|Array|Get(acopy) (Variables|/Game/CameraAndControllerStuff/controllerCam.controllerCam_C|GetColoniesFood (Variables|Default|GetControllerCam_Ref)) (Variables|Default|GetCurrentPlanet)) 50))
      (Variables|Default|SetCurrentPlanet (Variables|/Game/SaveGame/GlobalGameInstance.GlobalGameInstance_C|GetIndexOfPlanet _output_get))
      ;[0.2434 0 1] ОТНИМАЕТ У ИГРОКА КОЛ-ВО РЕССУРСОВ НА ПОСТРОЙКУ ЗНАНИЯ СООТВЕТСТВУЮЩЕЕ ПЕРЕМЕННОЙ Cost
      (CallFunction|NewFunction)
      (for (_array_element _array_index) (Variables|Default|GetCost)
        (Utilities|Array|SetArrayElem (Variables|/Game/CameraAndControllerStuff/controllerCam.controllerCam_C|GetPlayerRessourses (Variables|Default|GetControllerCam_Ref)) _array_index (- (Utilities|Array|Get(acopy) (Variables|/Game/CameraAndControllerStuff/controllerCam.controllerCam_C|GetPlayerRessourses (Variables|Default|GetControllerCam_Ref)) _array_index) _array_element)))))
  (bind _asbuilding_interaction_widget (Utilities|Casting|CastToBuilding_Interaction_Widget (UserInterface|GetWidget (Variables|Default|GetBuildingWidget))))
  (Variables|Default|SetBuildingInteraction_Ref _asbuilding_interaction_widget)
  (bind _asglobal_game_instance_2 (Utilities|Casting|CastToGlobalGameInstance (Game|GetGameInstance)))
  (Variables|Default|SetGlobalGameInstance_Ref _asglobal_game_instance_2)
  ;[0 0.1566 1] СЛЕДИТ ЗА НАЖАТИЕМ НА КНОПКУ ПРОДАЖИ, ПРИ НАЖАТИИ ВОЗВРАЩАЕТ ЦЕНУ ЗДАНИЯ УМНОЖЕНУЮ НА ПРОЦЕНТ SellCost
  (EventDispatchers|AssignSellBtnPressed (Variables|/Game/SaveGame/GlobalGameInstance.GlobalGameInstance_C|GetBuildingInteractionOnViewport (Variables|Default|GetGlobalGameInstance_Ref)) (delegate Custom|SellBtn_Pressed_Event))
  (bind _outactors_3 (Actor|GetAllActorsOfClass "/Game/Actors/Buildings/Civilian_Buildings/BP_Energy_Station.BP_Energy_Station_C"))
  (for _array_element_2 _outactors_3
    (bind _asbuilding_interaction_widget_2 (Utilities|Casting|CastToBuilding_Interaction_Widget (UserInterface|GetWidget (Variables|/Game/Actors/Buildings/Civilian_Buildings/BP_Energy_Station.BP_Energy_Station_C|GetBuildingWidget _array_element_2))))
    (Default|GetBuildingInfo _asbuilding_interaction_widget_2 "Электростанция" "Активен" (Utilities|Text|ToText(Integer) (Utilities|Array|Length _outactors_3)) (Utilities|Text|ToText(Float) (* (Variables|Default|GetSellCost) 1e+02) "HalfToEven") true)))

(event EventDestroyed
  ;[0 0.1566 1] СЛЕДИТ ЗА НАЖАТИЕМ НА КНОПКУ ПРОДАЖИ, ПРИ НАЖАТИИ ВОЗВРАЩАЕТ ЦЕНУ ЗДАНИЯ УМНОЖЕНУЮ НА ПРОЦЕНТ SellCost
  (Widget|SetVisibility (Variables|/Game/SaveGame/GlobalGameInstance.GlobalGameInstance_C|GetBuildingInteractionOnViewport (Variables|Default|GetGlobalGameInstance_Ref)) "Hidden")
  (bind _outactors (Actor|GetAllActorsOfClass "/Game/CameraAndControllerStuff/controllerCam.controllerCam_C"))
  (for (_array_element _array_index) (Variables|Default|GetCost)
    (Utilities|Array|SetArrayElem (Variables|/Game/CameraAndControllerStuff/controllerCam.controllerCam_C|GetPlayerRessourses (Utilities|Array|Get(acopy) _outactors)) _array_index (+ (Utilities|Array|Get(acopy) (Variables|/Game/CameraAndControllerStuff/controllerCam.controllerCam_C|GetPlayerRessourses (Utilities|Array|Get(acopy) _outactors)) _array_index) (* _array_element (Variables|Default|GetSellCost)))))
  (bind _outactors_2 (Actor|GetAllActorsOfClass "/Game/Actors/Buildings/Civilian_Buildings/BP_Energy_Station.BP_Energy_Station_C"))
  (for _array_element_2 _outactors_2
    (bind _asbuilding_interaction_widget (Utilities|Casting|CastToBuilding_Interaction_Widget (UserInterface|GetWidget (Variables|/Game/Actors/Buildings/Civilian_Buildings/BP_Energy_Station.BP_Energy_Station_C|GetBuildingWidget _array_element_2))))
    (Default|GetBuildingInfo _asbuilding_interaction_widget "Электростанция" (Variables|/Game/UI_and_Widgets/Colony_and_units_system/BuildingsWidgets/Building_Interaction_Widget.Building_Interaction_Widget_C|GetBuildingStatus _asbuilding_interaction_widget) (Utilities|Text|ToText(Integer) (- (Utilities|Array|Length _outactors_2) 1)) (Utilities|Text|ToText(Float) (* (Variables|Default|GetSellCost) 1e+02) "HalfToEven") true)))

(event EventTick
  (params (DeltaSeconds :type Float%20%28single-precision%29)))

(fn ConstructionScript)

(fn NewFunction
  (bind _returnvalue (Transformation|GetActorLocation))
  (bind _outactors (Actor|GetAllActorsOfClass "/Game/Actors/Planets/Master_Planet_BigVer_Asset.Master_Planet_BigVer_Asset_C"))
  (bind _output_get (Variables|Default|Setworld%20origin (Transformation|GetActorLocation (Utilities|Array|Get(acopy) _outactors (Variables|/Game/SaveGame/GlobalGameInstance.GlobalGameInstance_C|GetIndexOfPlanet (Variables|Default|GetGlobalGameInstance_Ref))))))
  (bind _outhit (Collision|LineTraceByChannel _output_get (+ (* (Math|Vector|GetUnitDirection(Vector) (Variables|Default|Getworld%20origin) _returnvalue) "10000.000000,10000.000000,10000.000000") _returnvalue) "TraceTypeQuery1" false 0 "ForOneFrame" true "(R=1.000000,G=0.000000,B=0.000000,A=1.000000)" "(R=0.000000,G=1.000000,B=0.000000,A=1.000000)" 1.0))
  (bind _outactors_2 (Actor|GetAllActorsOfClass "/Game/Actors/Planets/Master_Planet_Asset.Master_Planet_Asset_C"))
  (bind _returnvalue_2 (UserInterface|CreateWidget "/Game/UI_and_Widgets/Main_Houses_Widget.Main_Houses_Widget_C"))
  (bind _returnvalue_3 (AddComponent|AddWidgetComponent (Utilities|Array|Get(acopy) _outactors_2 (Variables|/Game/SaveGame/GlobalGameInstance.GlobalGameInstance_C|GetIndexOfPlanet (Variables|Default|GetGlobalGameInstance_Ref))) false (Math|Transform|MakeTransform (* (Utilities|Array|Get(acopy) (Variables|/Game/Actors/Planets/Master_Planet_BigVer_Asset.Master_Planet_BigVer_Asset_C|GetVertex (Utilities|Array|Get(acopy) _outactors (Variables|/Game/SaveGame/GlobalGameInstance.GlobalGameInstance_C|GetIndexOfPlanet (Variables|Default|GetGlobalGameInstance_Ref)))) (Utilities|Array|Get(acopy) (Variables|/Game/Actors/Planets/Master_Planet_BigVer_Asset.Master_Planet_BigVer_Asset_C|GetTriagles (Utilities|Array|Get(acopy) _outactors (Variables|/Game/SaveGame/GlobalGameInstance.GlobalGameInstance_C|GetIndexOfPlanet (Variables|Default|GetGlobalGameInstance_Ref)))) (* (.FaceIndex (Collision|BreakHitResult _outhit)) 3))) "1.200000,1.200000,1.200000") (Class|KismetMathLibrary|QuatRotator (Class|KismetMathLibrary|QuatFindBetweenNormals (Class|KismetMathLibrary|VectorBackward) (.Normal (Collision|BreakHitResult _outhit)))) "1.000000,1.000000,1.000000")))
  (UserInterface|SetWidget _returnvalue_3 _returnvalue_2)
  (Variables|/Game/UI_and_Widgets/Main_Houses_Widget.Main_Houses_Widget_C|SetNewVar _returnvalue_2 (Variables|Default|Gettransform))
  (Variables|Default|Sethui _returnvalue_3))