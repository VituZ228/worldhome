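; Power station building actor that players click to toggle a mouse-to-station energy line.
; On BeginPlay it refreshes the info widget on every station with Russian name and status text, station count and sell cost.
; Clicking the mesh flips the global ActiveEnergy flag and stores an ID parsed from the object's name in the GameInstance.
; While active, the matching station draws the line each Tick with a debug line trace whose result is unused.
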(event OnClicked(BuildMesh)
  (params (TouchedComponent :type Primitive%20Component%20Object%20Reference) (ButtonPressed :type Key%20Structure :default "None"))
  (bind _globalgameinstance_ref (Variables|Default|GetGlobalGameInstance_Ref))
  (if (Variables|/Game/SaveGame/GlobalGameInstance.GlobalGameInstance_C|GetActive_Energy _globalgameinstance_ref)
    (Variables|/Game/SaveGame/GlobalGameInstance.GlobalGameInstance_C|SetActive_Energy _globalgameinstance_ref false)
    (else
      (Variables|/Game/SaveGame/GlobalGameInstance.GlobalGameInstance_C|SetActive_Energy _globalgameinstance_ref true)))
  (Variables|/Game/SaveGame/GlobalGameInstance.GlobalGameInstance_C|Setidofenergy _globalgameinstance_ref (Math|Conversions|ToInteger(Byte) (Utilities|String|GetSubstring (Utilities|GetObjectName self) 20 2))))

(event EventBeginPlay
  (bind _asglobal_game_instance (Utilities|Casting|CastToGlobalGameInstance (Game|GetGameInstance)))
  (Variables|Default|SetGlobalGameInstance_Ref _asglobal_game_instance)
  (bind _outactors (Actor|GetAllActorsOfClass "BP_Energy_Station_C"))
  (for _array_element _outactors
    (bind _asbuilding_interaction_widget (Utilities|Casting|CastToBuilding_Interaction_Widget (UserInterface|GetWidget (Variables|BP_Energy_Station_C|GetBuildingWidget _array_element))))
    (Default|GetBuildingInfo _asbuilding_interaction_widget "Электростанция" "Активен" (Utilities|Text|ToText(Integer) (Utilities|Array|Length _outactors)) "50 %" true)))

(event EventTick
  (params (DeltaSeconds :type Float%20%28single-precision%29))
  (bind _globalgameinstance_ref (Variables|Default|GetGlobalGameInstance_Ref))
  (if (== (Variables|/Game/SaveGame/GlobalGameInstance.GlobalGameInstance_C|Getidofenergy _globalgameinstance_ref) (Math|Conversions|ToInteger(Byte) (Utilities|String|GetSubstring (Utilities|GetObjectName self) 20 2)))
    (if (Variables|/Game/SaveGame/GlobalGameInstance.GlobalGameInstance_C|GetActive_Energy _globalgameinstance_ref)
      (Collision|LineTraceByChannel (.WorldLocation (Game|Player|ConvertMouseLocationToWorldSpace (Game|GetPlayerController 0))) (Transformation|GetActorLocation) "TraceTypeQuery1" false 0 "ForDuration" false "(R=0.000000,G=0.000000,B=0.000000,A=1.000000)" "(R=0.000000,G=0.000000,B=0.000000,A=1.000000)" 0.02))))

(fn ConstructionScript)