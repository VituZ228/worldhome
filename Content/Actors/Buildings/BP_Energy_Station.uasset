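; BP_Energy_Station is a clickable building actor that toggles an energy link mode shared through GlobalGameInstance.
; Clicking its mesh flips ActiveEnergy and stores the station's ID, parsed from two characters of its object name.
; While active, the matching station's Tick draws a line from the deprojected mouse position to itself.
; The line is the debug drawing of a visibility trace whose hit result is unused.
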(event OnClicked(StaticMesh)
  (params (TouchedComponent :type Primitive%20Component%20Object%20Reference) (ButtonPressed :type Key%20Structure :default "None"))
  (bind _asglobal_game_instance (Utilities|Casting|CastToGlobalGameInstance (Game|GetGameInstance)))
  (if (Variables|/Game/SaveGame/GlobalGameInstance.GlobalGameInstance_C|GetActive_Energy _asglobal_game_instance)
    (Variables|/Game/SaveGame/GlobalGameInstance.GlobalGameInstance_C|SetActive_Energy _asglobal_game_instance false)
    (else
      (Variables|/Game/SaveGame/GlobalGameInstance.GlobalGameInstance_C|SetActive_Energy _asglobal_game_instance true)))
  (Variables|/Game/SaveGame/GlobalGameInstance.GlobalGameInstance_C|Setidofenergy _asglobal_game_instance (Math|Conversions|ToInteger(Byte) (Utilities|String|GetSubstring (Utilities|GetObjectName self) 20 2))))

(event EventBeginPlay)

(event EventTick
  (params (DeltaSeconds :type Float%20%28single-precision%29))
  (bind _asglobal_game_instance (Utilities|Casting|CastToGlobalGameInstance (Game|GetGameInstance)))
  (if (== (Variables|/Game/SaveGame/GlobalGameInstance.GlobalGameInstance_C|Getidofenergy _asglobal_game_instance) (Math|Conversions|ToInteger(Byte) (Utilities|String|GetSubstring (Utilities|GetObjectName self) 20 2)))
    (if (Variables|/Game/SaveGame/GlobalGameInstance.GlobalGameInstance_C|GetActive_Energy _asglobal_game_instance)
      (Collision|LineTraceByChannel (.WorldLocation (Game|Player|ConvertMouseLocationToWorldSpace (Game|GetPlayerController 0))) (Transformation|GetActorLocation) "TraceTypeQuery1" false 0 "ForDuration" false "(R=0.000000,G=0.000000,B=0.000000,A=1.000000)" "(R=0.000000,G=0.000000,B=0.000000,A=1.000000)" 0.02))))

(fn ConstructionScript)