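; BP_BigHouse is a building actor that adds 300 to the current planet's colonist population and spawns Colonists when play begins.
; It takes the planet index from GlobalGameInstance and uses that Master_Planet_BigVer_Asset actor's location as the planet center.
; Three spawns run two seconds apart, each offset from the house along the direction away from that center.
; Each Colonist gets a default controller and a reference to the house.
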(event Custom|new%20spawn
  (bind _returnvalue (Game|SpawnActorfromClass "/Game/Actors/Units/chuvachochki/colonist.colonist_C" (Math|Transform|MakeTransform (+ (* (Math|Vector|GetUnitDirection(Vector) (Variables|Default|Getworld) (Transformation|GetActorLocation)) "1000.000000,1000.000000,1200.000000") (Transformation|GetActorLocation)) (Transformation|GetActorRotation) "1.000000,1.000000,1.000000") "Undefined" "MultiplyWithRoot" 0 0))
  (Pawn|SpawnDefaultController _returnvalue)
  (Default|IndexOfHouse _returnvalue self))

(event EventBeginPlay
  (bind _outactors (Actor|GetAllActorsOfClass "/Game/Actors/Planets/Master_Planet_BigVer_Asset.Master_Planet_BigVer_Asset_C"))
  (bind _asglobal_game_instance (Utilities|Casting|CastToGlobalGameInstance (Game|GetGameInstance)))
  (Variables|Default|Setworld (Transformation|GetActorLocation (Utilities|Array|Get(acopy) _outactors (Variables|/Game/SaveGame/GlobalGameInstance.GlobalGameInstance_C|GetIndexOfPlanet _asglobal_game_instance))))
  (bind _output_get (Variables|Default|SetCurrent_planet (Variables|/Game/SaveGame/GlobalGameInstance.GlobalGameInstance_C|GetIndexOfPlanet _asglobal_game_instance)))
  (Utilities|Array|SetArrayElem (Variables|/Game/SaveGame/GlobalGameInstance.GlobalGameInstance_C|GetColonistsPopulation _asglobal_game_instance) _output_get (+ (Utilities|Array|Get(acopy) (Variables|/Game/SaveGame/GlobalGameInstance.GlobalGameInstance_C|GetColonistsPopulation _asglobal_game_instance) _output_get) 300))
  (CallFunction|NewSpawn)
  (Utilities|FlowControl|Delay 2.0)
  (CallFunction|NewSpawn)
  (Utilities|FlowControl|Delay 2.0)
  (CallFunction|NewSpawn))

(fn ConstructionScript)