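; BP_Dust_Cloud is a placeable self-shadowed dust cloud for the asteroid field scene, rendered on a ContainerBox component.
; The construction script creates a dynamic instance of MI_Dust_Cloud and feeds it the actor's depth, density and lit and depth color variables.
; It also passes the negated forward vector of a referenced DirectionalLight as the light direction, so that direction is set at construction, with no runtime logic.
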(event EventBeginPlay)

(event Collision|EventActorBeginOverlap
  (params (OtherActor :type Actor%20Object%20Reference)))

(event EventTick
  (params (DeltaSeconds :type Float%20%28single-precision%29)))

(fn ConstructionScript
  (bind _returnvalue (Rendering|Material|CreateDynamicMaterialInstance (Variables|Default|GetContainer_Box) 0 "/Game/Cosmic_Forge_Asteroid_Field/Forge/Materials/Asteroid_Ring/MI_Dust_Cloud.MI_Dust_Cloud" "None" :!class /Script/Engine.PrimitiveComponent))
  (Variables|Default|SetDMI_SelfShadowedCloud _returnvalue)
  (Rendering|Material|SetScalarParameterValue (Variables|Default|GetDMI_SelfShadowedCloud) "Depth_Distance" (Variables|Default|GetDepth_Distance) :!class /Script/Engine.MaterialInstanceDynamic)
  (Rendering|Material|SetScalarParameterValue (Variables|Default|GetDMI_SelfShadowedCloud) "Density" (Variables|Default|GetDensity) :!class /Script/Engine.MaterialInstanceDynamic)
  (Rendering|Material|SetScalarParameterValue (Variables|Default|GetDMI_SelfShadowedCloud) "Depth_Multiplier" (Variables|Default|GetDepth_Multiplier) :!class /Script/Engine.MaterialInstanceDynamic)
  (Rendering|Material|SetVectorParameterValue (Variables|Default|GetDMI_SelfShadowedCloud) "Color_Lit" (Variables|Default|GetColor_Lit) :!class /Script/Engine.MaterialInstanceDynamic)
  (Rendering|Material|SetVectorParameterValue (Variables|Default|GetDMI_SelfShadowedCloud) "Color_Depth" (Variables|Default|GetColor_Depth) :!class /Script/Engine.MaterialInstanceDynamic)
  (Rendering|Material|SetVectorParameterValue (Variables|Default|GetDMI_SelfShadowedCloud) "Directional_Light" (Math|Conversions|ToLinearColor(Vector) (* (Math|Rotator|GetRotationXVector (Transformation|GetActorRotation (Variables|Default|GetDirectional_Light))) "-1.000000,-1.000000,-1.000000")) :!class /Script/Engine.MaterialInstanceDynamic))