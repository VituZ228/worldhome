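; Procedural asteroid ring actor that scatters four instanced rock meshes around a circle, alongside a VDB dust volume.
; The construction script loops length by width, using CalculateAsteroidTransformation for seeded position and rotation jitter, then adds unseeded random scale and per-mesh ring multipliers.
; It also sets culling, dust material and scale, and a looping EditorTick timer that spins the dust.
; Optional Tick rotates the actor and updates every instance's spin and drift, at high performance cost.
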(event EventBeginPlay)

(event Collision|EventActorBeginOverlap
  (params (OtherActor :type Actor%20Object%20Reference)))

(event EventTick
  (params (DeltaSeconds :type Float%20%28single-precision%29))
  (bind _instancedstaticmesh_02 (Variables|Default|GetInstancedStaticMesh_02))
  (bind _instancedstaticmesh_00 (Variables|Default|GetInstancedStaticMesh_00))
  (bind _instancedstaticmesh_03 (Variables|Default|GetInstancedStaticMesh_03))
  (bind _instancedstaticmesh_01 (Variables|Default|GetInstancedStaticMesh_01))
  (if (Variables|Animation-System|GetPERFORMANCE_COST_Enable_Rotation?)
    (Transformation|AddActorLocalRotation (Math|Vector|RotatorfromAxisandAngle "0.000000,0.000000,1.000000" (* DeltaSeconds (Variables|Animation-System|GetRotationSpeed))) false false)
    (Utilities|FlowControl|Sequence
      (:then_0
        ;[0.5422 0 1] Asteroid Self spin - Very high cost in performance
        ;;[1 0 0] Figure out Index...
        (for _index (range 0 (Components|InstancedStaticMesh|GetInstanceCount _instancedstaticmesh_00)) ; Can use say "500" If you want some not to move
          (Components|InstancedStaticMesh|UpdateInstanceTransform _instancedstaticmesh_00 _index (Math|Transform|MakeTransform (+ (.location (.OutInstanceTransform (Components|InstancedStaticMesh|GetInstanceTransform _instancedstaticmesh_00 _index false))) (Variables|Animation-System|Get"Move%20In%20Direction")) (Math|Rotator|MakeRotator (+ (.Roll (Math|Rotator|BreakRotator (.rotation (.OutInstanceTransform (Components|InstancedStaticMesh|GetInstanceTransform _instancedstaticmesh_00 _index false))))) (Variables|Animation-RotateAstreroid01|GetRot%20X%20%28Roll%29_01)) (+ (.Pitch (Math|Rotator|BreakRotator (.rotation (.OutInstanceTransform (Components|InstancedStaticMesh|GetInstanceTransform _instancedstaticmesh_00 _index false))))) (Variables|Animation-RotateAstreroid01|GetRot%20Y%20%28Pitch%29_01)) (+ (.Yaw (Math|Rotator|BreakRotator (.rotation (.OutInstanceTransform (Components|InstancedStaticMesh|GetInstanceTransform _instancedstaticmesh_00 _index false))))) (Variables|Animation-RotateAstreroid01|GetRot%20Z%20%28Yaw%29_01))) (.scale (.OutInstanceTransform (Components|InstancedStaticMesh|GetInstanceTransform _instancedstaticmesh_00 _index false)))) false true false)))
      (:then_1
        ;[0.5422 0 1] Asteroid Self spin - Very high cost in performance
        ;;[1 0 0] Figure out Index...
        (for _index_2 (range 0 (Components|InstancedStaticMesh|GetInstanceCount _instancedstaticmesh_01)) ; Can use say "500" If you want some not to move
          (Components|InstancedStaticMesh|UpdateInstanceTransform _instancedstaticmesh_01 _index_2 (Math|Transform|MakeTransform (+ (.location (.OutInstanceTransform (Components|InstancedStaticMesh|GetInstanceTransform _instancedstaticmesh_01 _index_2 false))) (Variables|Animation-System|Get"Move%20In%20Direction")) (Math|Rotator|MakeRotator (+ (.Roll (Math|Rotator|BreakRotator (.rotation (.OutInstanceTransform (Components|InstancedStaticMesh|GetInstanceTransform _instancedstaticmesh_01 _index_2 false))))) (Variables|Animation-RotateAstreroid02|GetRot%20X%20%28Roll%29_02)) (+ (.Pitch (Math|Rotator|BreakRotator (.rotation (.OutInstanceTransform (Components|InstancedStaticMesh|GetInstanceTransform _instancedstaticmesh_01 _index_2 false))))) (Variables|Animation-RotateAstreroid03|GetRot%20Y%20%28Pitch%29_03)) (+ (.Yaw (Math|Rotator|BreakRotator (.rotation (.OutInstanceTransform (Components|InstancedStaticMesh|GetInstanceTransform _instancedstaticmesh_01 _index_2 false))))) (Variables|Animation-RotateAstreroid02|GetRot%20Z%20%28Yaw%29_02))) (.scale (.OutInstanceTransform (Components|InstancedStaticMesh|GetInstanceTransform _instancedstaticmesh_01 _index_2 false)))) false true false)))
      (:then_2
        ;[0.5422 0 1] Asteroid Self spin - Very high cost in performance
        ;;[1 0 0] Figure out Index...
        (for _index_3 (range 0 (Components|InstancedStaticMesh|GetInstanceCount _instancedstaticmesh_02)) ; Can use say "500" If you want some not to move
          (Components|InstancedStaticMesh|UpdateInstanceTransform _instancedstaticmesh_02 _index_3 (Math|Transform|MakeTransform (+ (.location (.OutInstanceTransform (Components|InstancedStaticMesh|GetInstanceTransform _instancedstaticmesh_02 _index_3 false))) (Variables|Animation-System|Get"Move%20In%20Direction")) (Math|Rotator|MakeRotator (+ (.Roll (Math|Rotator|BreakRotator (.rotation (.OutInstanceTransform (Components|InstancedStaticMesh|GetInstanceTransform _instancedstaticmesh_02 _index_3 false))))) (Variables|Animation-RotateAstreroid03|GetRot%20X%20%28Roll%29_03)) (+ (.Pitch (Math|Rotator|BreakRotator (.rotation (.OutInstanceTransform (Components|InstancedStaticMesh|GetInstanceTransform _instancedstaticmesh_02 _index_3 false))))) (Variables|Animation-RotateAstreroid03|GetRot%20Y%20%28Pitch%29_03)) (+ (.Yaw (Math|Rotator|BreakRotator (.rotation (.OutInstanceTransform (Components|InstancedStaticMesh|GetInstanceTransform _instancedstaticmesh_02 _index_3 false))))) (Variables|Animation-RotateAstreroid03|GetRot%20Z%20%28Yaw%29_03))) (.scale (.OutInstanceTransform (Components|InstancedStaticMesh|GetInstanceTransform _instancedstaticmesh_02 _index_3 false)))) false true false)))
      (:then_3
        ;[0.5422 0 1] Asteroid Self spin - Very high cost in performance
        ;;[1 0 0] Figure out Index...
        (for _index_4 (range 0 (Components|InstancedStaticMesh|GetInstanceCount _instancedstaticmesh_03)) ; Can use say "500" If you want some not to move
          (Components|InstancedStaticMesh|UpdateInstanceTransform _instancedstaticmesh_03 _index_4 (Math|Transform|MakeTransform (+ (.location (.OutInstanceTransform (Components|InstancedStaticMesh|GetInstanceTransform _instancedstaticmesh_03 _index_4 false))) (Variables|Animation-System|Get"Move%20In%20Direction")) (Math|Rotator|MakeRotator (+ (.Roll (Math|Rotator|BreakRotator (.rotation (.OutInstanceTransform (Components|InstancedStaticMesh|GetInstanceTransform _instancedstaticmesh_03 _index_4 false))))) (Variables|Animation-RotateAstreroid04|GetRot%20X%20%28Roll%29_04)) (+ (.Pitch (Math|Rotator|BreakRotator (.rotation (.OutInstanceTransform (Components|InstancedStaticMesh|GetInstanceTransform _instancedstaticmesh_03 _index_4 false))))) (Variables|Animation-RotateAstreroid04|GetRot%20Y%20%28Pitch%29_04)) (+ (.Yaw (Math|Rotator|BreakRotator (.rotation (.OutInstanceTransform (Components|InstancedStaticMesh|GetInstanceTransform _instancedstaticmesh_03 _index_4 false))))) (Variables|Animation-RotateAstreroid04|GetRot%20Z%20%28Yaw%29_04))) (.scale (.OutInstanceTransform (Components|InstancedStaticMesh|GetInstanceTransform _instancedstaticmesh_03 _index_4 false)))) false true false))))))

(event EventEndPlay
  (params (EndPlayReason :type EEndPlayReason%20Enum :default "Destroyed"))
  (Components|InstancedStaticMesh|ClearInstances (Variables|Default|GetHierarchicalInstancedStaticMesh)))

(event EventEditorTick
  (Transformation|AddLocalRotation (Variables|Default|GetHeterogeneousVolume) (Math|Rotator|MakeRotator 0.0 0.0 (Variables|(VDB)DustRingSettings|GetVDB_Rotation%20%28In-Editor%20Only%29)) false false))

(fn ConstructionScript
  (bind _heterogeneousvolume (Variables|Default|GetHeterogeneousVolume))
  (bind _randomscalemax (Variables|Transform|GetRandomScaleMAX))
  (bind _instancecountbylength (Variables|Instances|GetInstanceCountByLength))
  (bind _instancecountbywidth (Variables|Instances|GetInstanceCountByWidth))
  (bind _randomscaleminimum (Variables|Transform|GetRandomScaleMinimum))
  (bind _instance_location (Variables|Transform|GetInstance_Location))
  (bind _returnvalue (Math|Random|RandomFloatinRange _randomscaleminimum _randomscalemax))
  (bind _returnvalue_2 (Math|Vector|MakeVector _returnvalue _returnvalue _returnvalue))
  (Transformation|SetRelativeLocation (Variables|Default|GetInstancedStaticMesh_00) (* (Math|Random|RandomUnitVectorfromStream _instance_location) (Math|Random|RandomFloatinRangefromStream _instance_location 0.0 1e+05)) false false)
  (Utilities|FlowControl|Sequence
    (:then_0
      ;[1 1 1] Declaring Instances - Continue adding if you want more asteroid types per ring
      (Components|StaticMesh|SetStaticMesh (Variables|Default|GetInstancedStaticMesh_00) (Utilities|Array|Get(acopy) (Variables|Instances|GetInstanceMesh) (Math|Random|RandomIntegerinRange 0 0))) ; Set the mesh to be cloned
      (Components|StaticMesh|SetStaticMesh (Variables|Default|GetInstancedStaticMesh_01) (Utilities|Array|Get(acopy) (Variables|Instances|GetInstanceMesh) (Math|Random|RandomIntegerinRange 1 1))) ; Set the mesh to be cloned
      (Components|StaticMesh|SetStaticMesh (Variables|Default|GetInstancedStaticMesh_02) (Utilities|Array|Get(acopy) (Variables|Instances|GetInstanceMesh) (Math|Random|RandomIntegerinRange 2 2))) ; Set the mesh to be cloned
      (Components|StaticMesh|SetStaticMesh (Variables|Default|GetInstancedStaticMesh_03) (Utilities|Array|Get(acopy) (Variables|Instances|GetInstanceMesh) (Math|Random|RandomIntegerinRange 3 3))) ; Set the mesh to be cloned
    )
    (:then_1
      ;[1 1 1] Culling distance per Instance
      (Components|InstancedStaticMesh|SetCullDistances (Variables|Default|GetInstancedStaticMesh_00) (Variables|Performance|GetCullingNear) (Variables|Performance|GetCulling%20Far)) ; Visibility distances
    )
    (:then_2
      (for _index (range 0 (- _instancecountbylength 1))
        (for _index_2 (range 0 (- _instancecountbywidth 1))
          (bind (_outlocation _outrotator) (CallFunction|CalculateAsteroidTransformation _index_2 _instancecountbywidth _index _instancecountbylength))
          ;[1 1 1] Continue adding more instances if you want more Asteroid Types to be loaded
          (Components|InstancedStaticMesh|AddInstances (Variables|Default|GetInstancedStaticMesh_00) (Utilities|Array|MakeArray (Math|Transform|MakeTransform (* (Variables|Ring_Refinement|GetRing%201%20-%20Loc) (.Location (Math|Transform|BreakTransform (Math|Transform|MakeTransform (Math|Vector|MakeVector (* (.x _outlocation) (Variables|Transform|GetRing_Shape_X)) (* (.y _outlocation) (Variables|Transform|GetRing_Shape_Y)) (* (.z _outlocation) (Variables|Transform|GetRing_Shape_Z))) _outrotator (Math|Vector|MakeVector (+ (.x _returnvalue_2) (Variables|Animation-System|GetScale%20X)) (+ (.y _returnvalue_2) (Variables|Animation-System|GetScale%20Y)) (+ (.z _returnvalue_2) (Variables|Animation-System|GetScale%20Z))))))) (* (.Rotation (Math|Transform|BreakTransform (Math|Transform|MakeTransform (Math|Vector|MakeVector (* (.x _outlocation) (Variables|Transform|GetRing_Shape_X)) (* (.y _outlocation) (Variables|Transform|GetRing_Shape_Y)) (* (.z _outlocation) (Variables|Transform|GetRing_Shape_Z))) _outrotator (Math|Vector|MakeVector (+ (.x _returnvalue_2) (Variables|Animation-System|GetScale%20X)) (+ (.y _returnvalue_2) (Variables|Animation-System|GetScale%20Y)) (+ (.z _returnvalue_2) (Variables|Animation-System|GetScale%20Z)))))) (Variables|Ring_Refinement|GetRing%201%20-%20Rot)) (.Scale (Math|Transform|BreakTransform (Math|Transform|MakeTransform (Math|Vector|MakeVector (* (.x _outlocation) (Variables|Transform|GetRing_Shape_X)) (* (.y _outlocation) (Variables|Transform|GetRing_Shape_Y)) (* (.z _outlocation) (Variables|Transform|GetRing_Shape_Z))) _outrotator (Math|Vector|MakeVector (+ (.x _returnvalue_2) (Variables|Animation-System|GetScale%20X)) (+ (.y _returnvalue_2) (Variables|Animation-System|GetScale%20Y)) (+ (.z _returnvalue_2) (Variables|Animation-System|GetScale%20Z)))))))) false false)
          (Components|InstancedStaticMesh|AddInstances (Variables|Default|GetInstancedStaticMesh_01) (Utilities|Array|MakeArray (Math|Transform|MakeTransform (* (Variables|Ring_Refinement|GetRing%202%20-%20Loc) (.Location (Math|Transform|BreakTransform (Math|Transform|MakeTransform (Math|Vector|MakeVector (* (.x _outlocation) (Variables|Transform|GetRing_Shape_X)) (* (.y _outlocation) (Variables|Transform|GetRing_Shape_Y)) (* (.z _outlocation) (Variables|Transform|GetRing_Shape_Z))) _outrotator (Math|Vector|MakeVector (+ (.x _returnvalue_2) (Variables|Animation-System|GetScale%20X)) (+ (.y _returnvalue_2) (Variables|Animation-System|GetScale%20Y)) (+ (.z _returnvalue_2) (Variables|Animation-System|GetScale%20Z))))))) (* (.Rotation (Math|Transform|BreakTransform (Math|Transform|MakeTransform (Math|Vector|MakeVector (* (.x _outlocation) (Variables|Transform|GetRing_Shape_X)) (* (.y _outlocation) (Variables|Transform|GetRing_Shape_Y)) (* (.z _outlocation) (Variables|Transform|GetRing_Shape_Z))) _outrotator (Math|Vector|MakeVector (+ (.x _returnvalue_2) (Variables|Animation-System|GetScale%20X)) (+ (.y _returnvalue_2) (Variables|Animation-System|GetScale%20Y)) (+ (.z _returnvalue_2) (Variables|Animation-System|GetScale%20Z)))))) (Variables|Ring_Refinement|GetRing%202%20-%20Rot)) (.Scale (Math|Transform|BreakTransform (Math|Transform|MakeTransform (Math|Vector|MakeVector (* (.x _outlocation) (Variables|Transform|GetRing_Shape_X)) (* (.y _outlocation) (Variables|Transform|GetRing_Shape_Y)) (* (.z _outlocation) (Variables|Transform|GetRing_Shape_Z))) _outrotator (Math|Vector|MakeVector (+ (.x _returnvalue_2) (Variables|Animation-System|GetScale%20X)) (+ (.y _returnvalue_2) (Variables|Animation-System|GetScale%20Y)) (+ (.z _returnvalue_2) (Variables|Animation-System|GetScale%20Z)))))))) false false)
          (Components|InstancedStaticMesh|AddInstances (Variables|Default|GetInstancedStaticMesh_02) (Utilities|Array|MakeArray (Math|Transform|MakeTransform (* (Variables|Ring_Refinement|GetRing%203%20-%20Loc) (.Location (Math|Transform|BreakTransform (Math|Transform|MakeTransform (Math|Vector|MakeVector (* (.x _outlocation) (Variables|Transform|GetRing_Shape_X)) (* (.y _outlocation) (Variables|Transform|GetRing_Shape_Y)) (* (.z _outlocation) (Variables|Transform|GetRing_Shape_Z))) _outrotator (Math|Vector|MakeVector (+ (.x _returnvalue_2) (Variables|Animation-System|GetScale%20X)) (+ (.y _returnvalue_2) (Variables|Animation-System|GetScale%20Y)) (+ (.z _returnvalue_2) (Variables|Animation-System|GetScale%20Z))))))) (* (.Rotation (Math|Transform|BreakTransform (Math|Transform|MakeTransform (Math|Vector|MakeVector (* (.x _outlocation) (Variables|Transform|GetRing_Shape_X)) (* (.y _outlocation) (Variables|Transform|GetRing_Shape_Y)) (* (.z _outlocation) (Variables|Transform|GetRing_Shape_Z))) _outrotator (Math|Vector|MakeVector (+ (.x _returnvalue_2) (Variables|Animation-System|GetScale%20X)) (+ (.y _returnvalue_2) (Variables|Animation-System|GetScale%20Y)) (+ (.z _returnvalue_2) (Variables|Animation-System|GetScale%20Z)))))) (Variables|Ring_Refinement|GetRing%203%20-%20Rot)) (.Scale (Math|Transform|BreakTransform (Math|Transform|MakeTransform (Math|Vector|MakeVector (* (.x _outlocation) (Variables|Transform|GetRing_Shape_X)) (* (.y _outlocation) (Variables|Transform|GetRing_Shape_Y)) (* (.z _outlocation) (Variables|Transform|GetRing_Shape_Z))) _outrotator (Math|Vector|MakeVector (+ (.x _returnvalue_2) (Variables|Animation-System|GetScale%20X)) (+ (.y _returnvalue_2) (Variables|Animation-System|GetScale%20Y)) (+ (.z _returnvalue_2) (Variables|Animation-System|GetScale%20Z)))))))) false false)
          (Components|InstancedStaticMesh|AddInstances (Variables|Default|GetInstancedStaticMesh_03) (Utilities|Array|MakeArray (Math|Transform|MakeTransform (* (Variables|Ring_Refinement|GetRing%204%20-%20Loc) (.Location (Math|Transform|BreakTransform (Math|Transform|MakeTransform (Math|Vector|MakeVector (* (.x _outlocation) (Variables|Transform|GetRing_Shape_X)) (* (.y _outlocation) (Variables|Transform|GetRing_Shape_Y)) (* (.z _outlocation) (Variables|Transform|GetRing_Shape_Z))) _outrotator (Math|Vector|MakeVector (+ (.x _returnvalue_2) (Variables|Animation-System|GetScale%20X)) (+ (.y _returnvalue_2) (Variables|Animation-System|GetScale%20Y)) (+ (.z _returnvalue_2) (Variables|Animation-System|GetScale%20Z))))))) (* (.Rotation (Math|Transform|BreakTransform (Math|Transform|MakeTransform (Math|Vector|MakeVector (* (.x _outlocation) (Variables|Transform|GetRing_Shape_X)) (* (.y _outlocation) (Variables|Transform|GetRing_Shape_Y)) (* (.z _outlocation) (Variables|Transform|GetRing_Shape_Z))) _outrotator (Math|Vector|MakeVector (+ (.x _returnvalue_2) (Variables|Animation-System|GetScale%20X)) (+ (.y _returnvalue_2) (Variables|Animation-System|GetScale%20Y)) (+ (.z _returnvalue_2) (Variables|Animation-System|GetScale%20Z)))))) (Variables|Ring_Refinement|GetRing%204%20-%20Rot)) (.Scale (Math|Transform|BreakTransform (Math|Transform|MakeTransform (Math|Vector|MakeVector (* (.x _outlocation) (Variables|Transform|GetRing_Shape_X)) (* (.y _outlocation) (Variables|Transform|GetRing_Shape_Y)) (* (.z _outlocation) (Variables|Transform|GetRing_Shape_Z))) _outrotator (Math|Vector|MakeVector (+ (.x _returnvalue_2) (Variables|Animation-System|GetScale%20X)) (+ (.y _returnvalue_2) (Variables|Animation-System|GetScale%20Y)) (+ (.z _returnvalue_2) (Variables|Animation-System|GetScale%20Z)))))))) false false))))
    (:then_3
      ;[1 1 1] VDB Control
      (Rendering|Material|CreateDynamicMaterialInstance _heterogeneousvolume 0 "/Game/Cosmic_Forge_Asteroid_Field/Forge/Materials/Asteroid_Ring/MI_VDB_Dust.MI_VDB_Dust" "None" :!class /Script/Engine.PrimitiveComponent)
      (Rendering|Material|SetScalarParameterValueonMaterials _heterogeneousvolume "Temperature_Multiplier" (Variables|(VDB)DustRingSettings|GetVDB_Temp_Multiplier))
      (Utilities|Time|SetTimerbyFunctionName 0 "EditorTick" 0.01 true)
      (Transformation|SetRelativeScale3D (Variables|Default|GetHeterogeneousVolume) (Variables|(VDB)DustRingSettings|GetVDB_Dust_Ring_Scale)))))

(fn CalculateAsteroidTransformation
  (params (IndexFromWidthLoop :type Integer) (NumberOfInstancesByWidth :type Integer) (IndexFromLengthLoop :type Integer) (NumberOfInstancesByLength :type Integer))
  (bind _returnvalue (Math|Conversions|ToFloat(Integer) 0))
  (bind _returnvalue_2 (Math|Float|MakeLiteralFloat 3.6e+02))
  (bind _returnvalue_3 (Math|Conversions|ToFloat(Integer) IndexFromLengthLoop))
  (bind _returnvalue_4 (Math|Conversions|ToFloat(Integer) NumberOfInstancesByLength))
  (bind _returnvalue_5 (Math|Vector|MakeVector 0.0 0.0 1.0))
  (bind _returnvalue_6 (Math|Conversions|ToFloat(Integer) IndexFromWidthLoop))
  (bind _returnvalue_7 (Math|Conversions|ToFloat(Integer) NumberOfInstancesByWidth))
  (bind _ringradius (Variables|Instances|GetRingRadius))
  (bind _ringwidth (Variables|Instances|GetRingWidth))
  (bind _ringwidth_2 (Variables|Instances|GetRingWidth))
  (bind _transformrandom (Variables|Transform|GetTransformRandom))
  (bind _randomizeposition (Variables|Transform|GetRandomizePosition))
  (bind _randomizeupaxisposition (Variables|Transform|GetRandomizeUpAxisPosition))
  (bind _returnvalue_8 (/ _returnvalue_3 _returnvalue_4))
  (bind _returnvalue_9 (/ _returnvalue_6 _returnvalue_7))
  (bind _returnvalue_10 (Math|Random|RandomUnitVectorfromStream _transformrandom))
  (bind _returnvalue_11 (Math|Random|RandomFloatfromStream _transformrandom))
  (bind _returnvalue_12 (- _returnvalue_9 0.5))
  (bind _returnvalue_13 (* _returnvalue_10 _randomizeposition))
  (bind _returnvalue_14 (- _returnvalue _returnvalue_11))
  (bind _returnvalue_15 (* _returnvalue_8 _returnvalue_2))
  (bind _returnvalue_16 (* _returnvalue_12 _ringwidth_2))
  (bind _returnvalue_17 (* _returnvalue_14 _randomizeupaxisposition _ringwidth))
  (bind _returnvalue_18 (Math|Vector|MakeVector 0.0 0.0 _returnvalue_17))
  (bind _returnvalue_19 (+ _ringradius _returnvalue_16))
  (bind _returnvalue_20 (Math|Vector|MakeVector 0.0 _returnvalue_19 0.0))
  (bind _returnvalue_21 (+ _returnvalue_18 _returnvalue_13))
  (bind _returnvalue_22 (+ _returnvalue_21 _returnvalue_20))
  (bind _returnvalue_23 (Math|Vector|RotateVectorAroundAxis _returnvalue_22 _returnvalue_15 _returnvalue_5))
  (return _returnvalue_23 (Math|Rotator|Lerp(Rotator) (Class|KismetMathLibrary|MakeRotfromYZ (Math|Vector|CrossProduct _returnvalue_5 _returnvalue_23) _returnvalue_5) (Class|KismetMathLibrary|RandomRotatorfromStream (Variables|Transform|GetTransformRandom) true) (Variables|Transform|GetRandomizeRotation) true)))

(fn NewFunction0
  (params ([0] :type Transform))
  (return (Utilities|Array|MakeArray [0])))