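; Nebula generator actor that renders a volumetric cloud from a sparse volume (VDB) texture through a dynamic instance of MI_Nebula.
; Its variables drive the material's density, scattering, color, remap, temperature, erosion and noise parameters.
; The same setup runs in the construction script on CloudLoaderView and at BeginPlay on CloudLoader.
; Both passes also set global Heterogeneous Volumes cvars for indirect lighting and trace distance via console commands, affecting all such volumes.
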(event EventBeginPlay
  (bind _cloud_loader (Variables|Default|GetCloud_Loader))
  ;[1 1 1] Cloud_Quality
  (Utilities|FlowControl|Sequence
    (:then_0
      (if (Variables|Default|GetIndirect_Lighting?)
        (Development|ExecuteConsoleCommand "r.HeterogeneousVolumes.IndirectLighting 1" 0)
        (else
          (Development|ExecuteConsoleCommand "r.HeterogeneousVolumes.IndirectLighting 0" 0))))
    (:then_1
      (if (Variables|Default|GetInfinite_Trace?)
        (Development|ExecuteConsoleCommand "r.HeterogeneousVolumes.MaxTraceDistance 100000000" 0)
        (else
          (Development|ExecuteConsoleCommand "r.HeterogeneousVolumes.MaxTraceDistance 1" 0))))
    (:then_2
      ;[1 1 1] Cloud_Material_Setup
      (bind _returnvalue (Rendering|Material|CreateDynamicMaterialInstance _cloud_loader 0 "/Game/Cosmic_Forge_Asteroid_Field/Forge/Materials/Asteroid_Ring/MI_Nebula.MI_Nebula" "" :!class /Script/Engine.PrimitiveComponent))
      (Rendering|Material|SetScalarParameterValueonMaterials _cloud_loader "Density_Multiplier" (Variables|Default|GetDensity_Multiplier))
      (Rendering|Material|SetVectorParameterValueonMaterials _cloud_loader "Scattering_Color" (Math|Conversions|ToVector(LinearColor) (Variables|Color_Control|GetScattering_Color)))
      (Class|MaterialInstanceDynamic|SetSparseVolumeTextureParameterValue _returnvalue "VDB_Texture" (Variables|Default|GetVDB_Texture))
      (Rendering|Material|SetScalarParameterValueonMaterials _cloud_loader "Remap_InputHigh" (Variables|Default|GetRemap_InputHigh))
      (Rendering|Material|SetScalarParameterValueonMaterials _cloud_loader "Remap_InputLow" (Variables|Default|GetRemap_InputLow))
      (Rendering|Material|SetScalarParameterValueonMaterials _cloud_loader "Remap_TargetHigh" (Variables|Default|GetRemap_TargetHigh))
      (Rendering|Material|SetScalarParameterValueonMaterials _cloud_loader "Remap_TargetLow" (Variables|Default|GetRemap_TargetLow))
      (Rendering|Material|SetScalarParameterValueonMaterials _cloud_loader "Main_Color_Blend" (Variables|Color_Control|GetMain_Color_Blend))
      (Rendering|Material|SetScalarParameterValueonMaterials _cloud_loader "Desaturation" (Variables|Color_Control|GetDesaturation))
      (Rendering|Material|SetVectorParameterValueonMaterials _cloud_loader "Sub Scattering Control" (Math|Conversions|ToVector(LinearColor) (Variables|Color_Control|GetSub%20Scattering%20Control)))
      (Rendering|Material|SetVectorParameterValueonMaterials _cloud_loader "Main_Color_Blend_Direction" (Math|Conversions|ToVector(LinearColor) (Variables|Color_Control|GetMain_Color_Blend_Direction)))
      (Rendering|Material|SetScalarParameterValueonMaterials _cloud_loader "I_H_Color" (Variables|Color_Control|GetInput_High_Color))
      (Rendering|Material|SetScalarParameterValueonMaterials _cloud_loader "I_L_Color" (Variables|Color_Control|GetInput_Low_Color))
      (Rendering|Material|SetScalarParameterValueonMaterials _cloud_loader "T_H_Color" (Variables|Color_Control|GetTarget_High_Color))
      (Rendering|Material|SetScalarParameterValueonMaterials _cloud_loader "T_L_Color" (Variables|Color_Control|GetTarget_Low_Color))
      (Rendering|Material|SetScalarParameterValueonMaterials _cloud_loader "Blackbody_Parameter" (Variables|Default|GetBlackbody_Parameter))
      (Rendering|Material|SetScalarParameterValueonMaterials _cloud_loader "Temperature_Multiplier" (Variables|Default|GetTemperature_Multiplier))
      (Rendering|Material|SetScalarParameterValueonMaterials _cloud_loader "Nebula_Erosion_MAX" (Variables|Default|GetNebula_Erosion_MAX))
      (Rendering|Material|SetScalarParameterValueonMaterials _cloud_loader "Nebula_Erosion" (Variables|Default|GetNebula_Erosion))
      (Rendering|Material|SetScalarParameterValueonMaterials _cloud_loader "Small_Noise_Scale" (Variables|Default|GetSmall_Noise_Scale))
      (Rendering|Material|SetScalarParameterValueonMaterials _cloud_loader "Large_Noise_Scale" (Variables|Default|GetLarge_Noise_Scale))
      (Rendering|Material|SetVectorParameterValueonMaterials _cloud_loader "NoisePan" (Math|Conversions|ToVector(LinearColor) (Variables|Color_Control|GetNoisePan)))
      (Rendering|Material|SetVectorParameterValueonMaterials _cloud_loader "Temperature_Color" (Math|Conversions|ToVector(LinearColor) (Variables|Color_Control|GetTemperature_Color))))))

(event Collision|EventActorBeginOverlap
  (params (OtherActor :type Actor%20Object%20Reference)))

(event EventTick
  (params (DeltaSeconds :type Float%20%28single-precision%29)))

(fn ConstructionScript
  (bind _cloud_loader_view (Variables|Default|GetCloud_Loader_View))
  ;[1 1 1] Cloud_Quality
  (Utilities|FlowControl|Sequence
    (:then_0
      (if (Variables|Default|GetIndirect_Lighting?)
        (Development|ExecuteConsoleCommand "r.HeterogeneousVolumes.IndirectLighting 1" 0)
        (else
          (Development|ExecuteConsoleCommand "r.HeterogeneousVolumes.IndirectLighting 0" 0))))
    (:then_1
      (if (Variables|Default|GetInfinite_Trace?)
        (Development|ExecuteConsoleCommand "r.HeterogeneousVolumes.MaxTraceDistance 100000000" 0)
        (else
          (Development|ExecuteConsoleCommand "r.HeterogeneousVolumes.MaxTraceDistance 1" 0))))
    (:then_2
      ;[1 1 1] Cloud_Material_Setup
      (bind _returnvalue (Rendering|Material|CreateDynamicMaterialInstance _cloud_loader_view 0 "/Game/Cosmic_Forge_Asteroid_Field/Forge/Materials/Asteroid_Ring/MI_Nebula.MI_Nebula" "" :!class /Script/Engine.PrimitiveComponent))
      (Rendering|Material|SetScalarParameterValueonMaterials _cloud_loader_view "Density_Multiplier" (Variables|Default|GetDensity_Multiplier))
      (Rendering|Material|SetVectorParameterValueonMaterials _cloud_loader_view "Scattering_Color" (Math|Conversions|ToVector(LinearColor) (Variables|Color_Control|GetScattering_Color)))
      (Class|MaterialInstanceDynamic|SetSparseVolumeTextureParameterValue _returnvalue "VDB_Texture" (Variables|Default|GetVDB_Texture))
      (Rendering|Material|SetScalarParameterValueonMaterials _cloud_loader_view "Remap_InputHigh" (Variables|Default|GetRemap_InputHigh))
      (Rendering|Material|SetScalarParameterValueonMaterials _cloud_loader_view "Remap_InputLow" (Variables|Default|GetRemap_InputLow))
      (Rendering|Material|SetScalarParameterValueonMaterials _cloud_loader_view "Remap_TargetHigh" (Variables|Default|GetRemap_TargetHigh))
      (Rendering|Material|SetScalarParameterValueonMaterials _cloud_loader_view "Remap_TargetLow" (Variables|Default|GetRemap_TargetLow))
      (Rendering|Material|SetScalarParameterValueonMaterials _cloud_loader_view "Main_Color_Blend" (Variables|Color_Control|GetMain_Color_Blend))
      (Rendering|Material|SetScalarParameterValueonMaterials _cloud_loader_view "Desaturation" (Variables|Color_Control|GetDesaturation))
      (Rendering|Material|SetVectorParameterValueonMaterials _cloud_loader_view "Sub Scattering Control" (Math|Conversions|ToVector(LinearColor) (Variables|Color_Control|GetSub%20Scattering%20Control)))
      (Rendering|Material|SetVectorParameterValueonMaterials _cloud_loader_view "Main_Color_Blend_Direction" (Math|Conversions|ToVector(LinearColor) (Variables|Color_Control|GetMain_Color_Blend_Direction)))
      (Rendering|Material|SetScalarParameterValueonMaterials _cloud_loader_view "I_H_Color" (Variables|Color_Control|GetInput_High_Color))
      (Rendering|Material|SetScalarParameterValueonMaterials _cloud_loader_view "I_L_Color" (Variables|Color_Control|GetInput_Low_Color))
      (Rendering|Material|SetScalarParameterValueonMaterials _cloud_loader_view "T_H_Color" (Variables|Color_Control|GetTarget_High_Color))
      (Rendering|Material|SetScalarParameterValueonMaterials _cloud_loader_view "T_L_Color" (Variables|Color_Control|GetTarget_Low_Color))
      (Rendering|Material|SetScalarParameterValueonMaterials _cloud_loader_view "Blackbody_Parameter" (Variables|Default|GetBlackbody_Parameter))
      (Rendering|Material|SetScalarParameterValueonMaterials _cloud_loader_view "Temperature_Multiplier" (Variables|Default|GetTemperature_Multiplier))
      (Rendering|Material|SetScalarParameterValueonMaterials _cloud_loader_view "Nebula_Erosion_MAX" (Variables|Default|GetNebula_Erosion_MAX))
      (Rendering|Material|SetScalarParameterValueonMaterials _cloud_loader_view "Nebula_Erosion" (Variables|Default|GetNebula_Erosion))
      (Rendering|Material|SetScalarParameterValueonMaterials _cloud_loader_view "Small_Noise_Scale" (Variables|Default|GetSmall_Noise_Scale))
      (Rendering|Material|SetScalarParameterValueonMaterials _cloud_loader_view "Large_Noise_Scale" (Variables|Default|GetLarge_Noise_Scale))
      (Rendering|Material|SetVectorParameterValueonMaterials _cloud_loader_view "NoisePan" (Math|Conversions|ToVector(LinearColor) (Variables|Color_Control|GetNoisePan)))
      (Rendering|Material|SetVectorParameterValueonMaterials _cloud_loader_view "Temperature_Color" (Math|Conversions|ToVector(LinearColor) (Variables|Color_Control|GetTemperature_Color))))))