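; BP_DK2_Turret is a spaceship turret that rotates its mesh in yaw to track a Target actor, optionally the player pawn.
; Each tick it converts the direction to the target into actor-local space, applies a yaw offset and smoothly interpolates the mesh's relative rotation.
; When not recently rendered, it ticks less often and raises interpolation speed.
; It contains aiming only, with no firing logic.
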(event EventBeginPlay
  (if (Variables|Default|GetTarget%20is%20Player%20Pawn?)
    (Variables|Default|SetTarget (Game|Player|GetPlayerPawn 0)) ; Make turret aim at Camera
  ))

(event EventTick
  (params (DeltaSeconds :type Float%20%28single-precision%29))
  (bind _returnvalue (Class|Actor|WasRecentlyRendered 0.2))
  (bind _sm_dk2_turret (Variables|Default|GetSM_DK2_Turret))
  (bind _rotation_speed (Variables|Default|GetRotation%20Speed))
  (if _returnvalue
    (Actor|Tick|SetActorTickInterval 0.0)
    (else
      (Actor|Tick|SetActorTickInterval 0.25)))
  ;[1 1 1] Aim Turret
  (Transformation|SetRelativeRotation _sm_dk2_turret (Math|Interpolation|RInterpTo (Variables|/Script/Engine.SceneComponent|GetRelativeRotation _sm_dk2_turret) (Math|Rotator|MakeRotator 0.0 0.0 (- (.Yaw (Math|Rotator|BreakRotator (Math|Rotator|MakeRotfromX (Math|Transform|InverseTransformDirection (Transformation|GetActorTransform) (- (Transformation|GetActorLocation (Variables|Default|GetTarget)) (Transformation|GetWorldLocation (Variables|Default|GetSM_DK2_Turret))))))) 9e+01)) (Utilities|Time|GetWorldDeltaSeconds) (select _returnvalue _rotation_speed (* _rotation_speed 1e+01))) false false))

(fn ConstructionScript)