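; BP_DK3_Turret is a turret actor that smoothly turns to face a target actor, optionally the player pawn set at BeginPlay.
; Each Tick converts the target direction into actor-local space and interpolates the turret mesh's yaw toward it at RotationSpeed, with a 90-degree offset and no pitch.
; As an optimization, the actor ticks less often when it has not been rendered recently.
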(event EventBeginPlay
  (if (Variables|Default|GetTarget%20is%20Player%20Pawn?)
    (Variables|Default|SetTarget (Game|Player|GetPlayerPawn 0)) ; Make turret aim at Camera
  ))

(event EventTick
  (params (DeltaSeconds :type Float%20%28single-precision%29))
  (bind _sm_dk3_turret (Variables|Default|GetSM_DK3_Turret))
  (if (Class|Actor|WasRecentlyRendered 0.2)
    (Actor|Tick|SetActorTickInterval 0.0)
    (else
      (Actor|Tick|SetActorTickInterval 0.25)))
  ;[1 1 1] Aim Turret
  (Transformation|SetRelativeRotation _sm_dk3_turret (Math|Interpolation|RInterpTo (Variables|/Script/Engine.SceneComponent|GetRelativeRotation _sm_dk3_turret) (Math|Rotator|MakeRotator 0.0 0.0 (- (.Yaw (Math|Rotator|BreakRotator (Math|Rotator|MakeRotfromX (Math|Transform|InverseTransformDirection (Transformation|GetActorTransform) (- (Transformation|GetActorLocation (Variables|Default|GetTarget)) (Transformation|GetWorldLocation (Variables|Default|GetSM_DK3_Turret))))))) 9e+01)) (Utilities|Time|GetWorldDeltaSeconds) (Variables|Default|GetRotation%20Speed)) false false))

(fn ConstructionScript)