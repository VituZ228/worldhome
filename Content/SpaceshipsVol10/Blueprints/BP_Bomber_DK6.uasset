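; Bomber DK6 spaceship Blueprint with preset paint schemes and a controllable thruster effect.
; The construction script creates dynamic hull and flare materials, then applies Color's paint and matching thruster tint.
; Thrust drives hull glow, flare length and first-flare opacity.
; Optional demo modes play a thrust timeline after a Color-based delay and cycle schemes periodically, omitting the last preset.
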(event EventBeginPlay
  (if (Variables|Default|GetAnimateThrusters_Demo)
    (Utilities|FlowControl|Sequence
      (:then_0
        (Utilities|FlowControl|Delay (* (Variables|Default|GetColor) 0.4))
        (bind _thrust (Timeline|Timeline_0 Play)
          (:Update
            (Variables|Default|SetThrust _thrust)
            (CallFunction|AdjustThrusters))))
      (:then_1
        (if (Variables|Default|GetAnimate_Colors)
          (Utilities|FlowControl|Delay 3.0 :!label _label)
          (if (== (Variables|Default|GetColor) 5)
            (Variables|Default|SetColor 0)
            (else
              (Variables|Default|SetColor (+ (Variables|Default|GetColor) 1))))
          (CallFunction|SetColor)
          (CallFunction|SetThrusterColor)
          (goto _label))))))

(fn ConstructionScript
  (|CreateThrusterDynamicMaterials)
  (|CreateShipDynamicMaterial)
  (CallFunction|SetColor)
  (CallFunction|AdjustThrusters)
  (CallFunction|SetThrusterColor))

(fn AdjustThrusters
  (bind _thrust (Variables|Default|GetThrust))
  ;[1 1 1] Adjust Thruster Intensity
  (Rendering|Material|SetScalarParameterValue (Variables|Default|GetShipMaterial) "Thrust" (Math|Float|Lerp 0.0 1e+02 _thrust) :!class /Script/Engine.MaterialInstanceDynamic)
  (Transformation|SetRelativeScale3D (Variables|Default|GetThruster) (Math|Vector|MakeVector (Math|Float|Lerp 0.0 0.2 _thrust) 0.115 0.115))
  (Rendering|Material|SetScalarParameterValue (Variables|Default|GetDynMat_RocketFlare0) "Opacity" (Variables|Default|GetThrust) :!class /Script/Engine.MaterialInstanceDynamic))

(fn SetThrusterColor
  (Rendering|Material|SetVectorParameterValue (Variables|Default|GetDynMat_RocketFlare0) "Color" (Variables|Default|GetThruster_Color) :!class /Script/Engine.MaterialInstanceDynamic)
  (Rendering|Material|SetVectorParameterValue (Variables|Default|GetShipMaterial) "ThrusterColor" (Variables|Default|GetThruster_Color) :!class /Script/Engine.MaterialInstanceDynamic))

(fn SetColor
  (bind _shipmaterial (Variables|Default|GetShipMaterial))
  (bind _shipmaterial_2 (Variables|Default|GetShipMaterial))
  (bind _shipmaterial_3 (Variables|Default|GetShipMaterial))
  (bind _shipmaterial_4 (Variables|Default|GetShipMaterial))
  (bind _shipmaterial_5 (Variables|Default|GetShipMaterial))
  (bind _shipmaterial_6 (Variables|Default|GetShipMaterial))
  (bind _shipmaterial_7 (Variables|Default|GetShipMaterial))
  (switch int (Variables|Default|GetColor)
    (:0
      (Rendering|Material|SetVectorParameterValue _shipmaterial_3 "Dif_Texture_Mult" "(R=1.000000,G=1.000000,B=1.000000,A=1.000000)" :!class /Script/Engine.MaterialInstanceDynamic)
      (Rendering|Material|SetScalarParameterValue _shipmaterial_3 "Dif_Color_Brightness" 1.0 :!class /Script/Engine.MaterialInstanceDynamic)
      (Rendering|Material|SetScalarParameterValue _shipmaterial_3 "Dif_NonColor_Brightness" 1.0 :!class /Script/Engine.MaterialInstanceDynamic)
      (Rendering|Material|SetScalarParameterValue _shipmaterial_3 "Metal_Text_Value_A" 0.3 :!class /Script/Engine.MaterialInstanceDynamic)
      (Variables|Default|SetThruster_Color "(R=1.000000,G=0.000000,B=0.027019,A=1.000000)"))
    (:1
      (Rendering|Material|SetVectorParameterValue _shipmaterial_4 "Dif_Texture_Mult" "(R=1.000000,G=1.000000,B=1.000000,A=1.000000)" :!class /Script/Engine.MaterialInstanceDynamic)
      (Rendering|Material|SetScalarParameterValue _shipmaterial_4 "Dif_Color_Brightness" 5.0 :!class /Script/Engine.MaterialInstanceDynamic)
      (Rendering|Material|SetScalarParameterValue _shipmaterial_4 "Metal_Text_Value_A" 0.3 :!class /Script/Engine.MaterialInstanceDynamic)
      (Variables|Default|SetThruster_Color "(R=0.000000,G=0.357831,B=1.000000,A=1.000000)"))
    (:2
      (Rendering|Material|SetVectorParameterValue _shipmaterial_5 "Dif_Texture_Mult" "(R=1.000000,G=0.952280,B=0.000000,A=1.000000)" :!class /Script/Engine.MaterialInstanceDynamic)
      (Rendering|Material|SetScalarParameterValue _shipmaterial_5 "Dif_Color_Brightness" 3.0 :!class /Script/Engine.MaterialInstanceDynamic)
      (Rendering|Material|SetScalarParameterValue _shipmaterial_5 "Metal_Text_Value_A" 0.2 :!class /Script/Engine.MaterialInstanceDynamic)
      (Rendering|Material|SetScalarParameterValue _shipmaterial_5 "Roughness_Detail_A" 0.9 :!class /Script/Engine.MaterialInstanceDynamic)
      (Rendering|Material|SetScalarParameterValue _shipmaterial_5 "Roughness_Detail_B" 1.5 :!class /Script/Engine.MaterialInstanceDynamic)
      (Variables|Default|SetThruster_Color "(R=0.000000,G=0.357831,B=1.000000,A=1.000000)"))
    (:3
      (Rendering|Material|SetVectorParameterValue _shipmaterial_6 "Dif_Texture_Mult" "(R=0.000000,G=1.000000,B=0.250000,A=1.000000)" :!class /Script/Engine.MaterialInstanceDynamic)
      (Rendering|Material|SetScalarParameterValue _shipmaterial_6 "Dif_Color_Brightness" 1.5 :!class /Script/Engine.MaterialInstanceDynamic)
      (Rendering|Material|SetScalarParameterValue _shipmaterial_6 "Metal_Text_Value_A" 0.2 :!class /Script/Engine.MaterialInstanceDynamic)
      (Variables|Default|SetThruster_Color "(R=0.221802,G=0.530000,B=0.182850,A=1.000000)"))
    (:4
      (Rendering|Material|SetVectorParameterValue _shipmaterial_7 "Dif_Texture_Mult" "(R=1.000000,G=0.000000,B=0.000000,A=1.000000)" :!class /Script/Engine.MaterialInstanceDynamic)
      (Rendering|Material|SetScalarParameterValue _shipmaterial_7 "Dif_Color_Brightness" 3.0 :!class /Script/Engine.MaterialInstanceDynamic)
      (Rendering|Material|SetScalarParameterValue _shipmaterial_7 "Metal_Text_Value_A" 0.2 :!class /Script/Engine.MaterialInstanceDynamic)
      (Rendering|Material|SetScalarParameterValue _shipmaterial_7 "Rough_Tex_Value_A" 0.25 :!class /Script/Engine.MaterialInstanceDynamic)
      (Variables|Default|SetThruster_Color "(R=1.000000,G=0.737096,B=0.000000,A=1.000000)"))
    (:5
      (Rendering|Material|SetVectorParameterValue _shipmaterial_2 "Dif_Texture_Mult" "(R=0.000000,G=0.286710,B=1.000000,A=1.000000)" :!class /Script/Engine.MaterialInstanceDynamic)
      (Rendering|Material|SetScalarParameterValue _shipmaterial_2 "Dif_Color_Brightness" 7.0 :!class /Script/Engine.MaterialInstanceDynamic)
      (Rendering|Material|SetScalarParameterValue _shipmaterial_2 "Metal_Text_Value_A" 0.5 :!class /Script/Engine.MaterialInstanceDynamic)
      (Rendering|Material|SetScalarParameterValue _shipmaterial_2 "Rough_Tex_Value_A" 0.5 :!class /Script/Engine.MaterialInstanceDynamic)
      (Rendering|Material|SetScalarParameterValue _shipmaterial_2 "Rough_Tex_Value_B" 0.0 :!class /Script/Engine.MaterialInstanceDynamic)
      (Variables|Default|SetThruster_Color "(R=0.000000,G=0.590307,B=1.000000,A=1.000000)"))
    (:6
      (Rendering|Material|SetVectorParameterValue _shipmaterial "Dif_Texture_Mult" "(R=0.712500,G=0.568936,B=0.192375,A=1.000000)" :!class /Script/Engine.MaterialInstanceDynamic)
      (Rendering|Material|SetScalarParameterValue _shipmaterial "Dif_Color_Brightness" 7.0 :!class /Script/Engine.MaterialInstanceDynamic)
      (Rendering|Material|SetScalarParameterValue _shipmaterial "Metal_Text_Value_A" 1.0 :!class /Script/Engine.MaterialInstanceDynamic)
      (Rendering|Material|SetScalarParameterValue _shipmaterial "Rough_Tex_Value_A" 0.5 :!class /Script/Engine.MaterialInstanceDynamic)
      (Rendering|Material|SetScalarParameterValue _shipmaterial "Rough_Tex_Value_B" 0.0 :!class /Script/Engine.MaterialInstanceDynamic)
      (Variables|Default|SetThruster_Color "(R=1.000000,G=0.964861,B=0.625000,A=1.000000)"))))