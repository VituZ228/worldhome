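; Destroyer RF3 spaceship actor with a selectable hull color and thruster visuals driven by a Thrust value.
; Construction creates dynamic flare and hull materials, picks the hull skin from Color and applies ThrusterColor, which only some skins override.
; Every Tick, Thrust scales thruster mesh length, flare opacity and hull glow.
; When Thrust drops to zero, Tick steps it down from the previous value so the exhaust fades out.
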(event EventBeginPlay)

(event EventTick
  (params (DeltaSeconds :type Float%20%28single-precision%29))
  (if (and (> (Variables|Default|GetThurst_PrevTick) 0.1) (== (Variables|Default|GetThrust) 0.0))
    (Variables|Default|SetThrust (- (Variables|Default|GetThurst_PrevTick) 0.1))
    (CallFunction|AdjustThrusters)
    (else
      (CallFunction|AdjustThrusters)))
  (Variables|Default|SetThurst_PrevTick (Variables|Default|GetThrust)))

(fn ConstructionScript
  (|CreateThrusterDynamicMaterials)
  (Math|Color|SelectColor)
  (|CreateShipDynamicMaterial)
  (CallFunction|AdjustThrusters)
  (|SetThrusterColor))

(fn AdjustThrusters
  (bind _thrust (Variables|Default|GetThrust))
  ;[1 1 1] Adjust Thruster Intensity
  (Rendering|Material|SetScalarParameterValue (Variables|Default|GetShipMaterial) "Thrust" (Math|Float|Lerp 0.0 1e+01 _thrust) :!class /Script/Engine.MaterialInstanceDynamic)
  (Transformation|SetRelativeScale3D (Variables|Default|GetSM_Frigate_MB3_Thruster_TL2) (Math|Vector|MakeVector (Math|Float|Lerp 0.0 6e+01 _thrust) 19.0 19.0))
  (Transformation|SetRelativeScale3D (Variables|Default|GetSM_Frigate_MB3_Thruster_M_L) (Math|Vector|MakeVector (Math|Float|Lerp 0.0 4e+01 _thrust) 13.0 13.0))
  (Rendering|Material|SetScalarParameterValue (Variables|Default|GetDynMat_RocketFlare0) "Opacity" (Variables|Default|GetThrust) :!class /Script/Engine.MaterialInstanceDynamic))