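; Universal scatter actor that shows one randomly picked asset of a selected type: Niagara system, decal, static mesh or skeletal mesh.
; The construction script switches on SelectType, assigns a random entry from that type's array to the matching component, and destroys the other three components.
; The pick is unseeded, so it can change whenever construction reruns; the event graph has no active logic.
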(event EventBeginPlay)

(event Collision|EventActorBeginOverlap
  (params (OtherActor :type Actor%20Object%20Reference)))

(event EventTick
  (params (DeltaSeconds :type Float%20%28single-precision%29)))

(fn ConstructionScript
  (bind _decal (Variables|Default|Getdecal))
  (bind _skeletalmesh (Variables|Default|GetskeletalMesh))
  (bind _niagarasystem (Variables|Default|GetniagaraSystem))
  (switch Utilities|FlowControl|Switch|SwitchonE_bluePlug (Variables|Default|Getselect%20type)
    (:NewEnumerator1
      (Class|NiagaraComponent|SetAsset _niagarasystem (.OutItem (Utilities|Array|Random (Variables|Default|Getniagara%20systems))) true)
      (Components|DestroyComponent _decal))
    (:NewEnumerator11
      (Rendering|Components|Decal|SetDecalMaterial _decal (.OutItem (Utilities|Array|Random (Variables|Default|Getdecals))))
      (Components|DestroyComponent _niagarasystem))
    (:NewEnumerator5
      (Components|StaticMesh|SetStaticMesh (Variables|Default|GetstaticMesh) (.OutItem (Utilities|Array|Random (Variables|Default|Getstatic%20meshes))))
      (Components|DestroyComponent _skeletalmesh))
    (:NewEnumerator3
      (Components|SkeletalMesh|SetSkeletalMeshAsset _skeletalmesh (.OutItem (Utilities|Array|Random (Variables|Default|Getskeletal%20meshes))))
      (Components|DestroyComponent _niagarasystem))))