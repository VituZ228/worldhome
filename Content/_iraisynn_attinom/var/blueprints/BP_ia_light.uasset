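; BP_ia_light is an actor that shows either a cube or a sphere in a random color, with no runtime logic.
; The construction script gives each mesh a dynamic material instance and sets its "color" parameter to an independently randomized RGB value.
; A random boolean then makes one mesh visible and hides the other, so the look is rerolled whenever construction runs.
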(event EventBeginPlay)

(event Collision|EventActorBeginOverlap
  (params (OtherActor :type Actor%20Object%20Reference)))

(event EventTick
  (params (DeltaSeconds :type Float%20%28single-precision%29)))

(fn ConstructionScript
  (bind _returnvalue (Math|Random|RandomFloatinRange 0.0 1.0))
  (bind _returnvalue_2 (Math|Random|RandomFloatinRange 0.0 1.0))
  (bind _returnvalue_3 (Math|Random|RandomFloatinRange 0.0 1.0))
  (bind _sphere (Variables|Default|GetSphere))
  (bind _cube (Variables|Default|GetCube))
  (bind _returnvalue_4 (Math|Color|MakeColor _returnvalue_2 _returnvalue_3 _returnvalue))
  (bind _returnvalue_5 (Rendering|Material|CreateDynamicMaterialInstance _cube 0 0 "None" :!class /Script/Engine.PrimitiveComponent))
  (Rendering|Material|SetVectorParameterValue _returnvalue_5 "color" _returnvalue_4 :!class /Script/Engine.MaterialInstanceDynamic)
  (bind _returnvalue_6 (Rendering|Material|CreateDynamicMaterialInstance _sphere 0 0 "None" :!class /Script/Engine.PrimitiveComponent))
  (Rendering|Material|SetVectorParameterValue _returnvalue_6 "color" _returnvalue_4 :!class /Script/Engine.MaterialInstanceDynamic)
  (if (Math|Random|RandomBool)
    (Rendering|SetVisibility _cube true false)
    (Rendering|SetVisibility _sphere false false)
    (else
      (Rendering|SetVisibility _cube false false)
      (Rendering|SetVisibility _sphere true false))))