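; Portal actor that teleports an overlapping BasedShip pawn to its linked ExitPortal's arrow transform with a cinematic camera transition.
; Overlap spawns temporary cameras at both portals, and Teleport disables player input and blends the view from entry camera to exit camera to player pawn.
; A Teleporting flag and disabled exit collision block re-triggering until a delayed cleanup.
; The construction script applies the configurable mesh, angle, Niagara effect and effect scale.
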(event OnComponentBeginOverlap(Box)
  (params (OverlappedComponent :type Primitive%20Component%20Object%20Reference) (OtherActor :type Actor%20Object%20Reference) (OtherComp :type Primitive%20Component%20Object%20Reference) (OtherBodyIndex :type Integer) (bFromSweep :type Boolean) (SweepResult :type Hit%20Result%20Structure%20%28by%20ref%29))
  (bind _aspawn (Utilities|Casting|CastToPawn OtherActor))
  (Variables|Default|SetAs%20Pawn _aspawn)
  (if (not (Variables|Default|GetTeleporting))
    ;[1 1 1] Create cameras for blending
    (bind _returnvalue (Game|SpawnActorfromClass "/Game/PortalPack/Blueprint/BP_CameraActor.BP_CameraActor_C" (Transformation|GetWorldTransform (Variables|Default|GetCamLoc)) "Undefined" "OverrideRootScale" 0 0))
    (Variables|Default|SetBlendCamera _returnvalue)
    (bind _returnvalue_2 (Game|SpawnActorfromClass "/Game/PortalPack/Blueprint/BP_CameraActor.BP_CameraActor_C" (Transformation|GetWorldTransform (Variables|BP_Portal_1_C|GetCamLoc (Variables|Default|GetExitPortal))) "Undefined" "OverrideRootScale" 0 0))
    (Variables|Default|SetBlendCamera2 _returnvalue_2)
    (CallFunction|Teleport)))

(event Custom|Teleport
  ;[1 1 1] Teleporting
  (Collision|SetCollisionEnabled (Variables|BP_Portal_1_C|GetBox (Variables|Default|GetExitPortal)) "NoCollision")
  (Variables|Default|SetTeleporting true)
  (Input|DisableInput (Game|GetPlayerController 0))
  (Utilities|Casting|CastToBasedShip (Variables|Default|GetAs%20Pawn))
  (Game|Player|SetViewTargetwithBlend (Game|GetPlayerController 0) (Variables|Default|GetBlendCamera) 1.0 "VTBlend_Linear" 0.0 true)
  (Utilities|FlowControl|Delay 3.0)
  (Transformation|SetActorTransform (stale OnComponentBeginOverlap(Box) _aspawn) (Transformation|GetWorldTransform (Variables|BP_Portal_1_C|GetArrow (Variables|Default|GetExitPortal))))
  (Game|Player|SetViewTargetwithBlend (Game|GetPlayerController 0) (Variables|Default|GetBlendCamera2) 1.0 "VTBlend_Linear" 0.0 true)
  (Utilities|FlowControl|Delay 3.0)
  (Game|Player|SetViewTargetwithBlend (Game|GetPlayerController 0) (Game|Player|GetPlayerPawn 0) 1.0 "VTBlend_Linear" 0.0 true)
  (Utilities|FlowControl|Delay 1e+01)
  (Variables|Default|SetTeleporting false)
  (Actor|DestroyActor (stale OnComponentBeginOverlap(Box) _returnvalue))
  (Actor|DestroyActor (stale OnComponentBeginOverlap(Box) _returnvalue_2))
  (Collision|SetCollisionEnabled (Variables|BP_Portal_1_C|GetBox (Variables|Default|GetExitPortal)) "QueryAndPhysics"))

(fn ConstructionScript
  (bind _portalmesh (Variables|Default|GetPortalMesh))
  (bind _ns_portal (Variables|Default|GetNS_Portal))
  (Components|StaticMesh|SetStaticMesh _portalmesh (Variables|Default|GetPortal%20Mesh))
  (Transformation|SetRelativeRotation _portalmesh (Math|Rotator|MakeRotator 0.0 0.0 (Variables|Default|GetPortal%20Angle)) false false)
  (Class|NiagaraComponent|SetAsset _ns_portal (Variables|Default|GetPortal%20Particle) true)
  (Transformation|SetRelativeScale3D _ns_portal (* "3.000000,3.000000,3.000000" (Variables|Default|GetScale))))