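; Projectile fired by a BasedShip, with Niagara trail and impact effects, that can home on a target enemy at fixed speed by resetting its velocity each Tick.
; On hit it disables itself, spawns the impact effect and subtracts the owner ship's damage from the struck ship's HP, reduced for long-range shots against the "Крепкий каркас" (sturdy frame) ability.
; It then destroys itself, after a delay unless a living owner's shot hit a non-ship.
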(event OnComponentHit(Sphere)
  (params (HitComponent :type Primitive%20Component%20Object%20Reference) (OtherActor :type Actor%20Object%20Reference) (OtherComp :type Primitive%20Component%20Object%20Reference) (NormalImpulse :type Vector :default "0, 0, 0") (Hit :type Hit%20Result%20Structure%20%28by%20ref%29))
  (bind _sphere (Variables|Default|GetSphere))
  (Utilities|FlowControl|Sequence
    (:then_0
      (Components|Activation|Deactivate (Variables|Default|GetNiagara))
      (Physics|SetSimulatePhysics _sphere false)
      (Collision|SetCollisionEnabled _sphere "NoCollision")
      (Rendering|SetVisibility _sphere false false)
      (Utilities|FlowControl|Delay 4.0)
      (Actor|DestroyActor))
    (:then_1
      (Niagara|SpawnSystematLocation (Variables|Default|GetNS_Hit%20) (.Location (Collision|BreakHitResult Hit)) (Transformation|GetActorRotation))
      (bind _asbased_ship (Utilities|Casting|CastToBasedShip (Components|GetOwner))
        (:then
          (bind _asbased_ship_2 (Utilities|Casting|CastToBasedShip OtherActor)
            (:then
              (bind _array_element (Utilities|Array|ForEachLoopwithBreak (Variables|/Game/Actors/Units/SpaceShips/BasedShip.BasedShip_C|GetAbilities _asbased_ship_2) :!label _label)
                (:LoopBody
                  (if (Utilities|Enum|Equal(Enum) (.AbilityName (Utilities|Struct|BreakS_Unit_Ability _array_element)) "Крепкий каркас")
                    (Variables|Default|SetEnemyHaveAbilityHardCarcas true)
                    (goto _label Break)))
                (:Completed
                  (if (Variables|Default|GetEnemyHaveAbilityHardCarcas)
                    (if (>= (Variables|Default|GetStartShootingDistance) 3e+03)
                      (Variables|/Game/Actors/Units/SpaceShips/BasedShip.BasedShip_C|SetCurrentHp _asbased_ship_2 (- (Variables|/Game/Actors/Units/SpaceShips/BasedShip.BasedShip_C|GetCurrentHp _asbased_ship_2) (* (.damage (Variables|/Game/Actors/Units/SpaceShips/BasedShip.BasedShip_C|GetUnitInfo _asbased_ship)) 0.75)))
                      (else
                        (bind _output_get (Variables|/Game/Actors/Units/SpaceShips/BasedShip.BasedShip_C|SetCurrentHp _asbased_ship_2 (- (Variables|/Game/Actors/Units/SpaceShips/BasedShip.BasedShip_C|GetCurrentHp _asbased_ship_2) (.damage (Variables|/Game/Actors/Units/SpaceShips/BasedShip.BasedShip_C|GetUnitInfo _asbased_ship))) :!label _label_2))))
                    (else
                      (goto _label_2)))
                  (Development|PrintString (Utilities|String|ToString(Float) _output_get))
                  (Utilities|FlowControl|Delay 3.0)
                  (Actor|DestroyActor))))
            (:CastFailed
              (Actor|DestroyActor)
              (Development|PrintString "Miss"))))
        (:CastFailed
          (Development|PrintString "Your Shooting Unit Was Killed"))))))

(event EventTick
  (params (DeltaSeconds :type Float%20%28single-precision%29))
  (bind _projectilemovement (Variables|Default|GetProjectileMovement))
  (if (Variables|Default|GetAutoaimingToEnemy)
    (bind _targetenemy (Variables|Default|GetTargetEnemy)
      (:then
        (Variables|/Script/Engine.MovementComponent|SetVelocity (Variables|Default|GetProjectileMovement) (* (Math|Vector|Normalize (- (Transformation|GetActorLocation _targetenemy) (Transformation|GetActorLocation)) 0.0) 5000)))
      (:else
        (Variables|/Script/Engine.MovementComponent|SetVelocity _projectilemovement (Variables|/Script/Engine.MovementComponent|GetVelocity _projectilemovement))))))

(fn ConstructionScript
  (Class|NiagaraComponent|SetAsset (Variables|Default|GetNiagara) (Variables|Default|GetNS_Projectile) true))

(fn FindRotationProjectiletoEnemy
  (params (ForwardVectorOfProjectile :type Vector) (InputVectorToEnemy :type Vector))
  (return (Class|KismetMathLibrary|DegAcos (Math|Vector|DotProduct (Math|Vector|Normalize ForwardVectorOfProjectile) (Math|Vector|Normalize InputVectorToEnemy)))))