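; BP_Shooting is an automatic projectile launcher for showing projectile VFX.
; One second after BeginPlay it spawns ProjectileBP at its own location, scaled down and aimed along its Arrow component, plus a LaunchParticle system as the launch effect.
; The NextArrow event re-calls itself after a random delay of a few seconds, firing indefinitely.
; A random spawn-offset calculation is left unconnected.
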(event Custom|NextArrow
  (bind _returnvalue (Transformation|GetActorLocation))
  (Game|SpawnActorfromClass (Variables|Default|GetProjectileBP) (Math|Transform|MakeTransform _returnvalue (.rotation (Transformation|GetWorldTransform (Variables|Default|GetArrow))) "0.100000,0.100000,0.100000") "Undefined" "SelectDefaultAtRuntime" 0 0)
  (Niagara|SpawnSystematLocation (Variables|Default|GetLaunch_Particle) _returnvalue (Transformation|GetActorRotation))
  (Utilities|FlowControl|Delay (Math|Random|RandomFloatinRange 3.5 2.0))
  (CallFunction|NextArrow))

(event EventBeginPlay
  (bind _returnvalue (Transformation|GetActorLocation))
  (Utilities|FlowControl|Delay 1.0)
  (Game|SpawnActorfromClass (Variables|Default|GetProjectileBP) (Math|Transform|MakeTransform _returnvalue (.rotation (Transformation|GetWorldTransform (Variables|Default|GetArrow))) "0.100000,0.100000,0.100000") "Undefined" "SelectDefaultAtRuntime" 0 0)
  (Niagara|SpawnSystematLocation (Variables|Default|GetLaunch_Particle) _returnvalue (Transformation|GetActorRotation))
  (Utilities|FlowControl|Delay (Math|Random|RandomFloatinRange 3.5 2.0))
  (CallFunction|NextArrow))

(fn ConstructionScript)