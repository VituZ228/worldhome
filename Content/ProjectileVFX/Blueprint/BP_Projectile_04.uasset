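; BP_Projectile_04 is a ship-fired projectile with Niagara trail and impact effects that damages ships and planet defence towers.
; When autoaiming, Tick steers its velocity straight at the target enemy at fixed speed.
; On hit, it shuts off, spawns the impact effect and subtracts the owning ship's damage from the victim's HP.
; Ships with the "Крепкий каркас" ability take reduced damage from long-range shots; delays or misses end in destruction.
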(event OnComponentHit(Sphere)
  (params (HitComponent :type Primitive%20Component%20Object%20Reference) (OtherActor :type Actor%20Object%20Reference) (OtherComp :type Primitive%20Component%20Object%20Reference) (NormalImpulse :type Vector :default "0, 0, 0") (Hit :type Hit%20Result%20Structure%20%28by%20ref%29))
  (bind _sphere (Variables|Default|GetSphere))
  (Utilities|FlowControl|Sequence
    (:then_0
      (Components|Activation|Deactivate (Variables|Default|GetNiagara))
      (Physics|SetSimulatePhysics _sphere false)
      (Collision|SetCollisionEnabled _sphere "NoCollision")
      (Rendering|SetVisibility _sphere false false)
      (Utilities|FlowControl|Delay 4.0)
      (Actor|DestroyActor))
    (:then_1
      (Niagara|SpawnSystematLocation (Variables|Default|GetNS_Hit%20) (.Location (Collision|BreakHitResult Hit)) (Transformation|GetActorRotation))
      (bind _asbased_ship (Utilities|Casting|CastToBasedShip (Components|GetOwner))
        (:then
          (bind _asbased_ship_2 (Utilities|Casting|CastToBasedShip OtherActor)
            (:then
              (Utilities|IsValid _asbased_ship_2
                (:Is%20Valid
                  (bind _array_element (Utilities|Array|ForEachLoopwithBreak (Variables|/Game/Actors/Units/SpaceShips/BasedShip.BasedShip_C|GetAbilities _asbased_ship_2) :!label _label)
                    (:LoopBody
                      (if (Utilities|Enum|Equal(Enum) (.AbilityName (Utilities|Struct|BreakS_Unit_Ability _array_element)) "Крепкий каркас")
                        (Variables|Default|SetEnemyHaveAbilityHardCarcas true)
                        (goto _label Break)))
                    (:Completed
                      (if (Variables|Default|GetEnemyHaveAbilityHardCarcas)
                        (if (>= (Variables|Default|GetStartShootingDistance) 3e+03)
                          (Utilities|IsValid _asbased_ship_2
                            (:Is%20Valid
                              (Variables|/Game/Actors/Units/SpaceShips/BasedShip.BasedShip_C|SetCurrentHp _asbased_ship_2 (- (Variables|/Game/Actors/Units/SpaceShips/BasedShip.BasedShip_C|GetCurrentHp _asbased_ship_2) (* (.damage (Variables|/Game/Actors/Units/SpaceShips/BasedShip.BasedShip_C|GetCurrentUnitInfo _asbased_ship)) 0.75)))
                              (Development|PrintString (Utilities|String|ToString(Float) (stale _output_get)) :!label _label_2))
                            (:Is%20Not%20Valid
                              _))
                          (else
                            (bind _output_get (Variables|/Game/Actors/Units/SpaceShips/BasedShip.BasedShip_C|SetCurrentHp _asbased_ship_2 (- (Variables|/Game/Actors/Units/SpaceShips/BasedShip.BasedShip_C|GetCurrentHp _asbased_ship_2) (.damage (Variables|/Game/Actors/Units/SpaceShips/BasedShip.BasedShip_C|GetCurrentUnitInfo _asbased_ship))) :!label _label_3))
                            (goto _label_2)))
                        (else
                          (goto _label_3)))
                      (Utilities|FlowControl|Delay 3.0 :!label _label_4)
                      (Actor|DestroyActor))))))
            (:CastFailed
              (bind _asplanet_defence_tower (Utilities|Casting|CastToPlanetDefenceTower OtherActor)
                (:then
                  (bind _output_get_2 (Variables|/Game/Actors/Planets/PlanetTowers/PlanetDefenceTower.PlanetDefenceTower_C|SetCurrentHp _asplanet_defence_tower (- (Variables|/Game/Actors/Planets/PlanetTowers/PlanetDefenceTower.PlanetDefenceTower_C|GetCurrentHp _asplanet_defence_tower) (.damage (Variables|/Game/Actors/Units/SpaceShips/BasedShip.BasedShip_C|GetCurrentUnitInfo _asbased_ship)))))
                  (Development|PrintString (Utilities|String|ToString(Float) _output_get_2))
                  (goto _label_4))
                (:CastFailed
                  (Actor|DestroyActor)
                  (Development|PrintString "Miss"))))))
        (:CastFailed
          (Development|PrintString "Your Shooting Unit Was Killed"))))))

(event EventTick
  (params (DeltaSeconds :type Float%20%28single-precision%29))
  (bind _projectilemovement (Variables|Default|GetProjectileMovement))
  (if (Variables|Default|GetAutoaimingToEnemy)
    (bind _targetenemy (Variables|Default|GetTargetEnemy)
      (:then
        (Variables|/Script/Engine.MovementComponent|SetVelocity (Variables|Default|GetProjectileMovement) (* (Math|Vector|Normalize (- (Transformation|GetActorLocation _targetenemy) (Transformation|GetActorLocation)) 0.0) 5000)))
      (:else
        (Variables|/Script/Engine.MovementComponent|SetVelocity _projectilemovement (Variables|/Script/Engine.MovementComponent|GetVelocity _projectilemovement))))))

(fn ConstructionScript
  (Class|NiagaraComponent|SetAsset (Variables|Default|GetNiagara) (Variables|Default|GetNS_Projectile) true))